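; AI turret actor that rotates to face the closest actor tagged "Player".
; Every tick, Lookat scans the tagged actors to set LockedTarget, and Tick turns the Rootmotion component toward it.
; A range-checked branch that spawns BP_Bullet from two arrow components after a short delay is not connected to any event, so the turret never fires.
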(event EventTick
  (params (DeltaSeconds :type Float%20%28single-precision%29))
  (bind _lockedtarget (Variables|Default|GetLockedTarget))
  (CallFunction|Lookat)
  (Utilities|IsValid _lockedtarget
    (:Is%20Valid
      (Transformation|SetWorldRotation (Variables|Default|Getrootmotion) (Math|Rotator|FindLookatRotation (Transformation|GetWorldLocation (Variables|Default|Getrootmotion)) (Transformation|GetActorLocation _lockedtarget)) false false))))

(fn ConstructionScript)

(fn Lookat
  (bind _outactors (Actor|GetAllActorswithTag "Player"))
  (Variables|Default|SetClosestTarget (Utilities|Array|Get(acopy) _outactors))
  (for (_array_element _array_index) _outactors
    (if (!= _array_index 0)
      (if (< (Transformation|GetDistanceTo _array_element 0) (Transformation|GetDistanceTo (Variables|Default|GetClosestTarget) 0))
        (Variables|Default|SetClosestTarget _array_element))))
  (Variables|Default|SetLockedTarget (Variables|Default|GetClosestTarget)))