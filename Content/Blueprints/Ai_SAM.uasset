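; AI surface-to-air missile turret that detects player aircraft by noise and fires homing missiles at them.
; PawnSensing hearing locks the aircraft; if it is in range, a missile spawns after a delay, given ammo and life, with that target.
; Tick yaws the mesh toward the locked target while alive.
; It also links a health widget and supplies map icon data; the sight-based Lookat targeting is unused.
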(event OnHearNoise(PawnSensing)
  (params (Instigator :type Pawn%20Object%20Reference) (Location :type Vector%20%28by%20ref%29 :default "0, 0, 0") (Volume :type Float%20%28single-precision%29))
  (bind _arrow (Variables|Default|GetArrow))
  (bind _returnvalue (Transformation|GetWorldTransform _arrow))
  (if (Variables|Default|GetIsAlive)
    (bind _asbp_aircraft_2 (Utilities|Casting|CastToBP_Aircraft2 Instigator))
    (if (Actor|ActorHasTag _asbp_aircraft_2 "Player")
      (Variables|Default|SetLockedTarget _asbp_aircraft_2)
      (if (< (Math|Vector|Distance(Vector) (Transformation|GetActorLocation (Variables|Default|GetLockedTarget)) (Transformation|GetActorLocation)) 1e+05)
        (Utilities|FlowControl|Delay 8.0)
        (if (> (Variables|Default|GetAmmo) 0)
          (if (Variables|Default|GetIsAlive)
            (bind _returnvalue_2 (Game|SpawnActorfromClass "/Game/Blueprints/MissileBaseClass/MissileSam.MissileSam_C" (Math|Transform|MakeTransform (.location _returnvalue) (.rotation _returnvalue) "1.000000,1.000000,1.000000") "Undefined" 0 0 0))
            (Variables|/Game/Blueprints/MissileBaseClass/MissileSam.MissileSam_C|SetCurrentTarget _returnvalue_2 (Variables|Default|GetLockedTarget))
            (Default|MissileFireM _returnvalue_2)
            (Variables|/Game/Blueprints/MissileBaseClass/MissileSam.MissileSam_C|SetIsDeployed _returnvalue_2 true)))))))

(event EventTick
  (params (DeltaSeconds :type Float%20%28single-precision%29))
  (bind _lockedtarget (Variables|Default|GetLockedTarget))
  (if (Variables|Default|GetIsAlive)
    (Utilities|IsValid _lockedtarget
      (:Is%20Valid
        (Transformation|SetWorldRotation (Variables|Default|GetStaticMesh1) (Math|Rotator|MakeRotator 0.0 0.0 (- (.yaw (Math|Rotator|FindLookatRotation (Transformation|GetWorldLocation (Variables|Default|Getrootmotion)) (Transformation|GetActorLocation _lockedtarget))) 9e+01)) false false)))))

(event EventBeginPlay
  (bind _asturret_health (Utilities|Casting|CastToTurretHealth (UserInterface|GetWidget (Variables|Default|GetWidget))))
  (Variables|/Game/HUD/TurretHealth.TurretHealth_C|SetTurret _asturret_health self))

(fn ConstructionScript)

(fn Lookat
  (Variables|Default|SetClosestTarget 0)
  (for (_array_element _array_index) (Variables|Default|GetSeeTargets)
    (if (!= _array_index 0)
      (if (< (Transformation|GetDistanceTo _array_element 0) (Transformation|GetDistanceTo (Variables|Default|GetClosestTarget) 0))
        (Variables|Default|SetClosestTarget 0))))
  (Variables|Default|SetLockedTarget (Variables|Default|GetClosestTarget)))

(fn GetMapIconData
  (bind _mapiconcomponent (Variables|Default|GetMapIconComponent))
  (return (Transformation|GetActorLocation) (Variables|/Game/Blueprints/MapIconComponent.MapIconComponent_C|GetImageTex _mapiconcomponent) (Variables|/Game/Blueprints/MapIconComponent.MapIconComponent_C|GetSize _mapiconcomponent)))