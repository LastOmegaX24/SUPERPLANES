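; YFA-XX aircraft Blueprint that configures a parent aircraft class and drives its engine glow.
; The construction script sets top thrust speed, movement rate curve and gun class, and disables the internal weapons bay before running parent construction.
; Each Tick creates red and blue emissive dynamic materials on the mesh.
; Their Thrust parameter follows the clamped gap between thrust and current speed, maxing out near top thrust.
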(event EventBeginPlay
  (|CallParentFunction) ; This node is disabled and will not be called.\nDrag off pins to build functionality.
)

(event EventTick
  (params (DeltaSeconds :type Float%20%28single-precision%29))
  (bind _staticmesh (Variables|Default|GetStaticMesh))
  (|CallParentFunction DeltaSeconds)
  (CallFunction|ThrustEffect _staticmesh _staticmesh))

(fn ConstructionScript
  (Variables|Default|SetMaxThrustSpeed 4.5e+03)
  (Variables|/Game/Blueprints/AircraftBaseClass/GenMove1.GenMove1_C|SetRateCurve (Variables|Default|GetGenMove1) "/Game/Blueprints/Aircraft/YFA_XX_RateCurve.YFA_XX_RateCurve")
  (Variables|Default|SetGunClass "/Game/Blueprints/Aircraft/YFA_XXGun.YFA_XXGun_C")
  (Variables|Default|SetHasInternalWB false)
  (|CallParentFunction))

(fn ThrustEffect
  (params (self2 :type Primitive%20Component%20Object%20Reference) (self3 :type Primitive%20Component%20Object%20Reference))
  (bind _thrustspeed (Variables|Default|GetThrustSpeed))
  (bind _currentspeed (Variables|Default|GetCurrentSpeed))
  (bind _maxthrustspeed (Variables|Default|GetMaxThrustSpeed))
  (bind _thrustspeed_2 (Variables|Default|GetThrustSpeed))
  (bind _returnvalue (- _maxthrustspeed 5e+02))
  (bind _returnvalue_2 (- _thrustspeed_2 _currentspeed))
  (bind _returnvalue_3 (/ _returnvalue_2 1e+03))
  (bind _returnvalue_4 (> _returnvalue _thrustspeed))
  (bind _returnvalue_5 (Math|Float|Clamp(Float) _returnvalue_3 0.0 5.0))
  (bind _returnvalue_6 (Math|Float|SelectFloat _returnvalue_5 5.0 _returnvalue_4))
  (bind _returnvalue_7 (Rendering|Material|CreateDynamicMaterialInstance self2 0 "/Game/content/Assets/Global/RedEmission.RedEmission" "None" :!class /Script/Engine.PrimitiveComponent))
  (Rendering|Material|SetScalarParameterValue _returnvalue_7 "Thrust" _returnvalue_6 :!class /Script/Engine.MaterialInstanceDynamic)
  (bind _returnvalue_8 (Rendering|Material|CreateDynamicMaterialInstance self3 1 "/Game/content/Assets/Global/BlueEmission.BlueEmission" "None" :!class /Script/Engine.PrimitiveComponent))
  (Rendering|Material|SetScalarParameterValue _returnvalue_8 "Thrust" _returnvalue_6 :!class /Script/Engine.MaterialInstanceDynamic))