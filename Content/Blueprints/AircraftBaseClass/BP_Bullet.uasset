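; BP_Bullet is a bullet actor that damages the actor it overlaps.
; On spawn it sets a limited lifespan and makes its mesh ignore the instigator and its owner's owner when moving.
; Overlaps pass through a server-named RPC event to a damage event, which skips Weapon-tagged actors and its owner.
; Valid hits receive standard damage credited to the instigator, then the bullet destroys itself.
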(event Custom|RPC_Server_Damage
  (params (NewParam :type Actor%20Object%20Reference))
  (CallFunction|RPCDamage NewParam))

(event Custom|RPC_Damage
  (params (NewParam :type Actor%20Object%20Reference))
  (Utilities|IsValid NewParam
    (:Is%20Valid
      (if (not (Actor|ActorHasTag NewParam "Weapon"))
        (if (not (== NewParam (Components|GetOwner)))
          (Game|Damage|ApplyDamage NewParam (Variables|Default|GetBaseDamage) (Pawn|GetController (Game|GetInstigator)) (Game|GetInstigator) "/Game/Blueprints/MainSystem/StandardDamage.StandardDamage_C")
          (Actor|DestroyActor))))))

(event Collision|EventActorBeginOverlap
  (params (OtherActor :type Actor%20Object%20Reference))
  (CallFunction|RPCServerDamage OtherActor))

(event EventBeginPlay
  (bind _staticmesh (Variables|Default|GetStaticMesh))
  (Actor|SetLifeSpan 15.0)
  (Collision|IgnoreActorwhenMoving _staticmesh (Variables|Actor|GetInstigator) true)
  (Collision|IgnoreActorwhenMoving _staticmesh (Components|GetOwner (Components|GetOwner)) true))

(fn ConstructionScript)