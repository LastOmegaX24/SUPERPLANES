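; GMC movement component for a player aircraft, providing networked, predicted flight with separate airborne, landed, stall and death behaviour.
; Enhanced Input sets roll, pitch, yaw, thrust, landing gear and FCS-limit state, bound for replication alongside speed and flight state.
; The prediction tick interpolates rotation and speed toward those targets, then moves along the forward vector.
; Curves scale pitch rate by speed, and low speed adds sink or nose-down fall.
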(event Input|EnhancedActionEvents|EnhancedInputActionPitch
  (params (ActionValue :type Float%20%28double-precision%29) (ElapsedSeconds :type Float%20%28double-precision%29) (TriggeredSeconds :type Float%20%28double-precision%29) (InputAction :type Input%20Action%20Object%20Reference :default "/Game/Input/Actions/Pitch.Pitch"))
  (:Triggered
    (Variables|Default|SetTargetPitch (Math|Float|Clamp(Float) ActionValue -1.0)))
  (:Canceled
    (Variables|Default|SetTargetPitch 0.0 :!label _label))
  (:Completed
    (goto _label)))

(event Input|EnhancedActionEvents|EnhancedInputActionYaw
  (params (ActionValue :type Float%20%28double-precision%29) (ElapsedSeconds :type Float%20%28double-precision%29) (TriggeredSeconds :type Float%20%28double-precision%29) (InputAction :type Input%20Action%20Object%20Reference :default "/Game/Input/Actions/Yaw.Yaw"))
  (:Triggered
    (Variables|Default|SetTargetYaw (Math|Float|Clamp(Float) ActionValue -1.0)))
  (:Canceled
    (Variables|Default|SetTargetYaw 0.0 :!label _label))
  (:Completed
    (goto _label)))

(event Input|EnhancedActionEvents|EnhancedInputActionRoll
  (params (ActionValue :type Float%20%28double-precision%29) (ElapsedSeconds :type Float%20%28double-precision%29) (TriggeredSeconds :type Float%20%28double-precision%29) (InputAction :type Input%20Action%20Object%20Reference :default "/Game/Input/Actions/Roll.Roll"))
  (:Triggered
    (Variables|Default|SetTargetRoll (Math|Float|Clamp(Float) ActionValue -1.0)))
  (:Canceled
    (Variables|Default|SetTargetRoll 0.0 :!label _label))
  (:Completed
    (goto _label)))

(event Input|EnhancedActionEvents|EnhancedInputActionAccelerateDecelerate
  (params (ActionValue :type Float%20%28double-precision%29) (ElapsedSeconds :type Float%20%28double-precision%29) (TriggeredSeconds :type Float%20%28double-precision%29) (InputAction :type Input%20Action%20Object%20Reference :default "/Game/Input/Actions/AccelerateDecelerate.AccelerateDecelerate"))
  (bind _returnvalue (Class|GMCMovementUtilityCmp|GetPhysDeltaTime))
  (:Triggered
    (Math|Float|CompareFloat ActionValue 0.0 :!label _label
      (:>
        (Variables|Default|SetBrake (Math|Interpolation|FInterpTo (Variables|Default|GetBrake) 0.0 _returnvalue 1e+01) :!label _label_2))
      (:==
        (goto _label_2))
      (:<
        (Variables|Default|SetBrake (Math|Interpolation|FInterpTo (Variables|Default|GetBrake) 2e+01 _returnvalue 1e+01))))
    (CallFunction|Speed0 ActionValue (Class|GMCMovementUtilityCmp|GetPhysDeltaTime)))
  (:Ongoing
    (goto _label)))

(event Input|EnhancedActionEvents|EnhancedInputActionFCSMode
  (params (ActionValue :type Boolean) (ElapsedSeconds :type Float%20%28double-precision%29) (TriggeredSeconds :type Float%20%28double-precision%29) (InputAction :type Input%20Action%20Object%20Reference :default "/Game/Input/Actions/FCSMode.FCSMode"))
  (:Triggered
    (Variables|Default|SetFCSLimit false)
    (Variables|Default|SetPitchM 7.0))
  (:Canceled
    (Variables|Default|SetFCSLimit true :!label _label)
    (Variables|Default|SetPitchM 5.0))
  (:Completed
    (goto _label)))

(event Input|EnhancedActionEvents|EnhancedInputActionLandingGear
  (params (ActionValue :type Boolean) (ElapsedSeconds :type Float%20%28double-precision%29) (TriggeredSeconds :type Float%20%28double-precision%29) (InputAction :type Input%20Action%20Object%20Reference :default "/Game/Input/Actions/LandingGear.LandingGear"))
  (:Started
    (Utilities|FlowControl|FlipFlop
      (:A
        (Variables|Default|SetLandingGear false)
        (Default|RemoveWarning (Variables|/Game/Blueprints/AircraftBaseClass/BP_Aircraft2.BP_Aircraft2_C|GetHUDWidgetRef (Variables|Default|GetPlayerPawnRef)) 670))
      (:B
        (Variables|Default|SetLandingGear true)
        (Default|AddWarning (Variables|/Game/Blueprints/AircraftBaseClass/BP_Aircraft2.BP_Aircraft2_C|GetHUDWidgetRef (Variables|Default|GetPlayerPawnRef)) "Landing Gear" 670)))))

(event EventGenPredictionTick
  (params (DeltaTime :type Float%20%28single-precision%29))
  (bind _returnvalue (Class|GMCMovementUtilityCmp|GetRootCollisionRotation))
  (bind _returnvalue_2 (Components|GetOwner))
  (bind _returnvalue_3 (Class|GMCMovementUtilityCmp|GetRootCollisionRotation))
  (bind _returnvalue_4 (Class|GMCMovementUtilityCmp|GetPhysDeltaTime))
  (bind _returnvalue_5 (Class|GMCMovementUtilityCmp|GetPhysDeltaTime))
  (bind _currentspeed (Variables|Default|GetCurrentSpeed))
  (bind _returnvalue_6 (Math|Rotator|Lerp(Rotator) (Math|Rotator|MakeRotator (.roll _returnvalue) (.pitch _returnvalue) (.yaw _returnvalue)) (Math|Rotator|MakeRotator (.roll _returnvalue) -9e+01 0.0) 0.01 true))
  (bind _returnvalue_7 (Math|Rotator|Lerp(Rotator) _returnvalue_3 (Math|Rotator|MakeRotator 0.0 -9e+01 0.0) 0.02 true))
  (bind _returnvalue_8 (Transformation|GetActorForwardVector _returnvalue_2))
  (Utilities|IsValid (Components|GetOwner)
    (:Is%20Valid
      (if (Variables|Default|GetIsLanded)
        (if (Variables|/Game/Blueprints/AircraftBaseClass/BP_Aircraft2.BP_Aircraft2_C|GetIsAlive (Variables|Default|GetPlayerPawnRef))
          (if (>= (Variables|Default|GetCurrentSpeed) (Variables|/Game/Blueprints/AircraftBaseClass/BP_Aircraft2.BP_Aircraft2_C|GetMinThrustStall (Variables|Default|GetPlayerPawnRef)))
            (CallFunction|YawF)
            (CallFunction|ControlAdd)
            (CallFunction|UpdatePositionGround DeltaTime)
            (bind _outhit (Class|MovementComponent|MoveUpdatedComponent (* (Class|GMCReplicationCmp|GetVelocity) (Class|GMCMovementUtilityCmp|GetPhysDeltaTime) 1.0) (Class|GMCMovementUtilityCmp|GetRootCollisionRotation) true))
            (if (.bBlockingHit (Collision|BreakHitResult _outhit))
              (Class|GMCMovementUtilityCmp|AdjustVelocityfromHit _outhit false 0.0)
              (Class|MovementComponent|MoveUpdatedComponent (* (Class|GMCReplicationCmp|GetVelocity) (Class|GMCMovementUtilityCmp|GetPhysDeltaTime) 1.0) (Class|GMCMovementUtilityCmp|GetRootCollisionRotation) true))
            (else
              (Variables|Default|SetIsLanded false))))
        (else
          (CallFunction|LeadTargetLoc)
          (if (Variables|/Game/Blueprints/AircraftBaseClass/BP_Aircraft2.BP_Aircraft2_C|GetIsAlive (Variables|Default|GetPlayerPawnRef))
            (if (or (>= (Variables|Default|GetCurrentSpeed) (Variables|Default|GetMin%20Thrust%20Stall)) (Variables|Default|GetLandingGear))
              _
              (else
                (Class|GMCMovementUtilityCmp|AddAcceleration (* (Math|Vector|VectorDown) 9.8) _returnvalue_4)
                (Class|GMCReplicationCmp|SetBasedControlRotation _returnvalue_6)
                (Class|MovementComponent|MoveUpdatedComponent (* (Class|GMCReplicationCmp|GetVelocity) _returnvalue_4) _returnvalue_6 true)))
            (CallFunction|RollF)
            (CallFunction|PitchF)
            (CallFunction|YawF)
            (CallFunction|ControlAdd)
            (CallFunction|UpdatePosition DeltaTime)
            (bind _outhit_2 (Class|MovementComponent|MoveUpdatedComponent (* (Class|GMCReplicationCmp|GetVelocity) (Class|GMCMovementUtilityCmp|GetPhysDeltaTime)) (Class|GMCMovementUtilityCmp|GetRootCollisionRotation) true))
            (if (.bBlockingHit (Collision|BreakHitResult _outhit_2))
              (Class|GMCMovementUtilityCmp|AdjustVelocityfromHit _outhit_2 true 0.0)
              (Class|MovementComponent|MoveUpdatedComponent (* (Class|GMCReplicationCmp|GetVelocity) (Class|GMCMovementUtilityCmp|GetPhysDeltaTime)) (Class|GMCMovementUtilityCmp|GetRootCollisionRotation) true))
            (else
              (Class|GMCMovementUtilityCmp|UpdateVelocity (* _returnvalue_8 _currentspeed) _returnvalue_5)
              (Class|GMCReplicationCmp|SetBasedControlRotation _returnvalue_7)
              (Class|MovementComponent|MoveUpdatedComponent (* _returnvalue_8 _currentspeed _returnvalue_5) _returnvalue_7 true))))))))

(event EventBindReplicationData
  (|CallParentFunction)
  (Class|GMCReplicationCmp|BindDoublePrecisionFloat (Variables|Default|GetCurrentRoll) "ServerAuth_Input_ClientValidated" "AlwaysCombine" "Periodic_Output" "NearestNeighbour")
  (Class|GMCReplicationCmp|BindDoublePrecisionFloat (Variables|Default|GetCurrentPitch) "ServerAuth_Input_ClientValidated" "AlwaysCombine" "Periodic_Output" "NearestNeighbour")
  (Class|GMCReplicationCmp|BindDoublePrecisionFloat (Variables|Default|GetCurrentYaw) "ServerAuth_Input_ClientValidated" "AlwaysCombine" "Periodic_Output" "NearestNeighbour")
  (Class|GMCReplicationCmp|BindDoublePrecisionFloat (Variables|Default|GetThrustMultiplier) "ClientAuth_Input" "AlwaysCombine" "Periodic_Output" "NearestNeighbour")
  (Class|GMCReplicationCmp|BindDoublePrecisionFloat (Variables|Default|GetThrustSpeed) "ClientAuth_Input" "AlwaysCombine" "Periodic_Output" "NearestNeighbour")
  (Class|GMCReplicationCmp|BindDoublePrecisionFloat (Variables|Default|GetAcceleration) "ServerAuth_Output_ServerValidated" "AlwaysCombine" "Periodic_Output" "NearestNeighbour")
  (Class|GMCReplicationCmp|BindDoublePrecisionFloat (Variables|Default|GetCurrentSpeed) "ServerAuth_InputOutput_ClientValidated" "AlwaysCombine" "Periodic_InputOutput" "NearestNeighbour")
  (Class|GMCReplicationCmp|BindDoublePrecisionFloat (Variables|Default|GetPitchM) "ClientAuth_Input" "AlwaysCombine" "Periodic_Output" "NearestNeighbour")
  (Class|GMCReplicationCmp|BindDoublePrecisionFloat (Variables|Default|GetStall) "ServerAuth_Output_ServerValidated" "AlwaysCombine" "Periodic_Output" "NearestNeighbour")
  (Class|GMCReplicationCmp|BindDoublePrecisionFloat (Variables|Default|GetTargetRoll) "ClientAuth_Input" "CombineIfUnchanged" "None" "NearestNeighbour")
  (Class|GMCReplicationCmp|BindDoublePrecisionFloat (Variables|Default|GetTargetYaw) "ClientAuth_Input" "CombineIfUnchanged" "None" "NearestNeighbour")
  (Class|GMCReplicationCmp|BindDoublePrecisionFloat (Variables|Default|GetTargetPitch) "ClientAuth_Input" "CombineIfUnchanged" "None" "NearestNeighbour")
  (Class|GMCReplicationCmp|BindDoublePrecisionFloat (Variables|Default|GetMaxThrustSpeed) "ServerAuth_Input_ServerValidated" "Default" "None" "NearestNeighbour")
  (Class|GMCReplicationCmp|BindDoublePrecisionFloat (Variables|Default|GetMin%20Thrust%20Stall) "ServerAuth_Input_ServerValidated" "AlwaysCombine" "None" "NearestNeighbour")
  (Class|GMCReplicationCmp|BindBool (Variables|Default|GetFCSLimit) "ClientAuth_Input" "AlwaysCombine" "None" "NearestNeighbour")
  (Class|GMCReplicationCmp|BindBool (Variables|Default|GetIsDash) "ClientAuth_Input" "CombineIfUnchanged" "None" "NearestNeighbour")
  (Class|GMCReplicationCmp|BindBool (Variables|Default|GetIsLanded) "ServerAuth_Output_ServerValidated" "AlwaysCombine" "Periodic_Output" "NearestNeighbour")
  (Class|GMCReplicationCmp|BindBool (Variables|Default|GetLandingGear) "ClientAuth_Input" "AlwaysCombine" "Periodic_Output" "NearestNeighbour")
  (Class|GMCReplicationCmp|BindBool (Variables|Default|GetIsLanded) "ServerAuth_Output_ServerValidated" "AlwaysCombine" "Periodic_Output" "NearestNeighbour"))

(event EventBeginPlay
  (bind _asbp_aircraft_2 (Utilities|Casting|CastToBP_Aircraft2 (Components|GetOwner)))
  (Variables|Default|SetPlayerPawnRef _asbp_aircraft_2)
  (bind _asgmc_controller (Utilities|Casting|CastToGMC_Controller (Game|GetPlayerController 0)))
  (Utilities|IsValid (PlayerController|LocalPlayerSubsystems|GetEnhancedInputLocalPlayerSubsystem _asgmc_controller)
    (:Is%20Valid
      (Input|AddMappingContext (PlayerController|LocalPlayerSubsystems|GetEnhancedInputLocalPlayerSubsystem _asgmc_controller) "/Game/Input/HOTAS.HOTAS" 1 "(bIgnoreAllPressedKeysUntilRelease=True,bForceImmediately=False)")
      (Input|AddMappingContext (PlayerController|LocalPlayerSubsystems|GetEnhancedInputLocalPlayerSubsystem _asgmc_controller) "/Game/Input/KBM.KBM" 0 "(bIgnoreAllPressedKeysUntilRelease=True,bForceImmediately=False)")
      (Variables|Default|SetThrustSpeed 0.0)
      (Variables|Default|SetCurrentSpeed 0.0)
      (Variables|Default|SetStall (Variables|/Game/Blueprints/AircraftBaseClass/BP_Aircraft2.BP_Aircraft2_C|GetMinThrustStall (Variables|Default|GetPlayerPawnRef)))
      (Variables|Default|SetMaxThrustSpeed (Variables|/Game/Blueprints/AircraftBaseClass/BP_Aircraft2.BP_Aircraft2_C|GetMaxThrustSpeed (Variables|Default|GetPlayerPawnRef)))
      (Variables|Default|SetMin%20Thrust%20Stall (Variables|/Game/Blueprints/AircraftBaseClass/BP_Aircraft2.BP_Aircraft2_C|GetMinThrustStall (Variables|Default|GetPlayerPawnRef))))))

(fn CamRollF
  (params (AngleDegrees :type Float%20%28double-precision%29))
  (bind _maxlook (Variables|Default|GetMaxLook))
  (bind _returnvalue (* _maxlook 0.35))
  (Variables|Default|SetTargetRoll (Math|Float|ClampAngle AngleDegrees (* _returnvalue -1.0) _returnvalue)))

(fn CamRollRecF
  (Variables|Default|SetTargetRoll (Math|Interpolation|FInterpTo (Variables|Default|GetTargetRoll) 0.0 (Variables|Default|GetDeltaSeconds) 0.0)))

(fn CamPitchF
  (params (AngleDegrees :type Float%20%28double-precision%29))
  (bind _currentspeed (Variables|Default|GetCurrentSpeed))
  (bind _maxlook (Variables|Default|GetMaxLook))
  (bind _fcslimit (Variables|Default|GetFCSLimit))
  (bind _rotationcurve (Variables|Default|GetRotationCurve))
  (bind _returnvalue (Math|Curves|GetFloatValue _rotationcurve _currentspeed))
  (bind _returnvalue_2 (Math|Float|Clamp(Float) _returnvalue 0.1))
  (bind _returnvalue_3 (select _fcslimit _returnvalue_2 _maxlook))
  (bind _returnvalue_4 (* _returnvalue_3 2.0))
  (Variables|Default|SetTargetPitch (Math|Float|ClampAngle AngleDegrees (* _returnvalue_4 -1.0) _returnvalue_4)))

(fn CamPitchRecF
  (Variables|Default|SetTargetPitch (Math|Interpolation|FInterpTo (Variables|Default|GetTargetPitch) 0.0 (Variables|Default|GetDeltaSeconds) 0.0)))

(fn CamYawF
  (params (AngleDegrees :type Float%20%28double-precision%29))
  (bind _currentspeed (Variables|Default|GetCurrentSpeed))
  (bind _maxlook (Variables|Default|GetMaxLook))
  (bind _fcslimit (Variables|Default|GetFCSLimit))
  (bind _rotationcurve (Variables|Default|GetRotationCurve))
  (bind _returnvalue (Math|Curves|GetFloatValue _rotationcurve _currentspeed))
  (bind _returnvalue_2 (Math|Float|Clamp(Float) _returnvalue 0.1))
  (bind _returnvalue_3 (select _fcslimit _returnvalue_2 _maxlook))
  (bind _returnvalue_4 (* _returnvalue_3 1.2))
  (Variables|Default|SetTargetYaw (Math|Float|ClampAngle AngleDegrees (* _returnvalue_4 -1.0) _returnvalue_4)))

(fn CamYawRecF
  (Variables|Default|SetTargetYaw (Math|Interpolation|FInterpTo (Variables|Default|GetTargetYaw) 0.0 (Variables|Default|GetDeltaSeconds) 0.0)))

(fn CopyRot)

(fn UpdatePosition
  (params (Delta :type Float%20%28double-precision%29))
  (bind _output_get (Variables|Default|SetCurrentSpeed (Math|Float|Clamp(Float) (Math|Interpolation|FInterpTo (Variables|Default|GetCurrentSpeed) (Variables|Default|GetThrustSpeed) Delta (* (Variables|Default|GetAcceleration) 0.1)) 0.0 (Variables|Default|GetMaxThrustSpeed))))
  (if (> _output_get (Variables|Default|GetStall))
    (Class|GMCMovementUtilityCmp|UpdateVelocity (* (Transformation|GetActorForwardVector (Components|GetOwner)) (Variables|Default|GetCurrentSpeed)) (Class|GMCMovementUtilityCmp|GetPhysDeltaTime))
    (else
      (Class|GMCMovementUtilityCmp|UpdateVelocity (+ (* (Transformation|GetActorForwardVector (Components|GetOwner)) (Variables|Default|GetCurrentSpeed)) (* (Math|Vector|VectorDown) (Math|Float|SafeDivide (Variables|Default|GetGravity) (+ (Variables|Default|GetCurrentSpeed) 1.0)))) (Class|GMCMovementUtilityCmp|GetPhysDeltaTime))))
  (return (* (Transformation|GetActorForwardVector (Components|GetOwner)) (Variables|Default|GetCurrentSpeed))))

(fn RollF
  (Variables|Default|SetCurrentRoll (Math|Interpolation|FInterpTo (Variables|Default|GetCurrentRoll) (Variables|Default|GetTargetRoll) (Class|GMCMovementUtilityCmp|GetPhysDeltaTime) (Variables|Default|GetInterp%20Speed))))

(fn PitchF
  (Variables|Default|SetCurrentPitch (Math|Interpolation|FInterpTo (Variables|Default|GetCurrentPitch) (* (Variables|Default|GetTargetPitch) (Utilities|TurnspeedMacro)) (Class|GMCMovementUtilityCmp|GetPhysDeltaTime) (Variables|Default|GetInterp%20Speed))))

(fn YawF
  (Variables|Default|SetCurrentYaw (Math|Interpolation|FInterpTo (Variables|Default|GetCurrentYaw) (Variables|Default|GetTargetYaw) (Class|GMCMovementUtilityCmp|GetPhysDeltaTime) (Variables|Default|GetInterp%20Speed))))

(fn Speed0
  (params (Speed :type Float%20%28double-precision%29) (Delta :type Float%20%28double-precision%29))
  (Variables|Default|SetThrustSpeed (Math|Float|SelectFloat (Math|Float|Clamp(Float) (Math|Float|Clamp(Float) (+ (* Speed Delta (Variables|Default|GetThrustMultiplier)) (Variables|Default|GetThrustSpeed)) 0.0 (Variables|Default|GetMaxThrustSpeed)) 0.0 2e+03) (Math|Float|Clamp(Float) (+ (* Speed Delta (Variables|Default|GetThrustMultiplier)) (Variables|Default|GetThrustSpeed)) 0.0 (Variables|Default|GetMaxThrustSpeed)) (Variables|Default|GetLandingGear))))

(fn CopyRot2)

(fn Yaw2
  (params (A :type Float%20%28double-precision%29) (B :type Float%20%28double-precision%29))
  (bind _yawdif (Variables|Default|GetYawDif))
  (bind _returnvalue (* _yawdif -1.0))
  (Utilities|ComparewithError (Variables|Default|GeterrorMargin) A B
    (:EqualAbout
      (Variables|Default|SetAVYaw (Math|Interpolation|FInterptoConstant (Variables|Default|GetAVYaw) 0.0 (Class|GMCMovementUtilityCmp|GetPhysDeltaTime) (Variables|Default|Getintspeed))))
    (:Less
      (Variables|Default|SetAVYaw (Math|Interpolation|FInterptoConstant (Variables|Default|GetAVYaw) (Math|Float|Clamp(Float) (+ (Variables|Default|GetAVYaw) _yawdif) _returnvalue _yawdif) (Class|GMCMovementUtilityCmp|GetPhysDeltaTime) (Variables|Default|Getintspeed))))
    (:Greater
      (Variables|Default|SetAVYaw (Math|Interpolation|FInterptoConstant (Variables|Default|GetAVYaw) (Math|Float|Clamp(Float) (- (Variables|Default|GetAVYaw) _yawdif) _returnvalue _yawdif) (Class|GMCMovementUtilityCmp|GetPhysDeltaTime) (Variables|Default|Getintspeed))))))

(fn Pitch2
  (params (A :type Float%20%28double-precision%29) (B :type Float%20%28double-precision%29))
  (bind _pitchdif (Variables|Default|GetPitchDif))
  (bind _returnvalue (* _pitchdif -1.0))
  (Utilities|ComparewithError (Variables|Default|GeterrorMargin) A B
    (:EqualAbout
      (Variables|Default|SetAVPitch (Math|Interpolation|FInterptoConstant (Variables|Default|GetAVPitch) 0.0 (Class|GMCMovementUtilityCmp|GetPhysDeltaTime) (Variables|Default|Getintspeed))))
    (:Less
      (Variables|Default|SetAVPitch (Math|Interpolation|FInterptoConstant (Variables|Default|GetAVPitch) (Math|Float|Clamp(Float) (+ (Variables|Default|GetAVPitch) _pitchdif) _returnvalue _pitchdif) (Class|GMCMovementUtilityCmp|GetPhysDeltaTime) (Variables|Default|Getintspeed))))
    (:Greater
      (Variables|Default|SetAVPitch (Math|Interpolation|FInterptoConstant (Variables|Default|GetAVPitch) (Math|Float|Clamp(Float) (- (Variables|Default|GetAVPitch) _pitchdif) _returnvalue _pitchdif) (Class|GMCMovementUtilityCmp|GetPhysDeltaTime) (Variables|Default|Getintspeed))))))

(fn Roll2
  (params (A :type Float%20%28double-precision%29) (B :type Float%20%28double-precision%29))
  (bind _rolldif (Variables|Default|GetRollDif))
  (bind _returnvalue (* _rolldif -1.0))
  (Utilities|ComparewithError (Variables|Default|GeterrorMargin) A B
    (:EqualAbout
      (Variables|Default|SetAVRoll (Math|Interpolation|FInterptoConstant (Variables|Default|GetAVRoll) 0.0 (Class|GMCMovementUtilityCmp|GetPhysDeltaTime) (Variables|Default|Getintspeed))))
    (:Less
      (Variables|Default|SetAVRoll (Math|Interpolation|FInterptoConstant (Variables|Default|GetAVRoll) (Math|Float|Clamp(Float) (+ (Variables|Default|GetAVRoll) 0.0) _returnvalue _rolldif) (Class|GMCMovementUtilityCmp|GetPhysDeltaTime) (Variables|Default|Getintspeed))))
    (:Greater
      (Variables|Default|SetAVRoll (Math|Interpolation|FInterptoConstant (Variables|Default|GetAVRoll) (Math|Float|Clamp(Float) (- (Variables|Default|GetAVRoll) 0.0) _returnvalue _rolldif) (Class|GMCMovementUtilityCmp|GetPhysDeltaTime) (Variables|Default|Getintspeed))))))

(fn ControlAdd
  (bind _returnvalue (Class|PawnMovementComponent|GetPawnOwner))
  (Utilities|IsValid _returnvalue
    (:Is%20Valid
      (Transformation|AddActorLocalRotation _returnvalue (* (Math|Rotator|MakeRotator (* (Variables|Default|GetCurrentRoll) (Variables|Default|GetRollM)) (* (Variables|Default|GetCurrentPitch) (Variables|Default|GetPitchM)) (* (Variables|Default|GetCurrentYaw) (Variables|Default|GetYawM))) (* (Class|GMCMovementUtilityCmp|GetPhysDeltaTime) 1e+01)) false false))))

(fn UpdatePositionGround
  (params (Delta :type Float%20%28double-precision%29))
  (bind _output_get (Variables|Default|SetCurrentSpeed (Math|Float|Clamp(Float) (Math|Interpolation|FInterpTo (Variables|Default|GetCurrentSpeed) (Variables|Default|GetThrustSpeed) Delta (Variables|Default|GetAcceleration)) 0.0 (Variables|Default|GetStall))))
  (if (> _output_get (Variables|Default|GetStall))
    (Class|GMCMovementUtilityCmp|UpdateVelocity (* (Transformation|GetActorForwardVector (Components|GetOwner)) (Variables|Default|GetCurrentSpeed)) (Class|GMCMovementUtilityCmp|GetPhysDeltaTime))
    (else
      (Class|GMCMovementUtilityCmp|UpdateVelocity (+ (* (Transformation|GetActorForwardVector (Components|GetOwner)) (Variables|Default|GetCurrentSpeed)) (* (Math|Vector|VectorDown) (Math|Float|SafeDivide (Variables|Default|GetGravity) (+ (Variables|Default|GetCurrentSpeed) 1.0)))) (Class|GMCMovementUtilityCmp|GetPhysDeltaTime))))
  (return (* (Transformation|GetActorForwardVector (Components|GetOwner)) (Variables|Default|GetCurrentSpeed))))

(fn LeadTargetLoc
  (Transformation|SetRelativeLocation (Variables|/Game/Blueprints/AircraftBaseClass/BP_Aircraft2.BP_Aircraft2_C|GetLeadTarget (Variables|Default|GetPlayerPawnRef)) (Math|Vector|MakeVector (Math|Vector|VectorLength (Class|GMCReplicationCmp|GetVelocity)) 0.0 0.0) false false))