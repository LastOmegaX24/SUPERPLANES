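; Gun actor, attached to a parent actor in the aircraft classes, that fires bullets from its Arrow with random pitch and yaw spread set by Accuracy.
; GunFire waits FireRate, then, if Ammo remains, spawns a client bullet for local calls.
; Non-local calls require Source to match the parent, spawn the standard bullet and alone decrement Ammo.
; Tick mirrors PlayerRef's hidden state onto the gun.
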(event Custom|GunFire
  (params (Source :type Actor%20Object%20Reference) (Local :type Boolean))
  (bind _accuracy (Variables|Default|GetAccuracy))
  (bind _arrow (Variables|Default|GetArrow))
  (bind _accuracy_2 (Variables|Default|GetAccuracy))
  (bind _arrow_2 (Variables|Default|GetArrow))
  (bind _returnvalue (Transformation|GetWorldTransform _arrow_2))
  (bind _returnvalue_2 (Transformation|GetWorldTransform _arrow))
  (bind _returnvalue_3 (* _accuracy -1.0))
  (bind _returnvalue_4 (* _accuracy_2 -1.0))
  (if Local
    (if true
      (Variables|Default|SetIsFiring true)
      (Utilities|FlowControl|Delay (Variables|Default|GetFireRate))
      (if (> (Variables|Default|GetAmmo) 0)
        (Game|SpawnActorfromClass "/Game/Blueprints/AircraftBaseClass/BP_Client_Bullet.BP_Client_Bullet_C" (Math|Transform|MakeTransform (.location _returnvalue) (Math|Rotator|MakeRotator (.roll (.rotation _returnvalue)) (+ (.pitch (.rotation _returnvalue)) (Math|Random|RandomFloatinRange _returnvalue_3 _accuracy)) (+ (.yaw (.rotation _returnvalue)) (Math|Random|RandomFloatinRange _returnvalue_3 _accuracy))) (.scale _returnvalue)) "AlwaysSpawn" (Actor|GetAttachParentActor) (Game|GetInstigator))))
    (elif (== Source (Actor|GetAttachParentActor))
      (Variables|Default|SetIsFiring true)
      (Utilities|FlowControl|Delay (Variables|Default|GetFireRate))
      (if (> (Variables|Default|GetAmmo) 0)
        (Game|SpawnActorfromClass "/Game/Blueprints/AircraftBaseClass/BP_Bullet.BP_Bullet_C" (Math|Transform|MakeTransform (.location _returnvalue_2) (Math|Rotator|MakeRotator (.roll (.rotation _returnvalue_2)) (+ (.pitch (.rotation _returnvalue_2)) (Math|Random|RandomFloatinRange _returnvalue_4 _accuracy_2)) (+ (.yaw (.rotation _returnvalue_2)) (Math|Random|RandomFloatinRange _returnvalue_4 _accuracy_2))) (.scale _returnvalue_2)) "AlwaysSpawn" (Actor|GetAttachParentActor) (Game|GetInstigator))
        (Math|Integer|DecrementInt (Variables|Default|GetAmmo))))))

(event EventTick
  (params (DeltaSeconds :type Float%20%28single-precision%29))
  (bind _playerref (Variables|Default|GetPlayerRef))
  (Utilities|IsValid _playerref
    (:Is%20Valid
      (Rendering|SetActorHiddenInGame (Variables|/Script/Engine.Actor|GetbHidden _playerref)))))

(fn ConstructionScript)