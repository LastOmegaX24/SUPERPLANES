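; Test pawn for arcade-style aircraft flight, with throttle, pitch, roll, yaw, dash, gunfire and health.
; Enhanced Input drives local rotations, while Tick moves it forward with drag, turn speed loss and low-speed gravity, prints debug values and feeds thrust to ArcHorizonAnim.
; Firing loops on a delay, alternating two muzzles; damage spawns explosions and clears IsAlive at zero health.
; High-G turn logic and stat initialization are unwired.
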(event Custom|Firing
  (if (Variables|Default|GetIsFiring)
    (if (> (Math|Integer|%(Integer) (Variables|Default|GetFireSequence) 2) 0)
      (Variables|Default|SetFireLocation (Variables|Default|GetFireLocation1))
      (else
        (Variables|Default|SetFireLocation (Variables|Default|GetFirelocation2))))
    (Game|SpawnActorfromClass "/Game/Blueprints/BP_Projectile.BP_Projectile_C" (Transformation|GetWorldTransform (Variables|Default|GetFireLocation)) "AlwaysSpawn" 0 0)
    (Variables|Default|SetFireSequence (+ (Variables|Default|GetFireSequence) 1))
    (Utilities|FlowControl|Delay 0.03)
    (CallFunction|Firing)))

(event Input|EnhancedActionEvents|EnhancedInputActionYaw
  (params (ActionValue :type Float%20%28double-precision%29) (ElapsedSeconds :type Float%20%28double-precision%29) (TriggeredSeconds :type Float%20%28double-precision%29) (InputAction :type Input%20Action%20Object%20Reference :default "/Game/Input/Actions/Yaw.Yaw"))
  (:Triggered
    (CallFunction|UpdateYaw (Utilities|Time|GetWorldDeltaSeconds) ActionValue :!label _label))
  (:Ongoing
    (goto _label)))

(event Input|EnhancedActionEvents|EnhancedInputActionRoll
  (params (ActionValue :type Float%20%28double-precision%29) (ElapsedSeconds :type Float%20%28double-precision%29) (TriggeredSeconds :type Float%20%28double-precision%29) (InputAction :type Input%20Action%20Object%20Reference :default "/Game/Input/Actions/Roll.Roll"))
  (:Triggered
    (CallFunction|UpdateRoll (Utilities|Time|GetWorldDeltaSeconds) ActionValue :!label _label))
  (:Ongoing
    (goto _label)))

(event Input|EnhancedActionEvents|EnhancedInputActionPitch
  (params (ActionValue :type Float%20%28double-precision%29) (ElapsedSeconds :type Float%20%28double-precision%29) (TriggeredSeconds :type Float%20%28double-precision%29) (InputAction :type Input%20Action%20Object%20Reference :default "/Game/Input/Actions/Pitch.Pitch"))
  (:Triggered
    (CallFunction|UpdatePitch (Utilities|Time|GetWorldDeltaSeconds) ActionValue :!label _label))
  (:Ongoing
    (goto _label)))

(event Input|EnhancedActionEvents|EnhancedInputActionDash
  (params (ActionValue :type Boolean) (ElapsedSeconds :type Float%20%28double-precision%29) (TriggeredSeconds :type Float%20%28double-precision%29) (InputAction :type Input%20Action%20Object%20Reference :default "/Game/Input/Actions/Dash.Dash"))
  (:Triggered
    (CallFunction|DashF)))

(event EventBeginPlay
  (bind _asplayer_controller (Utilities|Casting|CastToPlayerController (Pawn|GetController)))
  (Utilities|IsValid (PlayerController|LocalPlayerSubsystems|GetEnhancedInputLocalPlayerSubsystem _asplayer_controller)
    (:Is%20Valid
      (Input|AddMappingContext (PlayerController|LocalPlayerSubsystems|GetEnhancedInputLocalPlayerSubsystem _asplayer_controller) "/Game/Input/NewInputMappingContext.NewInputMappingContext" 0 "(bIgnoreAllPressedKeysUntilRelease=True,bForceImmediately=False)"))))

(event EventTick
  (params (DeltaSeconds :type Float%20%28single-precision%29))
  (CallFunction|UpdatePosition DeltaSeconds)
  (CallFunction|PrintVar)
  (CallFunction|GetAirspeed))

(event Game|Damage|EventAnyDamage
  (params (Damage :type Float%20%28single-precision%29) (DamageType :type Damage%20Type%20Object%20Reference) (InstigatedBy :type Controller%20Object%20Reference) (DamageCauser :type Actor%20Object%20Reference))
  (Effects|SpawnEmitteratLocation "/Game/StarterContent/Particles/P_Explosion.P_Explosion" "0, 0, 0")
  (Variables|Default|SetHealth (Math|Float|Clamp(Float) (- (Variables|Default|GetHealth) Damage) 0.0 (Variables|Default|GetMaxHealth)))
  (if (<= (Variables|Default|GetHealth) 0.0)
    (Variables|Default|SetIsAlive false)))

(event Input|ActionEvents|InputActionFire
  (params (Key :type Key%20Structure :default "None"))
  (:Pressed
    (Variables|Default|SetIsFiring true)
    (CallFunction|Firing))
  (:Released
    (Variables|Default|SetIsFiring false)))

(event Input|AxisEvents|InputAxisThrottle
  (params (AxisValue :type Float%20%28single-precision%29))
  (Variables|Default|SetThrustSpeed (Math|Float|Clamp(Float) (+ (* AxisValue (Utilities|Time|GetWorldDeltaSeconds) (Variables|Default|GetThrustMultiplier)) (Variables|Default|GetThrustSpeed)) 0.0 (Variables|Default|GetMaxThrustSpeed))))

(fn ConstructionScript)

(fn ThrottleInput
  (bind _tempname (Variables|Default|GetTempName))
  (if true
    (bind _result (Math|Integer|IncrementInt _tempname))
    (elif true
      (bind _result_2 (Math|Integer|DecrementInt _tempname)))))

(fn UpdatePosition
  (params (DeltaSeconds :type Float%20%28double-precision%29))
  (bind _turnspeed (Variables|Default|GetTurnspeed))
  (bind _returnvalue (* _turnspeed 1e+02))
  ;[1 1 1] Calc Current Speed
  (Variables|Default|SetCurrentSpeed (Math|Float|Clamp(Float) (- (select (< (Variables|Default|GetThrustSpeed) (Variables|Default|GetCurrentSpeed)) (Math|Interpolation|FInterpTo (Variables|Default|GetCurrentSpeed) (Variables|Default|GetThrustSpeed) DeltaSeconds (Variables|Default|GetDrag)) (Variables|Default|GetThrustSpeed)) (Math|Float|Absolute(Float) (+ (* (Variables|Default|GetTargetPitch) _returnvalue) (* (Variables|Default|GetTargetYaw) _returnvalue)))) 0.0 1e+04))
  ;[1 1 1] Calc new position based on speed
  (Variables|Default|SetNewPos (* (* (Variables|Default|GetCurrentSpeed) DeltaSeconds) (Transformation|GetActorForwardVector)))
  ;[1 1 1] Calc Applied Gravity
  (Variables|Default|SetAppliedGravity (Math|Float|MapRangeClamped (Variables|Default|GetCurrentSpeed) 0.0 (Variables|Default|GetMinThrustStall) (Variables|Default|GetGravity) 0.0))
  ;[1 1 1] Get Position
  (Transformation|AddActorWorldOffset (Math|Vector|MakeVector (.X (Class|KismetMathLibrary|BreakVector3f (Variables|Default|GetNewPos))) (.Y (Class|KismetMathLibrary|BreakVector3f (Variables|Default|GetNewPos))) (- (.Z (Class|KismetMathLibrary|BreakVector3f (Variables|Default|GetNewPos))) (* (Variables|Default|GetAppliedGravity) DeltaSeconds))) true))

(fn PrintVar
  (Utilities|FlowControl|Sequence
    (:then_0
      (Development|PrintString (Utilities|String|Append "ThrustSpeed;" (Utilities|String|ToString(Float) (Variables|Default|GetThrustSpeed)))))
    (:then_1
      (Development|PrintString (Utilities|String|Append "CurrentSpeed;" (Utilities|String|ToString(Float) (Variables|Default|GetCurrentSpeed)))))
    (:then_2
      (Development|PrintString (Utilities|String|Append "AppliedGravity;" (Utilities|String|ToString(Float) (Variables|Default|GetAppliedGravity)))))
    (:then_3
      (Development|PrintString (Utilities|String|Append "Turnspeed;" (Utilities|String|ToString(Float) (Variables|Default|GetTurnspeed)))))
    (:then_4
      (Development|PrintString (Utilities|String|Append "Health;" (Utilities|String|ToString(Float) (Variables|Default|GetHealth)))))))

(fn UpdateYaw
  (params (DeltaSeconds :type Float%20%28double-precision%29) (Yaw :type Float%20%28double-precision%29))
  (bind _output_get (Variables|Default|SetTargetYaw Yaw))
  (Variables|Default|SetCurrentSpeed (- (Variables|Default|GetCurrentSpeed) (* (Math|Float|Absolute(Float) _output_get) 2.0)))
  (bind _output_get_2 (Variables|Default|SetCurrentYaw (Math|Interpolation|FInterpTo (Variables|Default|GetCurrentYaw) (Variables|Default|GetTargetYaw) DeltaSeconds 1e+01)))
  (Transformation|AddActorLocalRotation (Math|Rotator|MakeRotator 0.0 0.0 (* _output_get_2 DeltaSeconds (Variables|Default|GetTurnspeed) 8.0)) false false))

(fn UpdateRoll
  (params (DeltaSeconds :type Float%20%28double-precision%29) (Roll :type Float%20%28double-precision%29))
  (Variables|Default|SetTargetRoll Roll)
  (bind _output_get (Variables|Default|SetCurrentRoll (Math|Interpolation|FInterpTo (Variables|Default|GetCurrentRoll) (Variables|Default|GetTargetRoll) DeltaSeconds 1e+01)))
  (Transformation|AddActorLocalRotation (Math|Rotator|MakeRotator (* _output_get DeltaSeconds 1.5e+02) 0.0 0.0) false false))

(fn UpdatePitch
  (params (DeltaSeconds :type Float%20%28double-precision%29) (Pitch :type Float%20%28double-precision%29))
  (Variables|Default|SetCurrentPitch Pitch)
  (bind _output_get (Variables|Default|SetTargetPitch (Math|Interpolation|FInterpTo (Variables|Default|GetCurrentPitch) (Variables|Default|GetTargetPitch) DeltaSeconds 1e+01)))
  (Transformation|AddActorLocalRotation (Math|Rotator|MakeRotator 0.0 (* _output_get DeltaSeconds (Variables|Default|GetTurnspeed) 1e+01) 0.0) false false))

(fn DashF
  (Variables|Default|SetCurrentSpeed (Variables|Default|GetDashDist)))

(fn HighGTurnNPSM
  (if (and (<= (Variables|Default|GetCurrentSpeed) 1.5e+03) (Variables|Default|GetIsPSMCapable))
    (Variables|Default|SetTurnspeed 1e+01)
    (else
      (Variables|Default|SetTurnspeed 3.0))))

(fn GetAirspeed
  (bind _asarc_horizon_anim (Utilities|Casting|CastToArcHorizonAnim (Components|SkeletalMesh|GetAnimInstance (Variables|Default|GetSkeletalMesh))))
  (Variables|/Game/Blueprints/ArcHorizonAnim.ArcHorizonAnim_C|SetAirspeed _asarc_horizon_anim (Variables|Default|GetThrustSpeed)))