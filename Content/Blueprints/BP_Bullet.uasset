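; BP_Bullet is a projectile actor that damages what it overlaps, then destroys itself.
; On spawn it stores player pawn 0 as Prototype_9 and sets a limited lifespan.
; Overlaps pass through RPC_Server_Damage to RPC_Damage, which ignores that stored pawn and applies damage with it as causer.
; A scaled-down Sparks Niagara effect exists in the graph but is unconnected.
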(event Custom|RPC_Server_Damage
  (params (NewParam :type Actor%20Object%20Reference))
  (CallFunction|RPCDamage NewParam))

(event Custom|RPC_Damage
  (params (NewParam :type Actor%20Object%20Reference))
  (bind _playerref (Variables|Default|GetPlayerRef))
  (if (!= NewParam _playerref)
    (Game|Damage|ApplyDamage NewParam (Variables|Default|GetBaseDamage) 0 _playerref "/Script/Engine.DamageType")
    (Actor|DestroyActor)))

(event Collision|EventActorBeginOverlap
  (params (OtherActor :type Actor%20Object%20Reference))
  (CallFunction|RPCServerDamage OtherActor))

(event EventBeginPlay
  (bind _asprototype_9 (Utilities|Casting|CastToPrototype_9 (Game|Player|GetPlayerPawn 0)))
  (Variables|Default|SetPlayerRef _asprototype_9)
  (Actor|SetLifeSpan 15.0))

(fn ConstructionScript)