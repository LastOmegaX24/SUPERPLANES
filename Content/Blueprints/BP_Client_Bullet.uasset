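; BP_Client_Bullet is a short-lived bullet actor that removes itself on contact and applies no damage of its own.
; On spawn it sets a fixed lifespan and tells its static mesh to ignore the instigator and its owner's owner when moving.
; On overlap it destroys itself unless the other actor is tagged Weapon or is its direct owner.
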(event Collision|EventActorBeginOverlap
  (params (OtherActor :type Actor%20Object%20Reference))
  (Utilities|IsValid OtherActor
    (:Is%20Valid
      (if (not (Actor|ActorHasTag OtherActor "Weapon"))
        (if (not (== OtherActor (Components|GetOwner)))
          (Actor|DestroyActor))))))

(event EventBeginPlay
  (bind _staticmesh (Variables|Default|GetStaticMesh))
  (Actor|SetLifeSpan 15.0)
  (Collision|IgnoreActorwhenMoving _staticmesh (Variables|Actor|GetInstigator) true)
  (Collision|IgnoreActorwhenMoving _staticmesh (Components|GetOwner (Components|GetOwner)) true))

(fn ConstructionScript)