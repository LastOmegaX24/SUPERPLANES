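; Railgun projectile actor that damages what it overlaps and expires after a fixed lifespan.
; BeginPlay caches player pawn 1 as a BP_Aircraft reference.
; Overlaps pass through server-named and damage RPC events, which apply damage and destroy the projectile only if the target is that aircraft or has the Weapon tag.
; Damage is always credited to player controller 0, and Hit is unused.
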(event Custom|RPC_Damage
  (params (NewParam :type Actor%20Object%20Reference))
  (if (not (and (!= NewParam (Variables|Default|GetPlayerRef)) (not (Actor|ActorHasTag NewParam "Weapon"))))
    (Game|Damage|ApplyDamage NewParam (Variables|Default|GetBaseDamage) (Game|GetPlayerController 0) 0 "/Script/Engine.DamageType")
    (Actor|DestroyActor)))

(event Custom|RPC_Server_Damage
  (params (NewParam :type Actor%20Object%20Reference))
  (CallFunction|RPCDamage NewParam))

(event Collision|EventHit
  (params (MyComp :type Primitive%20Component%20Object%20Reference) (Other :type Actor%20Object%20Reference) (OtherComp :type Primitive%20Component%20Object%20Reference) (bSelfMoved :type Boolean) (HitLocation :type Vector :default "0, 0, 0") (HitNormal :type Vector :default "0, 0, 0") (NormalImpulse :type Vector :default "0, 0, 0") (Hit :type Hit%20Result%20Structure%20%28by%20ref%29)))

(event Collision|EventActorBeginOverlap
  (params (OtherActor :type Actor%20Object%20Reference))
  (CallFunction|RPCServerDamage OtherActor))

(event EventBeginPlay
  (bind _asbp_aircraft (Utilities|Casting|CastToBP_Aircraft (Game|Player|GetPlayerPawn 1)))
  (Variables|Default|SetPlayerRef _asbp_aircraft)
  (Actor|SetLifeSpan 2e+01))

(fn ConstructionScript)