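; Basic control pawn that sets up Enhanced Input and lets the player toggle the map.
; On BeginPlay it casts player 0's controller to GMC_Controller and adds the HOTAS and keyboard/mouse mapping contexts, with HOTAS at higher priority.
; The OpenMap action uses a FlipFlop to send alternating show and hide ToggleMapMessage calls to the HUD.
; A gamepad mapping context node exists but is left unconnected.
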(event Input|EnhancedActionEvents|EnhancedInputActionOpenMap
  (params (ActionValue :type Boolean) (ElapsedSeconds :type Float%20%28double-precision%29) (TriggeredSeconds :type Float%20%28double-precision%29) (InputAction :type Input%20Action%20Object%20Reference :default "/Game/Input/Actions/OpenMap.OpenMap"))
  (bind _returnvalue (Game|GetPlayerController 0))
  (bind _returnvalue_2 (HUD|GetHUD _returnvalue))
  (:Started
    (Utilities|FlowControl|FlipFlop
      (:A
        (Class|HUDDataRedist|ToggleMap(Message) _returnvalue_2 true))
      (:B
        (Class|HUDDataRedist|ToggleMap(Message) _returnvalue_2 false)))))

(event EventBeginPlay
  (bind _returnvalue (Game|Player|GetPlayerPawn 0))
  (Utilities|IsValid _returnvalue
    (:Is%20Valid
      (bind _asgmc_controller (Utilities|Casting|CastToGMC_Controller (Pawn|GetController _returnvalue)))
      (Utilities|IsValid (PlayerController|LocalPlayerSubsystems|GetEnhancedInputLocalPlayerSubsystem _asgmc_controller)
        (:Is%20Valid
          (Input|AddMappingContext (PlayerController|LocalPlayerSubsystems|GetEnhancedInputLocalPlayerSubsystem _asgmc_controller) "/Game/Input/HOTAS.HOTAS" 2 "(bIgnoreAllPressedKeysUntilRelease=True,bForceImmediately=False)")
          (Input|AddMappingContext (PlayerController|LocalPlayerSubsystems|GetEnhancedInputLocalPlayerSubsystem _asgmc_controller) "/Game/Input/KBM.KBM" 0 "(bIgnoreAllPressedKeysUntilRelease=True,bForceImmediately=False)"))))))

(fn ConstructionScript)