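; Base bomb actor dropped by a BP_Aircraft2, dealing radial area damage when it hits after arming.
; On fire it takes the aircraft's missile lock target if valid, detaches, passes the aircraft's speed to its GenBomb movement and primes after a short delay.
; A primed hit spawns an explosion and routes damage to overlapping sphere actors through RPC events, skipping "Weapon" tags.
; BlastRadius scales both the damage sphere and the effect.
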(event Custom|BombFireM
  (bind _playerref (Variables|Default|GetPlayerRef))
  (bind _locktargetmissile (Variables|/Game/Blueprints/AircraftBaseClass/BP_Aircraft2.BP_Aircraft2_C|GetLockTargetMissile _playerref))
  (Utilities|IsValid _locktargetmissile
    (:Is%20Valid
      (Variables|Default|SetCurrentTarget _locktargetmissile))
    (:Is%20Not%20Valid
      _))
  (Rendering|SetVisibility (Variables|Default|GetWidget) true true)
  (Transformation|DetachFromActor "KeepWorld" "KeepWorld" "KeepWorld")
  (Variables|/Game/Blueprints/BombBaseClass/GenBomb1.GenBomb1_C|SetCurrent%20Speed%20M (Variables|Default|GetGenBomb1) (Variables|/Game/Blueprints/AircraftBaseClass/BP_Aircraft2.BP_Aircraft2_C|GetCurrentSpeed (Variables|Default|GetPlayerRef)))
  (Components|Activation|Activate (Variables|Default|GetGenBomb1) false)
  (Utilities|FlowControl|Delay 1.0)
  (Variables|Default|SetPrimed true))

(event Custom|RPC_Damage
  (params (NewParam :type Actor%20Object%20Reference))
  (Utilities|IsValid NewParam
    (:Is%20Valid
      (if (not (Actor|ActorHasTag NewParam "Weapon"))
        (Game|Damage|ApplyDamage NewParam (Variables|Default|GetBaseDamage) (Pawn|GetController (Game|GetInstigator)) (Game|GetInstigator) "/Game/Blueprints/MainSystem/StandardDamage.StandardDamage_C")))))

(event Custom|RPC_Server_Damage
  (params (OtherActor :type Actor%20Object%20Reference))
  (CallFunction|RPCDamage OtherActor))

(event EventBeginPlay
  (bind _blastradius (Variables|Default|GetBlastRadius))
  (bind _asbp_aircraft_2 (Utilities|Casting|CastToBP_Aircraft2 (Game|GetInstigator)))
  (Variables|Default|SetPlayerRef _asbp_aircraft_2)
  (Transformation|SetRelativeScale3D (Variables|Default|GetSphere1) (Math|Vector|MakeVector _blastradius _blastradius _blastradius)))

(event Collision|EventHit
  (params (MyComp :type Primitive%20Component%20Object%20Reference) (Other :type Actor%20Object%20Reference) (OtherComp :type Primitive%20Component%20Object%20Reference) (bSelfMoved :type Boolean) (HitLocation :type Vector :default "0, 0, 0") (HitNormal :type Vector :default "0, 0, 0") (NormalImpulse :type Vector :default "0, 0, 0") (Hit :type Hit%20Result%20Structure%20%28by%20ref%29))
  (if (Variables|Default|GetPrimed)
    (CallFunction|Explode)))

(fn ConstructionScript)

(fn Explode
  (bind _blastradius (Variables|Default|GetBlastRadius))
  (bind _returnvalue (* _blastradius 0.1))
  (Niagara|SpawnSystematLocation "/Niagara/DefaultAssets/Templates/Systems/SimpleExplosion.SimpleExplosion" (Transformation|GetActorLocation) "0, 0, 0" (Math|Vector|MakeVector _returnvalue _returnvalue _returnvalue))
  (for _array_element (Collision|GetOverlappingActors (Variables|Default|GetSphere1) "/Script/Engine.Actor" :!class /Script/Engine.PrimitiveComponent)
    (CallFunction|RPCServerDamage _array_element))
  (Components|Activation|Deactivate (Variables|Default|GetGenBomb1))
  (Actor|DestroyActor))