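; GMC movement component for the Bomb pawn, predicting and replicating its fall and impact response.
; Each prediction tick applies gravity and sweeps the move; blocking hits adjust velocity, move again and count down HomingDelay, setting IsHoming once it reaches zero.
; Speed, target, bomb and homing state are bound for server-authoritative replication.
; The homing and nose-down steering branches, including the FollowTarget call, are disconnected, so IsHoming currently has no effect on movement here.
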(event EventBindReplicationData
  (|CallParentFunction)
  (Class|GMCReplicationCmp|BindDoublePrecisionFloat (Variables|Default|GetCurrentSpeedM) "ServerAuth_Output_ServerValidated" "AlwaysCombine" "Periodic_Output" "NearestNeighbour")
  (Class|GMCReplicationCmp|BindDoublePrecisionFloat (Variables|Default|GetSpeedMultiplier) "ServerAuth_Output_ServerValidated" "AlwaysCombine" "Periodic_Output" "NearestNeighbour")
  (Class|GMCReplicationCmp|BindActorReference (Variables|Default|GetCurrent%20Target) "ServerAuth_Output_ClientValidated" "AlwaysCombine" "Periodic_Output" "NearestNeighbour")
  (Class|GMCReplicationCmp|BindActorReference (Variables|Default|GetAs%20Bomb) "ServerAuth_Output_ClientValidated" "AlwaysCombine" "Periodic_Output" "NearestNeighbour")
  (Class|GMCReplicationCmp|BindBool (Variables|Default|GetIsHoming) "ServerAuth_Output_ClientValidated" "AlwaysCombine" "Periodic_Output" "NearestNeighbour")
  (Class|GMCReplicationCmp|BindDoublePrecisionFloat (Variables|Default|GetHomingDelay) "ServerAuth_Output_ClientValidated" "AlwaysCombine" "Periodic_Output" "NearestNeighbour"))

(event EventGenPredictionTick
  (params (DeltaTime :type Float%20%28single-precision%29))
  (bind _returnvalue (Class|GMCMovementUtilityCmp|GetPhysDeltaTime))
  (Class|GMCMovementUtilityCmp|AddAcceleration (* (Math|Vector|VectorDown) 9.8e+02) DeltaTime)
  (bind _outhit (Class|MovementComponent|MoveUpdatedComponent (* (Class|GMCReplicationCmp|GetVelocity) (Class|GMCMovementUtilityCmp|GetPhysDeltaTime)) (Class|GMCMovementUtilityCmp|GetRootCollisionRotation) true))
  (if (.bBlockingHit (Collision|BreakHitResult _outhit))
    (Class|GMCMovementUtilityCmp|AdjustVelocityfromHit _outhit true _returnvalue)
    (Class|MovementComponent|MoveUpdatedComponent (* (Class|GMCReplicationCmp|GetVelocity) _returnvalue) (Class|GMCMovementUtilityCmp|GetRootCollisionRotation) true)
    (if (== (Variables|Default|GetHomingDelay) 0.0)
      (Utilities|FlowControl|DoOnce false
        (:Completed
          (Variables|Default|SetIsHoming true)))
      (else
        (Variables|Default|SetHomingDelay (Math|Float|Clamp(Float) (- (Variables|Default|GetHomingDelay) (Class|GMCMovementUtilityCmp|GetPhysDeltaTime)) 0.0 1e+01))))))

(event EventBeginPlay
  (bind _asbomb (Utilities|Casting|CastToBomb (Components|GetOwner)))
  (Variables|Default|SetAs%20Bomb _asbomb))

(fn FollowTarget
  (params (Turnspeed :type Float%20%28double-precision%29))
  (bind _returnvalue (Components|GetOwner))
  (bind _as_bomb (Variables|Default|GetAs%20Bomb))
  (bind _returnvalue_2 (Transformation|GetActorTransform _returnvalue))
  (bind _currenttarget (Variables|/Game/Blueprints/BombBaseClass/Bomb.Bomb_C|GetCurrentTarget _as_bomb))
  (Utilities|IsValid _currenttarget
    (:Is%20Valid
      (Transformation|SetActorRotation (Components|GetOwner) (Math|Rotator|Lerp(Rotator) (.rotation _returnvalue_2) (Math|Rotator|FindLookatRotation (.location _returnvalue_2) (Transformation|GetActorLocation _currenttarget)) 0.1 true)))
    (:Is%20Not%20Valid
      _))
  (return))