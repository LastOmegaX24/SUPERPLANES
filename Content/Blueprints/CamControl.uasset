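; CamControl is the player's flight-control pawn, handling Enhanced Input, the HUD and camera rotation for a spawned X42AMagic_CamControl craft.
; Clamped roll, pitch and yaw inputs are interpolated each tick into local camera rotations, while the pawn's location follows the craft's camera.
; It stores speed, ability and landing-gear inputs, fires spread bullets from two muzzles, and toggles a sphere-trace radar lock with a marker actor.
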(event Input|EnhancedActionEvents|EnhancedInputActionPitch
  (params (ActionValue :type Float%20%28double-precision%29) (ElapsedSeconds :type Float%20%28double-precision%29) (TriggeredSeconds :type Float%20%28double-precision%29) (InputAction :type Input%20Action%20Object%20Reference :default "/Game/Input/Actions/Pitch.Pitch"))
  (bind _maxlook (Variables|Default|GetMaxLook))
  (bind _returnvalue (* _maxlook 2.0))
  (:Triggered
    (Variables|Default|SetTargetPitch (Math|Float|ClampAngle ActionValue (* _returnvalue -1.0) _returnvalue) :!label _label)
    (Variables|Default|SetIsPitch true))
  (:Ongoing
    (goto _label))
  (:Canceled
    (Variables|Default|SetTargetPitch (Math|Interpolation|FInterpTo (Variables|Default|GetTargetPitch) 0.0 (Utilities|Time|GetWorldDeltaSeconds) 0.0) :!label _label_2)
    (Variables|Default|SetIsPitch false))
  (:Completed
    (goto _label_2)))

(event Input|EnhancedActionEvents|EnhancedInputActionYaw
  (params (ActionValue :type Float%20%28double-precision%29) (ElapsedSeconds :type Float%20%28double-precision%29) (TriggeredSeconds :type Float%20%28double-precision%29) (InputAction :type Input%20Action%20Object%20Reference :default "/Game/Input/Actions/Yaw.Yaw"))
  (bind _maxlook (Variables|Default|GetMaxLook))
  (bind _returnvalue (* _maxlook 1.2))
  (:Triggered
    (Variables|Default|SetTargetYaw (Math|Float|ClampAngle ActionValue (* _returnvalue -1.0) _returnvalue) :!label _label)
    (Variables|Default|SetIsYaw true))
  (:Ongoing
    (goto _label))
  (:Canceled
    (Variables|Default|SetTargetYaw (Math|Interpolation|FInterpTo (Variables|Default|GetTargetYaw) 0.0 (Utilities|Time|GetWorldDeltaSeconds) 0.0) :!label _label_2)
    (Variables|Default|SetIsYaw false))
  (:Completed
    (goto _label_2)))

(event Input|EnhancedActionEvents|EnhancedInputActionRoll
  (params (ActionValue :type Float%20%28double-precision%29) (ElapsedSeconds :type Float%20%28double-precision%29) (TriggeredSeconds :type Float%20%28double-precision%29) (InputAction :type Input%20Action%20Object%20Reference :default "/Game/Input/Actions/Roll.Roll"))
  (bind _maxlook (Variables|Default|GetMaxLook))
  (bind _returnvalue (* _maxlook 0.35))
  (:Triggered
    (Variables|Default|SetTargetRoll (Math|Float|ClampAngle ActionValue (* _returnvalue -1.0) _returnvalue) :!label _label)
    (Variables|Default|SetIsRoll true))
  (:Ongoing
    (goto _label))
  (:Canceled
    (Variables|Default|SetTargetRoll (Math|Interpolation|FInterpTo (Variables|Default|GetTargetRoll) 0.0 (Utilities|Time|GetWorldDeltaSeconds) 0.0) :!label _label_2)
    (Variables|Default|SetIsRoll false))
  (:Completed
    (goto _label_2)))

(event Input|EnhancedActionEvents|EnhancedInputActionAccelerateDecelerate
  (params (ActionValue :type Float%20%28double-precision%29) (ElapsedSeconds :type Float%20%28double-precision%29) (TriggeredSeconds :type Float%20%28double-precision%29) (InputAction :type Input%20Action%20Object%20Reference :default "/Game/Input/Actions/AccelerateDecelerate.AccelerateDecelerate"))
  (:Triggered
    (Variables|Default|SetSendSpeedData ActionValue)))

(event Input|EnhancedActionEvents|EnhancedInputActionAbility
  (params (ActionValue :type Boolean) (ElapsedSeconds :type Float%20%28double-precision%29) (TriggeredSeconds :type Float%20%28double-precision%29) (InputAction :type Input%20Action%20Object%20Reference :default "/Game/Input/Actions/Ability.Ability"))
  (:Triggered
    (bind _isa (Utilities|FlowControl|FlipFlop)
      (:A
        _)
      (:B
        _))
    (Variables|Default|SetIs%20in%20Ability _isa)))

(event Input|EnhancedActionEvents|EnhancedInputActionFire
  (params (ActionValue :type Boolean) (ElapsedSeconds :type Float%20%28double-precision%29) (TriggeredSeconds :type Float%20%28double-precision%29) (InputAction :type Input%20Action%20Object%20Reference :default "/Game/Input/Actions/Fire.Fire"))
  (:Triggered
    (Utilities|FlowControl|Delay 0.01 :!label _label)
    (CallFunction|GunFire))
  (:Ongoing
    (goto _label)))

(event Input|EnhancedActionEvents|EnhancedInputActionLandingGear
  (params (ActionValue :type Boolean) (ElapsedSeconds :type Float%20%28double-precision%29) (TriggeredSeconds :type Float%20%28double-precision%29) (InputAction :type Input%20Action%20Object%20Reference :default "/Game/Input/Actions/LandingGear.LandingGear"))
  (:Triggered
    (bind _isa (Utilities|FlowControl|FlipFlop)
      (:A
        _)
      (:B
        _))
    (Variables|Default|SetIsLandingGear _isa)))

(event Input|EnhancedActionEvents|EnhancedInputActionFreeCam
  (params (ActionValue :type Boolean) (ElapsedSeconds :type Float%20%28double-precision%29) (TriggeredSeconds :type Float%20%28double-precision%29) (InputAction :type Input%20Action%20Object%20Reference :default "/Game/Input/Actions/FreeCam.FreeCam")))

(event Input|EnhancedActionEvents|EnhancedInputActionLockTarget
  (params (ActionValue :type Boolean) (ElapsedSeconds :type Float%20%28double-precision%29) (TriggeredSeconds :type Float%20%28double-precision%29) (InputAction :type Input%20Action%20Object%20Reference :default "/Game/Input/Actions/LockTarget.LockTarget"))
  (:Triggered
    (CallFunction|Radar :!label _label))
  (:Ongoing
    (goto _label)))

(event EventBeginPlay
  (bind _returnvalue (Game|SpawnActorfromClass "/Game/Blueprints/X42AMagic_CamControl.X42AMagic_CamControl_C" (Transformation|GetActorTransform) "Undefined" 0 0))
  (Variables|Default|SetFollowTarget _returnvalue)
  (bind _asplayer_controller (Utilities|Casting|CastToPlayerController (Pawn|GetController)))
  (Utilities|IsValid (PlayerController|LocalPlayerSubsystems|GetEnhancedInputLocalPlayerSubsystem _asplayer_controller)
    (:Is%20Valid
      (Input|AddMappingContext (PlayerController|LocalPlayerSubsystems|GetEnhancedInputLocalPlayerSubsystem _asplayer_controller) "/Game/Input/NewInputMappingContext.NewInputMappingContext" 0 "(bIgnoreAllPressedKeysUntilRelease=True,bForceImmediately=False)")
      (bind _returnvalue_2 (UserInterface|CreateWidget "/Game/HUD/HUD_Widget.HUD_Widget_C"))
      (UserInterface|Viewport|AddtoViewport _returnvalue_2 0))))

(event EventTick
  (params (DeltaSeconds :type Float%20%28single-precision%29))
  (bind _followtarget (Variables|Default|GetFollowTarget))
  (bind _camera (Variables|/Game/Blueprints/X42AMagic_CamControl.X42AMagic_CamControl_C|GetCamera _followtarget))
  (bind _returnvalue (Transformation|GetWorldTransform _camera))
  (CallFunction|RollF)
  (CallFunction|PitchF)
  (CallFunction|YawF)
  (Utilities|IsValid _followtarget
    (:Is%20Valid
      (Transformation|SetActorTransform (Math|Transform|MakeTransform (.location _returnvalue) "0, 0, 0" (.scale _returnvalue))))))

(fn ConstructionScript)

(fn PitchF
  (bind _output_get (Variables|Default|SetCurrentPitch (Math|Interpolation|FInterpTo (Variables|Default|GetCurrentPitch) (Variables|Default|GetTargetPitch) (Utilities|Time|GetWorldDeltaSeconds) (Variables|Default|GetInterp%20Speed))))
  (Variables|Default|SetPitchRec (* _output_get (Variables|Default|GetTurnspeed) 1.0))
  (Transformation|AddLocalRotation (Variables|Default|GetCamera) (Math|Rotator|MakeRotator 0.0 (* _output_get (Variables|Default|GetTurnspeed) 1.0) 0.0) false false))

(fn YawF
  (bind _output_get (Variables|Default|SetCurrentYaw (Math|Interpolation|FInterpTo (Variables|Default|GetCurrentYaw) (Variables|Default|GetTargetYaw) (Utilities|Time|GetWorldDeltaSeconds) (Variables|Default|GetInterp%20Speed))))
  (Variables|Default|SetYawRec (* _output_get (Variables|Default|GetTurnspeed) 1.0))
  (Transformation|AddLocalRotation (Variables|Default|GetCamera) (Math|Rotator|MakeRotator 0.0 0.0 (* _output_get (Variables|Default|GetTurnspeed) 1.0)) false false))

(fn RollF
  (bind _output_get (Variables|Default|SetCurrentRoll (Math|Interpolation|FInterpTo (Variables|Default|GetCurrentRoll) (Variables|Default|GetTargetRoll) (Utilities|Time|GetWorldDeltaSeconds) (Variables|Default|GetInterp%20Speed))))
  (Variables|Default|SetRollRec (* _output_get 5.0))
  (Transformation|AddLocalRotation (Variables|Default|GetCamera) (Math|Rotator|MakeRotator (* _output_get 5.0) 0.0 0.0) false false))

(fn RollRe
  (bind _camera (Variables|Default|GetCamera))
  (bind _returnvalue (Transformation|GetSocketRotation _camera "None"))
  (if (not (Variables|Default|GetIsRoll))
    (Transformation|SetRelativeRotation (Variables|Default|GetCamera) (Math|Rotator|MakeRotator (.roll (Math|Interpolation|RInterpTo (Math|Rotator|MakeRotator (.roll _returnvalue) (.pitch _returnvalue) (.yaw _returnvalue)) "0, 0, 0" (Utilities|Time|GetWorldDeltaSeconds) 1.0)) (.pitch _returnvalue) (.yaw _returnvalue)) false false)))

(fn PitchRe
  (bind _camera (Variables|Default|GetCamera))
  (bind _returnvalue (Transformation|GetSocketRotation _camera "None"))
  (if (not (Variables|Default|GetIsPitch))
    (Transformation|SetRelativeRotation (Variables|Default|GetCamera) (Math|Rotator|MakeRotator (.roll _returnvalue) (.pitch (Math|Interpolation|RInterpTo (Math|Rotator|MakeRotator (.roll _returnvalue) (.pitch _returnvalue) (.yaw _returnvalue)) "0, 0, 0" (Utilities|Time|GetWorldDeltaSeconds) 1.0)) (.yaw _returnvalue)) false false)))

(fn YawRe
  (bind _camera (Variables|Default|GetCamera))
  (bind _returnvalue (Transformation|GetSocketRotation _camera "None"))
  (if (not (Variables|Default|GetIsYaw))
    (Transformation|SetRelativeRotation (Variables|Default|GetCamera) (Math|Rotator|MakeRotator (.roll _returnvalue) (.pitch _returnvalue) (.yaw (Math|Interpolation|RInterpTo (Math|Rotator|MakeRotator (.roll _returnvalue) (.pitch _returnvalue) (.yaw _returnvalue)) "0, 0, 0" (Utilities|Time|GetWorldDeltaSeconds) 1.0))) false false)))

(fn GunFire
  (bind _followtarget (Variables|Default|GetFollowTarget))
  (bind _firelocation1 (Variables|/Game/Blueprints/X42AMagic_CamControl.X42AMagic_CamControl_C|GetFireLocation1 _followtarget))
  (bind _firelocation2 (Variables|/Game/Blueprints/X42AMagic_CamControl.X42AMagic_CamControl_C|GetFireLocation2 _followtarget))
  (bind _returnvalue (Transformation|GetWorldTransform _firelocation1))
  (bind _returnvalue_2 (Transformation|GetWorldTransform _firelocation2))
  (Utilities|IsValid _followtarget
    (:Is%20Valid
      (Utilities|FlowControl|Sequence
        (:then_0
          (Game|SpawnActorfromClass "/Game/Blueprints/BP_Bullet.BP_Bullet_C" (Math|Transform|MakeTransform (.location _returnvalue) (Math|Rotator|MakeRotator (.roll (.rotation _returnvalue)) (+ (.pitch (.rotation _returnvalue)) (Math|Random|RandomFloatinRange -1.0 1.0)) (+ (.yaw (.rotation _returnvalue)) (Math|Random|RandomFloatinRange -1.0 1.0))) (.scale _returnvalue)) "AlwaysSpawn" 0 0))
        (:then_1
          (Game|SpawnActorfromClass "/Game/Blueprints/BP_Bullet.BP_Bullet_C" (Math|Transform|MakeTransform (.location _returnvalue_2) (Math|Rotator|MakeRotator (.roll (.rotation _returnvalue_2)) (+ (.pitch (.rotation _returnvalue_2)) (Math|Random|RandomFloatinRange -1.0 1.0)) (+ (.yaw (.rotation _returnvalue_2)) (Math|Random|RandomFloatinRange -1.0 1.0))) (.scale _returnvalue_2)) "AlwaysSpawn" 0 0))))))

(fn Radar
  (bind _followtarget (Variables|Default|GetFollowTarget))
  (bind _radarorigin (Variables|/Game/Blueprints/X42AMagic_CamControl.X42AMagic_CamControl_C|GetRadarOrigin _followtarget))
  (bind _returnvalue (Transformation|GetWorldLocation _radarorigin))
  (Variables|Default|GetTargetLockTracker
    (:then
      (Actor|DestroyActor (Variables|Default|GetTargetLockTracker)))
    (:else
      _))
  (Utilities|FlowControl|FlipFlop
    (:A
      (Variables|Default|SetIsTargetLocked true)
      (bind (_outhit _returnvalue_2) (Collision|SphereTraceForObjects _returnvalue (+ _returnvalue (* (Math|Vector|GetForwardVector (Transformation|GetWorldRotation _radarorigin)) (Variables|Default|GetRadarMaxRange))) (Variables|Default|GetRadarRadius) (Utilities|Array|MakeArray "ObjectTypeQuery3") false 0 "ForDuration"))
      (if _returnvalue_2
        (bind _output_get (Variables|Default|SetLockTarget (.HitActor (Collision|BreakHitResult _outhit))))
        (bind _returnvalue_3 (Game|SpawnActorfromClass "/Game/Blueprints/Target_Lock.Target_Lock_C" (Math|Transform|MakeTransform (Transformation|GetActorLocation _output_get) "0, 0, 0" "1.000000,1.000000,1.000000") "Undefined" 0 0))
        (Variables|Default|SetTargetLockTracker _returnvalue_3)))
    (:B
      (Variables|Default|SetIsTargetLocked false)
      (Variables|Default|SetLockTarget 0))))