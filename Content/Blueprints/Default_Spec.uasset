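; Default_Spec is a Blueprint that fires railgun projectiles while it has Ammo.
; FireCall passes an Index through a server-named RPC event to RPC_Railgun, which waits Index × 0.1 seconds to stagger shots.
; It then spawns BP_Railgun_Pr at the Arrow transform, owned by player controller 0, and decrements Ammo.
; With no ammo left, it sets IsEmpty to false.
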(event Custom|RPC_Railgun
  (params (Index :type Integer))
  (if (> (Variables|Default|GetAmmo) 0)
    (Utilities|FlowControl|Delay (* Index 0.1))
    (Game|SpawnActorfromClass "/Game/Blueprints/BP_Railgun_Pr.BP_Railgun_Pr_C" (Transformation|GetWorldTransform (Variables|Default|GetArrow)) "Undefined" (Game|GetPlayerController 0) (Game|Player|GetPlayerPawn 0))
    (Math|Integer|DecrementInt (Variables|Default|GetAmmo))
    (else
      (Variables|Default|SetIsEmpty false))))

(event Custom|RPC_Server_Railgun
  (params (Index :type Integer))
  (CallFunction|RPCRailgun Index))

(event Custom|FireCall
  (params (Index :type Integer))
  (CallFunction|RPCServerRailgun Index))

(fn ConstructionScript)