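; Drone actor that flies forward under a simple thrust and stall model and explodes when its health runs out.
; Each Tick, UpdatePosition clamps speed, easing down by Drag when thrust drops, maps it to a gravity pull for stalling, and applies a swept world offset.
; Damage lowers health until an explosion spawns and the actor is destroyed; pawn sensing only sets a SeePlayer flag.
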(event OnSeePawn(PawnSensing)
  (params (Pawn :type Pawn%20Object%20Reference))
  (Variables|Default|SetSeePlayer true))

(event EventTick
  (params (DeltaSeconds :type Float%20%28single-precision%29))
  (CallFunction|UpdatePosition DeltaSeconds DeltaSeconds))

(event EventBeginPlay)

(event Game|Damage|EventAnyDamage
  (params (Damage :type Float%20%28single-precision%29) (DamageType :type Damage%20Type%20Object%20Reference) (InstigatedBy :type Controller%20Object%20Reference) (DamageCauser :type Actor%20Object%20Reference))
  (bind _returnvalue (Transformation|GetActorTransform))
  (Variables|Default|SetHealth (Math|Float|Clamp(Float) (- (Variables|Default|GetHealth) Damage) 0.0 (Variables|Default|GetMaxHealth)))
  (if (<= (Variables|Default|GetHealth) 0.0)
    (Variables|Default|SetIsAlive false)
    (Effects|SpawnEmitteratLocation "/Game/StarterContent/Particles/P_Explosion.P_Explosion" (.location _returnvalue) (.rotation _returnvalue) "20.000000,20.000000,20.000000")
    (Actor|DestroyActor)))

(fn ConstructionScript)

(fn UpdatePosition
  (params (DeltaTime :type Float%20%28double-precision%29) (B :type Float%20%28single-precision%29))
  ;[1 1 1] Calc Current Speed
  (Variables|Default|SetCurrentSpeed (Math|Float|Clamp(Float) (select (< (Variables|Default|GetThrustSpeed) (Variables|Default|GetCurrentSpeed)) (Math|Interpolation|FInterpTo (Variables|Default|GetCurrentSpeed) (Variables|Default|GetThrustSpeed) DeltaTime (Variables|Default|GetDrag)) (Variables|Default|GetThrustSpeed)) 0.0 (Variables|Default|GetMaxThrustSpeed)))
  ;[1 1 1] Calc new position based on speed
  (Variables|Default|SetNewPos (* (* (Variables|Default|GetCurrentSpeed) B) (Transformation|GetActorForwardVector)))
  ;[1 1 1] Calc Applied Gravity
  (Variables|Default|SetAppliedGravity (Math|Float|MapRangeClamped (Variables|Default|GetCurrentSpeed) 0.0 (Variables|Default|GetMinThrustStall) (Variables|Default|GetGravity) 0.0))
  ;[1 1 1] Get Position
  (Transformation|AddActorWorldOffset (Math|Vector|MakeVector (.X (Class|KismetMathLibrary|BreakVector3f (Variables|Default|GetNewPos))) (.Y (Class|KismetMathLibrary|BreakVector3f (Variables|Default|GetNewPos))) (- (.Z (Class|KismetMathLibrary|BreakVector3f (Variables|Default|GetNewPos))) (* (Variables|Default|GetAppliedGravity) 1.0))) true))