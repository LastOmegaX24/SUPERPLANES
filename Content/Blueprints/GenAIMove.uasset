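; GenAIMove is a networked movement component, apparently for AI, that drives its owner straight along its forward vector.
; Each prediction tick updates velocity from that vector and CurrentSpeed, then does a swept move using the physics delta time, keeping root collision rotation.
; CurrentSpeed is bound for replication as a server-authoritative, validated value with periodic output, and nothing in this graph sets it.
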(event EventBindReplicationData
  (|CallParentFunction)
  (Class|GMCReplicationCmp|BindDoublePrecisionFloat (Variables|Default|GetCurrentSpeed) "ServerAuth_InputOutput_ServerValidated" "AlwaysCombine" "Periodic_Output" "NearestNeighbour"))

(event EventGenPredictionTick
  (params (DeltaTime :type Float%20%28single-precision%29))
  (Class|GMCMovementUtilityCmp|UpdateVelocity (* (Transformation|GetActorForwardVector (Components|GetOwner)) (Variables|Default|GetCurrentSpeed)) (Class|GMCMovementUtilityCmp|GetPhysDeltaTime))
  (Class|MovementComponent|MoveUpdatedComponent (* (Class|GMCReplicationCmp|GetVelocity) (Class|GMCMovementUtilityCmp|GetPhysDeltaTime)) (Class|GMCMovementUtilityCmp|GetRootCollisionRotation) true))