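; GenMissile is a replicated movement component, apparently built on the General Movement Component, that flies a homing missile once deployed.
; Each replicated tick turns the owner toward CurrentTarget at a constant rate, then eases speed toward ThrustSpeed using Drag, clamped to a maximum.
; It updates velocity and sweeps along the forward vector, with a move delta not scaled by DeltaTime and a look-at rotation computed without the target validity check.
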(event EventGenReplicatedTick
  (params (DeltaTime :type Float%20%28single-precision%29))
  (bind _returnvalue (Components|GetOwner))
  (bind _turnspeed (Variables|Default|GetTurnspeed))
  (bind _currenttarget (Variables|Default|GetCurrentTarget))
  (bind _returnvalue_2 (Transformation|GetActorRotation _returnvalue))
  (bind _returnvalue_3 (Transformation|GetActorLocation _returnvalue))
  (bind _returnvalue_4 (Transformation|GetActorLocation _currenttarget))
  (bind _returnvalue_5 (Math|Rotator|FindLookatRotation _returnvalue_3 _returnvalue_4))
  (bind _returnvalue_6 (Class|KismetMathLibrary|RInterptoConstant _returnvalue_2 _returnvalue_5 DeltaTime _turnspeed))
  (|CallParentFunction DeltaTime)
  (if (Variables|Default|GetIsDeployed)
    (Utilities|IsValid _currenttarget
      (:Is%20Valid
        (Transformation|SetActorRotation _returnvalue _returnvalue_6))
      (:Is%20Not%20Valid
        _))
    (Variables|Default|SetCurrentSpeed (Math|Float|Clamp(Float) (Math|Interpolation|FInterpTo (Variables|Default|GetCurrentSpeed) (Variables|Default|GetThrustSpeed) DeltaTime (Variables|Default|GetDrag)) 0.0 (Variables|Default|GetMaxThrustSpeed)))
    (Class|GenMovementComponent|UpdateVelocity (* (Transformation|GetActorForwardVector (Components|GetOwner)) (Variables|Default|GetCurrentSpeed)) DeltaTime)
    (Class|MovementComponent|MoveUpdatedComponent (* (Transformation|GetActorForwardVector (Components|GetOwner)) (Variables|Default|GetCurrentSpeed)) _returnvalue_6 true)))

(event EventBindReplicationData
  (|CallParentFunction))