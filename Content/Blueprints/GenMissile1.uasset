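; GMC movement component for the Missile3 actor that flies it forward as a fuel-limited homing missile with networked prediction.
; Each prediction tick eases speed toward thrust while fuel lasts, then decelerates with weakened turning, and sweeps the move.
; FollowTarget lerps rotation toward the missile's target, leading distant targets along their forward vector by speed and distance.
; Speed, fuel, thrust, multiplier and a target reference are bound as server-authoritative replication data.
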(event EventBindReplicationData
  (|CallParentFunction)
  (Class|GMCReplicationCmp|BindDoublePrecisionFloat (Variables|Default|GetCurrentSpeedM) "ServerAuth_Output_ServerValidated" "AlwaysCombine" "Periodic_Output" "NearestNeighbour")
  (Class|GMCReplicationCmp|BindDoublePrecisionFloat (Variables|Default|GetFuel) "ServerAuth_Output_ServerValidated" "AlwaysCombine" "Periodic_Output" "NearestNeighbour")
  (Class|GMCReplicationCmp|BindDoublePrecisionFloat (Variables|Default|GetThrustSpeedM) "ServerAuth_Output_ServerValidated" "AlwaysCombine" "Periodic_Output" "NearestNeighbour")
  (Class|GMCReplicationCmp|BindDoublePrecisionFloat (Variables|Default|GetSpeedMultiplier) "ServerAuth_Output_ServerValidated" "AlwaysCombine" "Periodic_Output" "NearestNeighbour")
  (Class|GMCReplicationCmp|BindActorReference (Variables|Default|GetCurrentTarget) "ServerAuth_Output_ClientValidated" "AlwaysCombine" "Periodic_Output" "NearestNeighbour"))

(event EventGenPredictionTick
  (params (DeltaTime :type Float%20%28single-precision%29))
  (if (> (Variables|Default|GetFuel) 0.0)
    (Variables|Default|SetCurrentSpeedM (Math|Interpolation|FInterpTo (Variables|Default|GetCurrentSpeedM) (Variables|Default|GetThrustSpeedM) DeltaTime 0.1))
    (Variables|Default|SetFuel (- (Variables|Default|GetFuel) DeltaTime))
    (CallFunction|FollowTarget (Variables|Default|GetTurnspeed))
    (else
      (Variables|Default|SetCurrentSpeedM (- (Variables|Default|GetCurrentSpeedM) (* DeltaTime 5.0)))
      (CallFunction|FollowTarget (* (Variables|Default|GetTurnspeed) 0.2))))
  (Class|GMCMovementUtilityCmp|UpdateVelocity (* (Transformation|GetActorForwardVector (Class|GMCReplicationCmp|GetGMCPawnOwner)) (Variables|Default|GetCurrentSpeedM) (Variables|Default|GetSpeedMultiplier)) (Class|GMCMovementUtilityCmp|GetPhysDeltaTime))
  (Class|MovementComponent|MoveUpdatedComponent (* (Class|GMCReplicationCmp|GetVelocity) (Class|GMCMovementUtilityCmp|GetPhysDeltaTime)) (Class|GMCMovementUtilityCmp|GetRootCollisionRotation) true))

(event EventBeginPlay
  (bind _asmissile_3 (Utilities|Casting|CastToMissile3 (Components|GetOwner)))
  (Variables|Default|SetAs%20Missile%203 _asmissile_3))

(fn FollowTarget
  (params (Turnspeed :type Float%20%28double-precision%29))
  (bind _returnvalue (Components|GetOwner))
  (bind _as_missile_3 (Variables|Default|GetAs%20Missile%203))
  (bind _returnvalue_2 (Transformation|GetActorTransform _returnvalue))
  (bind _currenttarget (Variables|/Game/Blueprints/Missile3.Missile3_C|GetCurrentTarget _as_missile_3))
  (bind _returnvalue_3 (Transformation|GetActorLocation _currenttarget))
  (bind _returnvalue_4 (Math|Vector|Distance(Vector) _returnvalue_3 (.location _returnvalue_2)))
  (Utilities|IsValid _currenttarget
    (:Is%20Valid
      (Transformation|SetActorRotation (Components|GetOwner) (Math|Rotator|Lerp(Rotator) (.rotation _returnvalue_2) (Math|Rotator|FindLookatRotation (.location _returnvalue_2) (select (< _returnvalue_4 1e+03) _returnvalue_3 (+ _returnvalue_3 (* (Transformation|GetActorForwardVector _currenttarget) (* (* (Math|Vector|VectorLength (Transformation|GetVelocity _currenttarget)) 0.01) (* _returnvalue_4 0.0005)))))) (* Turnspeed 1.0) true)))
    (:Is%20Not%20Valid
      _))
  (return))