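; GenMove is a GMC-style movement component that gives the Prototype_9_GMC pawn camera-led, six-axis-style flight rotation.
; Enhanced Input sets clamped roll, pitch and yaw targets, with optional speed-curve limits on pitch and yaw.
; Each replicated tick interpolates these into local camera rotation, while the pawn lerps toward the camera's orientation.
; AccelerateDecelerate sets a fixed velocity; thrust-and-drag speed logic is present but disconnected, and MovementUpdate is empty.
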(event Input|EnhancedActionEvents|EnhancedInputActionPitch
  (params (ActionValue :type Float%20%28double-precision%29) (ElapsedSeconds :type Float%20%28double-precision%29) (TriggeredSeconds :type Float%20%28double-precision%29) (InputAction :type Input%20Action%20Object%20Reference :default "/Game/Input/Actions/Pitch.Pitch"))
  (:Triggered
    (CallFunction|CamPitchF ActionValue :!label _label))
  (:Ongoing
    (goto _label))
  (:Canceled
    (CallFunction|CamPitchRecF :!label _label_2))
  (:Completed
    (goto _label_2)))

(event Input|EnhancedActionEvents|EnhancedInputActionYaw
  (params (ActionValue :type Float%20%28double-precision%29) (ElapsedSeconds :type Float%20%28double-precision%29) (TriggeredSeconds :type Float%20%28double-precision%29) (InputAction :type Input%20Action%20Object%20Reference :default "/Game/Input/Actions/Yaw.Yaw"))
  (:Triggered
    (CallFunction|CamYawF ActionValue :!label _label))
  (:Ongoing
    (goto _label))
  (:Canceled
    (CallFunction|CamYawRecF :!label _label_2))
  (:Completed
    (goto _label_2)))

(event Input|EnhancedActionEvents|EnhancedInputActionRoll
  (params (ActionValue :type Float%20%28double-precision%29) (ElapsedSeconds :type Float%20%28double-precision%29) (TriggeredSeconds :type Float%20%28double-precision%29) (InputAction :type Input%20Action%20Object%20Reference :default "/Game/Input/Actions/Roll.Roll"))
  (:Triggered
    (CallFunction|CamRollF ActionValue :!label _label))
  (:Ongoing
    (goto _label))
  (:Canceled
    (CallFunction|CamRollRecF :!label _label_2))
  (:Completed
    (goto _label_2)))

(event Input|EnhancedActionEvents|EnhancedInputActionAccelerateDecelerate
  (params (ActionValue :type Float%20%28double-precision%29) (ElapsedSeconds :type Float%20%28double-precision%29) (TriggeredSeconds :type Float%20%28double-precision%29) (InputAction :type Input%20Action%20Object%20Reference :default "/Game/Input/Actions/AccelerateDecelerate.AccelerateDecelerate"))
  (:Triggered
    (Class|GenMovementReplicationComponent|SetVelocity (Math|Vector|MakeVector 1.11e+03 1.11e+03 1.11e+03))))

(event EventBindReplicationData
  (|CallParentFunction))

(event EventBeginPlay
  (bind _asgen_controller (Utilities|Casting|CastToGEN_Controller (Game|GetPlayerController 0)))
  (Utilities|IsValid (PlayerController|LocalPlayerSubsystems|GetEnhancedInputLocalPlayerSubsystem _asgen_controller)
    (:Is%20Valid
      (Input|AddMappingContext (PlayerController|LocalPlayerSubsystems|GetEnhancedInputLocalPlayerSubsystem _asgen_controller) "/Game/Input/NewInputMappingContext.NewInputMappingContext" 0 "(bIgnoreAllPressedKeysUntilRelease=True,bForceImmediately=False)")
      (bind _asprototype_9_gmc (Utilities|Casting|CastToPrototype_9_GMC (Game|Player|GetPlayerPawn 0)))
      (bind _output_get (Variables|Default|SetPlayerPawnRef _asprototype_9_gmc))
      (Variables|Default|SetP_Camera (Variables|/Game/Blueprints/Prototype_9_GMC.Prototype_9_GMC_C|GetCamera _output_get)))))

(event EventMovementUpdate
  (params (DeltaSeconds :type Float%20%28single-precision%29)))

(event EventGenReplicatedTick
  (params (DeltaTime :type Float%20%28single-precision%29))
  (bind _output_get (Variables|Default|SetDeltaSeconds DeltaTime))
  (Transformation|SetWorldRotation (Variables|/Game/Blueprints/Prototype_9_GMC.Prototype_9_GMC_C|Getcamroot (Variables|Default|GetPlayerPawnRef)) "0, 0, 0" false false)
  (CallFunction|CopyRot)
  (CallFunction|RollF)
  (CallFunction|PitchF)
  (CallFunction|YawF)
  (Class|GenOrganicMovementComponent|ApplyRotation false _output_get))

(fn CamRollF
  (params (AngleDegrees :type Float%20%28double-precision%29))
  (bind _maxlook (Variables|Default|GetMaxLook))
  (bind _returnvalue (* _maxlook 0.35))
  (Variables|Default|SetTargetRoll (Math|Float|ClampAngle AngleDegrees (* _returnvalue -1.0) _returnvalue)))

(fn CamRollRecF
  (Variables|Default|SetTargetRoll (Math|Interpolation|FInterpTo (Variables|Default|GetTargetRoll) 0.0 (Variables|Default|GetDeltaSeconds) 0.0)))

(fn CamPitchF
  (params (AngleDegrees :type Float%20%28double-precision%29))
  (bind _currentspeed (Variables|Default|GetCurrentSpeed))
  (bind _maxlook (Variables|Default|GetMaxLook))
  (bind _fcslimit (Variables|Default|GetFCSLimit))
  (bind _rotationcurve (Variables|Default|GetRotationCurve))
  (bind _returnvalue (Math|Curves|GetFloatValue _rotationcurve _currentspeed))
  (bind _returnvalue_2 (Math|Float|Clamp(Float) _returnvalue 0.1))
  (bind _returnvalue_3 (select _fcslimit _returnvalue_2 _maxlook))
  (bind _returnvalue_4 (* _returnvalue_3 2.0))
  (Variables|Default|SetTargetPitch (Math|Float|ClampAngle AngleDegrees (* _returnvalue_4 -1.0) _returnvalue_4)))

(fn CamPitchRecF
  (Variables|Default|SetTargetPitch (Math|Interpolation|FInterpTo (Variables|Default|GetTargetPitch) 0.0 (Variables|Default|GetDeltaSeconds) 0.0)))

(fn CamYawF
  (params (AngleDegrees :type Float%20%28double-precision%29))
  (bind _currentspeed (Variables|Default|GetCurrentSpeed))
  (bind _maxlook (Variables|Default|GetMaxLook))
  (bind _fcslimit (Variables|Default|GetFCSLimit))
  (bind _rotationcurve (Variables|Default|GetRotationCurve))
  (bind _returnvalue (Math|Curves|GetFloatValue _rotationcurve _currentspeed))
  (bind _returnvalue_2 (Math|Float|Clamp(Float) _returnvalue 0.1))
  (bind _returnvalue_3 (select _fcslimit _returnvalue_2 _maxlook))
  (bind _returnvalue_4 (* _returnvalue_3 1.2))
  (Variables|Default|SetTargetYaw (Math|Float|ClampAngle AngleDegrees (* _returnvalue_4 -1.0) _returnvalue_4)))

(fn CamYawRecF
  (Variables|Default|SetTargetYaw (Math|Interpolation|FInterpTo (Variables|Default|GetTargetYaw) 0.0 (Variables|Default|GetDeltaSeconds) 0.0)))

(fn CopyRot
  (bind _p_camera (Variables|Default|GetP_Camera))
  (bind _returnvalue (Transformation|GetSocketRotation _p_camera "None"))
  (Utilities|IsValid _p_camera
    (:Is%20Valid
      (Variables|Default|SetTargetRotation (Math|Rotator|MakeRotator (.roll (Math|Rotator|Lerp(Rotator) (Math|Rotator|MakeRotator (.roll (Variables|Default|GetTargetRotation)) 0.0 0.0) (Math|Rotator|MakeRotator (.roll _returnvalue) 0.0 0.0) (Utilities|TurnspeedMacro) true)) (.pitch (Math|Rotator|Lerp(Rotator) (Math|Rotator|MakeRotator 0.0 (.pitch (Variables|Default|GetTargetRotation)) 0.0) (Math|Rotator|MakeRotator 0.0 (.pitch _returnvalue) 0.0) (Utilities|TurnspeedMacro) true)) (.yaw (Math|Rotator|Lerp(Rotator) (Math|Rotator|MakeRotator 0.0 0.0 (.yaw (Variables|Default|GetTargetRotation))) (Math|Rotator|MakeRotator 0.0 0.0 (.yaw _returnvalue)) (Utilities|TurnspeedMacro) true))))
      (Transformation|SetActorRotation (Variables|Default|GetPlayerPawnRef) (Math|Rotator|Lerp(Rotator) (Transformation|GetActorRotation (Game|Player|GetPlayerPawn 0)) (Variables|Default|GetTargetRotation) 0.05 true)))))

(fn UpdateSpeed
  (params (DeltaTime :type Float%20%28double-precision%29))
  (bind _output_get (Variables|Default|SetCurrentSpeed (Math|Interpolation|FInterpTo (Variables|Default|GetCurrentSpeed) (Variables|Default|GetThrustSpeed) DeltaTime (Variables|Default|GetDrag))))
  (Class|GenMovementReplicationComponent|SetVelocity (* (* _output_get DeltaTime) (Transformation|GetActorForwardVector (Game|Player|GetPlayerPawn 0)))))

(fn RollF
  (bind _output_get (Variables|Default|SetCurrentRoll (Math|Interpolation|FInterpTo (Variables|Default|GetCurrentRoll) (Variables|Default|GetTargetRoll) (Variables|Default|GetDeltaSeconds) (Variables|Default|GetInterp%20Speed))))
  (Transformation|AddLocalRotation (Variables|Default|GetP_Camera) (Math|Rotator|MakeRotator (* _output_get 5.0) 0.0 0.0) false false))

(fn PitchF
  (bind _output_get (Variables|Default|SetCurrentPitch (Math|Interpolation|FInterpTo (Variables|Default|GetCurrentPitch) (Variables|Default|GetTargetPitch) (Variables|Default|GetDeltaSeconds) (Variables|Default|GetInterp%20Speed))))
  (Transformation|AddLocalRotation (Variables|Default|GetP_Camera) (Math|Rotator|MakeRotator 0.0 (* _output_get (Variables|Default|GetTurnspeed) 1.0) 0.0) false false))

(fn YawF
  (bind _output_get (Variables|Default|SetCurrentYaw (Math|Interpolation|FInterpTo (Variables|Default|GetCurrentYaw) (Variables|Default|GetTargetYaw) (Variables|Default|GetDeltaSeconds) (Variables|Default|GetInterp%20Speed))))
  (Transformation|AddLocalRotation (Variables|Default|GetP_Camera) (Math|Rotator|MakeRotator 0.0 0.0 (* _output_get (Variables|Default|GetTurnspeed) 1.0)) false false))