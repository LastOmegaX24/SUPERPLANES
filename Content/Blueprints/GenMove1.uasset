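; GMC movement component for BP_Aircraft2 that drives predicted, networked aircraft flight from Enhanced Input.
; Prediction tick eases roll, pitch and yaw toward input, applies local rotation, then eases speed toward thrust, adding a gravity term below stall and adjusting velocity on hits.
; Landed mode allows only yaw and caps speed at stall; dead aircraft nose down.
; FCS limit scales pitch by a speed curve; camera-follow steering helpers are unused.
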(event Custom|Dash
  (Variables|Default|SetIsDash true)
  (Utilities|FlowControl|Delay 0.6)
  (Variables|Default|SetIsDash false))

(event Input|EnhancedActionEvents|EnhancedInputActionPitch
  (params (ActionValue :type Float%20%28double-precision%29) (ElapsedSeconds :type Float%20%28double-precision%29) (TriggeredSeconds :type Float%20%28double-precision%29) (InputAction :type Input%20Action%20Object%20Reference :default "/Game/Input/Actions/Pitch.Pitch"))
  (:Triggered
    (Variables|Default|SetTargetPitch (Math|Float|Clamp(Float) ActionValue -1.0)))
  (:Canceled
    (Variables|Default|SetTargetPitch 0.0 :!label _label))
  (:Completed
    (goto _label)))

(event Input|EnhancedActionEvents|EnhancedInputActionYaw
  (params (ActionValue :type Float%20%28double-precision%29) (ElapsedSeconds :type Float%20%28double-precision%29) (TriggeredSeconds :type Float%20%28double-precision%29) (InputAction :type Input%20Action%20Object%20Reference :default "/Game/Input/Actions/Yaw.Yaw"))
  (:Triggered
    (Variables|Default|SetTargetYaw (Math|Float|Clamp(Float) ActionValue -1.0)))
  (:Canceled
    (Variables|Default|SetTargetYaw 0.0 :!label _label))
  (:Completed
    (goto _label)))

(event Input|EnhancedActionEvents|EnhancedInputActionRoll
  (params (ActionValue :type Float%20%28double-precision%29) (ElapsedSeconds :type Float%20%28double-precision%29) (TriggeredSeconds :type Float%20%28double-precision%29) (InputAction :type Input%20Action%20Object%20Reference :default "/Game/Input/Actions/Roll.Roll"))
  (:Triggered
    (Variables|Default|SetTargetRoll (Math|Float|Clamp(Float) ActionValue -1.0)))
  (:Canceled
    (Variables|Default|SetTargetRoll 0.0 :!label _label))
  (:Completed
    (goto _label)))

(event Input|EnhancedActionEvents|EnhancedInputActionAccelerateDecelerate
  (params (ActionValue :type Float%20%28double-precision%29) (ElapsedSeconds :type Float%20%28double-precision%29) (TriggeredSeconds :type Float%20%28double-precision%29) (InputAction :type Input%20Action%20Object%20Reference :default "/Game/Input/Actions/AccelerateDecelerate.AccelerateDecelerate"))
  (:Triggered
    (CallFunction|Speed0 ActionValue (Class|GMCMovementUtilityCmp|GetPhysDeltaTime) :!label _label))
  (:Ongoing
    (goto _label)))

(event Input|EnhancedActionEvents|EnhancedInputActionFCSMode
  (params (ActionValue :type Boolean) (ElapsedSeconds :type Float%20%28double-precision%29) (TriggeredSeconds :type Float%20%28double-precision%29) (InputAction :type Input%20Action%20Object%20Reference :default "/Game/Input/Actions/FCSMode.FCSMode"))
  (:Triggered
    (Variables|Default|SetFCSLimit false)
    (Variables|Default|SetPitchM 7.0))
  (:Canceled
    (Variables|Default|SetFCSLimit true :!label _label)
    (Variables|Default|SetPitchM 5.0))
  (:Completed
    (goto _label)))

(event Input|EnhancedActionEvents|EnhancedInputActionLandingGear
  (params (ActionValue :type Boolean) (ElapsedSeconds :type Float%20%28double-precision%29) (TriggeredSeconds :type Float%20%28double-precision%29) (InputAction :type Input%20Action%20Object%20Reference :default "/Game/Input/Actions/LandingGear.LandingGear"))
  (:Started
    (Utilities|FlowControl|FlipFlop
      (:A
        (Variables|Default|SetLandingGear false))
      (:B
        (Variables|Default|SetLandingGear true)))))

(event EventGenPredictionTick
  (params (DeltaTime :type Float%20%28single-precision%29))
  (if (Variables|Default|GetIsLanded)
    (if (Variables|/Game/Blueprints/BP_Aircraft2.BP_Aircraft2_C|GetIsAlive (Variables|Default|GetPlayerPawnRef))
      (if true
        _
        (else
          (Variables|Default|SetIsLanded false)
          (CallFunction|PitchF)))
      (CallFunction|YawF)
      (CallFunction|ControlAdd)
      (CallFunction|UpdatePositionGround DeltaTime)
      (bind _outhit (Class|MovementComponent|MoveUpdatedComponent (* (Class|GMCReplicationCmp|GetVelocity) (Class|GMCMovementUtilityCmp|GetPhysDeltaTime) 1.0) (Class|GMCMovementUtilityCmp|GetRootCollisionRotation) true))
      (if (.bBlockingHit (Collision|BreakHitResult _outhit))
        (Class|GMCMovementUtilityCmp|AdjustVelocityfromHit _outhit false 0.0)
        (Class|MovementComponent|MoveUpdatedComponent (* (Class|GMCReplicationCmp|GetVelocity) (Class|GMCMovementUtilityCmp|GetPhysDeltaTime) 1.0) (Class|GMCMovementUtilityCmp|GetRootCollisionRotation) true)))
    (elif (Variables|/Game/Blueprints/BP_Aircraft2.BP_Aircraft2_C|GetIsAlive (Variables|Default|GetPlayerPawnRef))
      (CallFunction|RollF)
      (CallFunction|PitchF)
      (CallFunction|YawF)
      (CallFunction|ControlAdd)
      (CallFunction|UpdatePosition DeltaTime)
      (bind _outhit_2 (Class|MovementComponent|MoveUpdatedComponent (* (Class|GMCReplicationCmp|GetVelocity) (Class|GMCMovementUtilityCmp|GetPhysDeltaTime)) (Class|GMCMovementUtilityCmp|GetRootCollisionRotation) true))
      (if (.bBlockingHit (Collision|BreakHitResult _outhit_2))
        (Class|GMCMovementUtilityCmp|AdjustVelocityfromHit _outhit_2 false 0.0)
        (Class|MovementComponent|MoveUpdatedComponent (* (Class|GMCReplicationCmp|GetVelocity) (Class|GMCMovementUtilityCmp|GetPhysDeltaTime)) (Class|GMCMovementUtilityCmp|GetRootCollisionRotation) true))
      (else
        (Class|MovementComponent|MoveUpdatedComponent (* (Transformation|GetActorForwardVector (Components|GetOwner)) 4e+01) (Math|Rotator|Lerp(Rotator) (Class|GMCMovementUtilityCmp|GetRootCollisionRotation) (Math|Rotator|MakeRotator 0.0 -9e+01 0.0) 0.7 true) true)))))

(event EventBindReplicationData
  (|CallParentFunction)
  (Class|GMCReplicationCmp|BindDoublePrecisionFloat (Variables|Default|GetCurrentRoll) "ServerAuth_Input_ClientValidated" "AlwaysCombine" "Periodic_Output" "NearestNeighbour")
  (Class|GMCReplicationCmp|BindDoublePrecisionFloat (Variables|Default|GetCurrentPitch) "ServerAuth_Input_ClientValidated" "AlwaysCombine" "Periodic_Output" "NearestNeighbour")
  (Class|GMCReplicationCmp|BindDoublePrecisionFloat (Variables|Default|GetCurrentYaw) "ServerAuth_Input_ClientValidated" "AlwaysCombine" "Periodic_Output" "NearestNeighbour")
  (Class|GMCReplicationCmp|BindDoublePrecisionFloat (Variables|Default|GetThrustMultiplier) "ClientAuth_Input" "AlwaysCombine" "Periodic_Output" "NearestNeighbour")
  (Class|GMCReplicationCmp|BindDoublePrecisionFloat (Variables|Default|GetThrustSpeed) "ClientAuth_Input" "AlwaysCombine" "Periodic_Output" "NearestNeighbour")
  (Class|GMCReplicationCmp|BindDoublePrecisionFloat (Variables|Default|GetDrag) "ServerAuth_Output_ServerValidated" "AlwaysCombine" "Periodic_Output" "NearestNeighbour")
  (Class|GMCReplicationCmp|BindDoublePrecisionFloat (Variables|Default|GetCurrentSpeed) "ServerAuth_InputOutput_ClientValidated" "AlwaysCombine" "Periodic_InputOutput" "NearestNeighbour")
  (Class|GMCReplicationCmp|BindDoublePrecisionFloat (Variables|Default|GetTargetRoll) "ClientAuth_Input" "CombineIfUnchanged" "None" "NearestNeighbour")
  (Class|GMCReplicationCmp|BindDoublePrecisionFloat (Variables|Default|GetTargetYaw) "ClientAuth_Input" "CombineIfUnchanged" "None" "NearestNeighbour")
  (Class|GMCReplicationCmp|BindDoublePrecisionFloat (Variables|Default|GetTargetPitch) "ClientAuth_Input" "CombineIfUnchanged" "None" "NearestNeighbour")
  (Class|GMCReplicationCmp|BindBool (Variables|Default|GetFCSLimit) "ClientAuth_Input" "CombineIfUnchanged" "None" "NearestNeighbour")
  (Class|GMCReplicationCmp|BindBool (Variables|Default|GetIsDash) "ServerAuth_InputOutput_ServerValidated" "CombineIfUnchanged" "None" "NearestNeighbour")
  (Class|GMCReplicationCmp|BindBool (Variables|Default|GetIsLanded) "ServerAuth_Output_ServerValidated" "AlwaysCombine" "Periodic_Output" "NearestNeighbour"))

(event EventBeginPlay
  (bind _asbp_aircraft_2 (Utilities|Casting|CastToBP_Aircraft2 (Components|GetOwner)))
  (Variables|Default|SetPlayerPawnRef _asbp_aircraft_2)
  (Variables|Default|SetP_Camera 0)
  (bind _asgmc_controller (Utilities|Casting|CastToGMC_Controller (Game|GetPlayerController 0)))
  (Utilities|IsValid (PlayerController|LocalPlayerSubsystems|GetEnhancedInputLocalPlayerSubsystem _asgmc_controller)
    (:Is%20Valid
      (Input|AddMappingContext (PlayerController|LocalPlayerSubsystems|GetEnhancedInputLocalPlayerSubsystem _asgmc_controller) "/Game/Input/HOTAS.HOTAS" 1 "(bIgnoreAllPressedKeysUntilRelease=True,bForceImmediately=False)")
      (Input|AddMappingContext (PlayerController|LocalPlayerSubsystems|GetEnhancedInputLocalPlayerSubsystem _asgmc_controller) "/Game/Input/NewInputMappingContext.NewInputMappingContext" 0 "(bIgnoreAllPressedKeysUntilRelease=True,bForceImmediately=False)"))))

(fn CamRollF
  (params (AngleDegrees :type Float%20%28double-precision%29))
  (bind _maxlook (Variables|Default|GetMaxLook))
  (bind _returnvalue (* _maxlook 0.35))
  (Variables|Default|SetTargetRoll (Math|Float|ClampAngle AngleDegrees (* _returnvalue -1.0) _returnvalue)))

(fn CamRollRecF
  (Variables|Default|SetTargetRoll (Math|Interpolation|FInterpTo (Variables|Default|GetTargetRoll) 0.0 (Variables|Default|GetDeltaSeconds) 0.0)))

(fn CamPitchF
  (params (AngleDegrees :type Float%20%28double-precision%29))
  (bind _currentspeed (Variables|Default|GetCurrentSpeed))
  (bind _maxlook (Variables|Default|GetMaxLook))
  (bind _fcslimit (Variables|Default|GetFCSLimit))
  (bind _rotationcurve (Variables|Default|GetRotationCurve))
  (bind _returnvalue (Math|Curves|GetFloatValue _rotationcurve _currentspeed))
  (bind _returnvalue_2 (Math|Float|Clamp(Float) _returnvalue 0.1))
  (bind _returnvalue_3 (select _fcslimit _returnvalue_2 _maxlook))
  (bind _returnvalue_4 (* _returnvalue_3 2.0))
  (Variables|Default|SetTargetPitch (Math|Float|ClampAngle AngleDegrees (* _returnvalue_4 -1.0) _returnvalue_4)))

(fn CamPitchRecF
  (Variables|Default|SetTargetPitch (Math|Interpolation|FInterpTo (Variables|Default|GetTargetPitch) 0.0 (Variables|Default|GetDeltaSeconds) 0.0)))

(fn CamYawF
  (params (AngleDegrees :type Float%20%28double-precision%29))
  (bind _currentspeed (Variables|Default|GetCurrentSpeed))
  (bind _maxlook (Variables|Default|GetMaxLook))
  (bind _fcslimit (Variables|Default|GetFCSLimit))
  (bind _rotationcurve (Variables|Default|GetRotationCurve))
  (bind _returnvalue (Math|Curves|GetFloatValue _rotationcurve _currentspeed))
  (bind _returnvalue_2 (Math|Float|Clamp(Float) _returnvalue 0.1))
  (bind _returnvalue_3 (select _fcslimit _returnvalue_2 _maxlook))
  (bind _returnvalue_4 (* _returnvalue_3 1.2))
  (Variables|Default|SetTargetYaw (Math|Float|ClampAngle AngleDegrees (* _returnvalue_4 -1.0) _returnvalue_4)))

(fn CamYawRecF
  (Variables|Default|SetTargetYaw (Math|Interpolation|FInterpTo (Variables|Default|GetTargetYaw) 0.0 (Variables|Default|GetDeltaSeconds) 0.0)))

(fn CopyRot)

(fn UpdatePosition
  (params (Delta :type Float%20%28double-precision%29))
  (bind _output_get (Variables|Default|SetCurrentSpeed (Math|Float|Clamp(Float) (Math|Interpolation|FInterpTo (Variables|Default|GetCurrentSpeed) (Variables|Default|GetThrustSpeed) Delta (Variables|Default|GetDrag)) 0.0 (Variables|Default|GetMaxThrustSpeed))))
  (if (> _output_get (Variables|Default|GetStall))
    (Class|GMCMovementUtilityCmp|UpdateVelocity (* (Transformation|GetActorForwardVector (Components|GetOwner)) (Variables|Default|GetCurrentSpeed)) (Class|GMCMovementUtilityCmp|GetPhysDeltaTime))
    (else
      (Class|GMCMovementUtilityCmp|UpdateVelocity (+ (* (Transformation|GetActorForwardVector (Components|GetOwner)) (Variables|Default|GetCurrentSpeed)) (* (Transformation|GetActorUpVector (Components|GetOwner)) (Math|Float|SafeDivide (Variables|Default|GetGravity) (+ (Variables|Default|GetCurrentSpeed) 1.0)))) (Class|GMCMovementUtilityCmp|GetPhysDeltaTime))))
  (return (* (Transformation|GetActorForwardVector (Components|GetOwner)) (Variables|Default|GetCurrentSpeed))))

(fn RollF
  (Variables|Default|SetCurrentRoll (Math|Interpolation|FInterpTo (Variables|Default|GetCurrentRoll) (Variables|Default|GetTargetRoll) (Class|GMCMovementUtilityCmp|GetPhysDeltaTime) (Variables|Default|GetInterp%20Speed))))

(fn PitchF
  (Variables|Default|SetCurrentPitch (Math|Interpolation|FInterpTo (Variables|Default|GetCurrentPitch) (* (Variables|Default|GetTargetPitch) (Utilities|TurnspeedMacro)) (Class|GMCMovementUtilityCmp|GetPhysDeltaTime) (Variables|Default|GetInterp%20Speed))))

(fn YawF
  (Variables|Default|SetCurrentYaw (Math|Interpolation|FInterpTo (Variables|Default|GetCurrentYaw) (Variables|Default|GetTargetYaw) (Class|GMCMovementUtilityCmp|GetPhysDeltaTime) (Variables|Default|GetInterp%20Speed))))

(fn Speed0
  (params (Speed :type Float%20%28double-precision%29) (Delta :type Float%20%28double-precision%29))
  (Variables|Default|SetThrustSpeed (Math|Float|Clamp(Float) (+ (* Speed Delta (Variables|Default|GetThrustMultiplier)) (Variables|Default|GetThrustSpeed)) 0.0 (Variables|Default|GetMaxThrustSpeed))))

(fn CopyRot2)

(fn Yaw2
  (params (A :type Float%20%28double-precision%29) (B :type Float%20%28double-precision%29))
  (bind _yawdif (Variables|Default|GetYawDif))
  (bind _returnvalue (* _yawdif -1.0))
  (Utilities|ComparewithError (Variables|Default|GeterrorMargin) A B
    (:EqualAbout
      (Variables|Default|SetAVYaw (Math|Interpolation|FInterptoConstant (Variables|Default|GetAVYaw) 0.0 (Class|GMCMovementUtilityCmp|GetPhysDeltaTime) (Variables|Default|Getintspeed))))
    (:Less
      (Variables|Default|SetAVYaw (Math|Interpolation|FInterptoConstant (Variables|Default|GetAVYaw) (Math|Float|Clamp(Float) (+ (Variables|Default|GetAVYaw) _yawdif) _returnvalue _yawdif) (Class|GMCMovementUtilityCmp|GetPhysDeltaTime) (Variables|Default|Getintspeed))))
    (:Greater
      (Variables|Default|SetAVYaw (Math|Interpolation|FInterptoConstant (Variables|Default|GetAVYaw) (Math|Float|Clamp(Float) (- (Variables|Default|GetAVYaw) _yawdif) _returnvalue _yawdif) (Class|GMCMovementUtilityCmp|GetPhysDeltaTime) (Variables|Default|Getintspeed))))))

(fn Pitch2
  (params (A :type Float%20%28double-precision%29) (B :type Float%20%28double-precision%29))
  (bind _pitchdif (Variables|Default|GetPitchDif))
  (bind _returnvalue (* _pitchdif -1.0))
  (Utilities|ComparewithError (Variables|Default|GeterrorMargin) A B
    (:EqualAbout
      (Variables|Default|SetAVPitch (Math|Interpolation|FInterptoConstant (Variables|Default|GetAVPitch) 0.0 (Class|GMCMovementUtilityCmp|GetPhysDeltaTime) (Variables|Default|Getintspeed))))
    (:Less
      (Variables|Default|SetAVPitch (Math|Interpolation|FInterptoConstant (Variables|Default|GetAVPitch) (Math|Float|Clamp(Float) (+ (Variables|Default|GetAVPitch) _pitchdif) _returnvalue _pitchdif) (Class|GMCMovementUtilityCmp|GetPhysDeltaTime) (Variables|Default|Getintspeed))))
    (:Greater
      (Variables|Default|SetAVPitch (Math|Interpolation|FInterptoConstant (Variables|Default|GetAVPitch) (Math|Float|Clamp(Float) (- (Variables|Default|GetAVPitch) _pitchdif) _returnvalue _pitchdif) (Class|GMCMovementUtilityCmp|GetPhysDeltaTime) (Variables|Default|Getintspeed))))))

(fn Roll2
  (params (A :type Float%20%28double-precision%29) (B :type Float%20%28double-precision%29))
  (bind _rolldif (Variables|Default|GetRollDif))
  (bind _returnvalue (* _rolldif -1.0))
  (Utilities|ComparewithError (Variables|Default|GeterrorMargin) A B
    (:EqualAbout
      (Variables|Default|SetAVRoll (Math|Interpolation|FInterptoConstant (Variables|Default|GetAVRoll) 0.0 (Class|GMCMovementUtilityCmp|GetPhysDeltaTime) (Variables|Default|Getintspeed))))
    (:Less
      (Variables|Default|SetAVRoll (Math|Interpolation|FInterptoConstant (Variables|Default|GetAVRoll) (Math|Float|Clamp(Float) (+ (Variables|Default|GetAVRoll) 0.0) _returnvalue _rolldif) (Class|GMCMovementUtilityCmp|GetPhysDeltaTime) (Variables|Default|Getintspeed))))
    (:Greater
      (Variables|Default|SetAVRoll (Math|Interpolation|FInterptoConstant (Variables|Default|GetAVRoll) (Math|Float|Clamp(Float) (- (Variables|Default|GetAVRoll) 0.0) _returnvalue _rolldif) (Class|GMCMovementUtilityCmp|GetPhysDeltaTime) (Variables|Default|Getintspeed))))))

(fn ControlAdd
  (Transformation|AddActorLocalRotation (Class|PawnMovementComponent|GetPawnOwner) (* (Math|Rotator|MakeRotator (* (Variables|Default|GetCurrentRoll) (Variables|Default|GetRollM)) (* (Variables|Default|GetCurrentPitch) (Variables|Default|GetPitchM)) (* (Variables|Default|GetCurrentYaw) (Variables|Default|GetYawM))) (* (Class|GMCMovementUtilityCmp|GetPhysDeltaTime) 1e+01)) false false))

(fn UpdatePositionGround
  (params (Delta :type Float%20%28double-precision%29))
  (bind _output_get (Variables|Default|SetCurrentSpeed (Math|Float|Clamp(Float) (Math|Interpolation|FInterpTo (Variables|Default|GetCurrentSpeed) (Variables|Default|GetThrustSpeed) Delta (Variables|Default|GetDrag)) 0.0 (Variables|Default|GetStall))))
  (if (> _output_get (Variables|Default|GetStall))
    (Class|GMCMovementUtilityCmp|UpdateVelocity (* (Transformation|GetActorForwardVector (Components|GetOwner)) (Variables|Default|GetCurrentSpeed)) (Class|GMCMovementUtilityCmp|GetPhysDeltaTime))
    (else
      (Class|GMCMovementUtilityCmp|UpdateVelocity (+ (* (Transformation|GetActorForwardVector (Components|GetOwner)) (Variables|Default|GetCurrentSpeed)) (* (Transformation|GetActorUpVector (Components|GetOwner)) (Math|Float|SafeDivide (Variables|Default|GetGravity) (+ (Variables|Default|GetCurrentSpeed) 1.0)))) (Class|GMCMovementUtilityCmp|GetPhysDeltaTime))))
  (return (* (Transformation|GetActorForwardVector (Components|GetOwner)) (Variables|Default|GetCurrentSpeed))))