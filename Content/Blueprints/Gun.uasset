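; Gun Blueprint that fires bullet actors on behalf of the player's Prototype_9 pawn.
; BeginPlay caches the player pawn, which GunFire passes as the owner of each bullet.
; After a very short delay, GunFire checks Ammo, spawns BP_Bullet at the Arrow component's transform, and decrements Ammo.
; Random pitch and yaw offsets within the Accuracy range give the shots spread.
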(event Custom|GunFire
  (bind _accuracy (Variables|Default|GetAccuracy))
  (bind _arrow (Variables|Default|GetArrow))
  (bind _returnvalue (Transformation|GetWorldTransform _arrow))
  (bind _returnvalue_2 (* _accuracy -1.0))
  (Utilities|FlowControl|Delay 0.01)
  (if (> (Variables|Default|GetAmmo) 0)
    (Game|SpawnActorfromClass "/Game/Blueprints/BP_Bullet.BP_Bullet_C" (Math|Transform|MakeTransform (.location _returnvalue) (Math|Rotator|MakeRotator (.roll (.rotation _returnvalue)) (+ (.pitch (.rotation _returnvalue)) (Math|Random|RandomFloatinRange _returnvalue_2 _accuracy)) (+ (.yaw (.rotation _returnvalue)) (Math|Random|RandomFloatinRange _returnvalue_2 _accuracy))) (.scale _returnvalue)) "AlwaysSpawn" (Variables|Default|GetPlayerRef) 0)
    (Math|Integer|DecrementInt (Variables|Default|GetAmmo))))

(event EventBeginPlay
  (bind _asprototype_9 (Utilities|Casting|CastToPrototype_9 (Game|Player|GetPlayerPawn 0)))
  (Variables|Default|SetPlayerRef _asprototype_9))

(fn ConstructionScript)