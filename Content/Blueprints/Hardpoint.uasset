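; Weapon hardpoint that carries and launches missiles, with the Prototype_9 player pawn as their owner.
; On BeginPlay it spawns a weapon class per WepLocEX-tagged component and snaps those tagged Weapon onto their mounts.
; RelayFire passes through a server RPC to RPC_Fire, which releases and fires the first equipped missile, removing it from the list.
; Tick sets IsEmpty once no valid weapon remains at the front.
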(event Custom|RPC_Fire
  (bind _equippedweapons (Variables|Default|GetEquippedWeapons))
  (bind _asmissile (Utilities|Casting|CastToMissile (Utilities|Array|Get(acopy) _equippedweapons)))
  (Variables|/Game/Blueprints/Missile.Missile_C|SetIsAttatched _asmissile false)
  (Utilities|Array|RemoveIndex _equippedweapons)
  (Default|MissileFireM _asmissile))

(event Custom|RPC_Server_Fire
  (CallFunction|RPCFire))

(event Custom|RelayFire
  (CallFunction|RPCServerFire))

(event EventBeginPlay
  (bind _asprototype_9 (Utilities|Casting|CastToPrototype_9 (Game|Player|GetPlayerPawn 0)))
  (bind _output_get (Variables|Default|SetPlayerRef _asprototype_9))
  (for (_array_element _array_index) (Actor|GetComponentsbyTag "/Script/Engine.SceneComponent" "WepLocEX")
    (bind _returnvalue (Utilities|Array|Add (Variables|Default|GetWeaponLocation) _array_element))
    (if (Utilities|IsValidClass (Utilities|Array|Get(acopy) (Variables|Default|GetWeaponClassArray) _array_index))
      (bind _returnvalue_2 (Game|SpawnActorfromClass (Utilities|Array|Get(acopy) (Variables|Default|GetWeaponClassArray) _array_index) (Transformation|GetActorTransform) "Undefined" _output_get 0))
      (if (Actor|ActorHasTag _returnvalue_2 "Weapon")
        (Utilities|Array|Add (Variables|Default|GetEquippedWeapons) _returnvalue_2)
        (Transformation|AttachComponentToComponent _returnvalue_2 (Utilities|Array|Get(acopy) (Variables|Default|GetWeaponLocation) _returnvalue) "None" "SnapToTarget" "SnapToTarget" "SnapToTarget" false)))))

(event EventTick
  (params (DeltaSeconds :type Float%20%28single-precision%29))
  (Utilities|IsValid (Utilities|Array|Get(acopy) (Variables|Default|GetEquippedWeapons))
    (:Is%20Not%20Valid
      (Variables|Default|SetIsEmpty true))))

(fn ConstructionScript)