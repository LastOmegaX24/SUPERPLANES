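; Laser turret that locks onto the player's BP_Aircraft2 when it hears it and fires a damaging beam.
; Tick turns OuterCircle toward the target, faster as it gets closer.
; Each heard noise within LaserRange triggers a pawn trace along InnerCircle's forward, applying curve-based distance damage and spawning a Niagara beam to the impact.
; It also links its health widget and supplies map icon data.
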(event OnHearNoise(PawnSensing)
  (params (Instigator :type Pawn%20Object%20Reference) (Location :type Vector%20%28by%20ref%29 :default "0, 0, 0") (Volume :type Float%20%28single-precision%29))
  (bind _innercircle (Variables|Default|GetInnerCircle))
  (bind _returnvalue (Transformation|GetWorldLocation _innercircle))
  (Utilities|IsValid Instigator
    (:Is%20Valid
      (if (Variables|Default|GetIsAlive)
        (bind _asbp_aircraft_2 (Utilities|Casting|CastToBP_Aircraft2 Instigator))
        (if (Actor|ActorHasTag _asbp_aircraft_2 "Player")
          (Variables|Default|SetLocked%20Target _asbp_aircraft_2)
          (if (< (Math|Vector|Distance(Vector) (Transformation|GetActorLocation (Variables|Default|GetLocked%20Target)) (Transformation|GetActorLocation)) (Variables|Default|GetLaserRange))
            (if (Variables|Default|GetIsAlive)
              (bind _outhits (Class|KismetSystemLibrary|LineTraceMultiforObjects _returnvalue (+ _returnvalue (* (Math|Vector|GetForwardVector _innercircle) (Variables|Default|GetLaserRange))) (Utilities|Array|MakeArray "ObjectTypeQuery3") false 0 "None" true))
              (for _array_element _outhits
                (if (Actor|ActorHasTag (.HitActor (Collision|BreakHitResult _array_element)) "Player")
                  (Game|Damage|ApplyDamage (.HitActor (Collision|BreakHitResult _array_element)) (Math|Curves|GetFloatValue (Variables|Default|GetDamageCurve) (Math|Vector|Distance(Vector) (.ImpactPoint (Collision|BreakHitResult _array_element)) (.TraceStart (Collision|BreakHitResult _array_element)))) 0 0 "/Game/Blueprints/MainSystem/StandardDamage.StandardDamage_C")
                  (bind _returnvalue_2 (Niagara|SpawnSystematLocation "/Game/Particle/Laser.Laser" (Transformation|GetWorldLocation (Variables|Default|GetInnerCircle)) "0, 0, 0" "1.000000,1.000000,1.000000" true true "AutoRelease"))
                  (Utilities|IsValid _returnvalue_2
                    (:Is%20Valid
                      (Niagara|SetNiagaraVariable(Vector3) _returnvalue_2 "BeamEnd" (.ImpactPoint (Collision|BreakHitResult _array_element))))))))))))))

(event EventTick
  (params (DeltaSeconds :type Float%20%28single-precision%29))
  (bind _locked_target (Variables|Default|GetLocked%20Target))
  (bind _outercircle (Variables|Default|GetOuterCircle))
  (bind _returnvalue (Transformation|GetActorLocation _locked_target))
  (bind _returnvalue_2 (Transformation|GetWorldLocation _outercircle))
  (if (Variables|Default|GetIsAlive)
    (Utilities|IsValid _locked_target
      (:Is%20Valid
        (Transformation|SetWorldRotation (Variables|Default|GetOuterCircle) (Math|Rotator|Lerp(Rotator) (Transformation|GetWorldRotation (Variables|Default|GetOuterCircle)) (Math|Rotator|FindLookatRotation _returnvalue_2 _returnvalue) (Math|Float|Clamp(Float) (Math|Float|SafeDivide 2e+03 (Math|Vector|Distance(Vector) _returnvalue _returnvalue_2)) 0.03) true) false false)))))

(event EventBeginPlay
  (bind _asturret_health (Utilities|Casting|CastToTurretHealth (UserInterface|GetWidget (Variables|Default|GetWidget))))
  (Variables|/Game/HUD/TurretHealth.TurretHealth_C|SetTurret _asturret_health self))

(fn ConstructionScript)

(fn GetMapIconData
  (bind _mapiconcomponent (Variables|Default|GetMapIconComponent))
  (return (Transformation|GetActorLocation) (Variables|/Game/Blueprints/MapIconComponent.MapIconComponent_C|GetImageTex _mapiconcomponent) (Variables|/Game/Blueprints/MapIconComponent.MapIconComponent_C|GetSize _mapiconcomponent)))