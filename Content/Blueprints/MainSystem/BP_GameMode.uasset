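; BP_GameMode is a game mode that numbers joining players and respawns them when they die.
; PostLogin gives each BP_PlayerController a sequential PlayerID and records it in an ID list.
; PlayerDied, bound to OnPlayerDied at BeginPlay, restarts the dead character's controller.
; ChoosePlayerStart returns a random PlayerStart; it increments a NextPlayer counter but does not use it for the choice.
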(event Custom|PlayerDied
  (params (Character :type Pawn%20Object%20Reference))
  (Class|GameModeBase|RestartPlayer (Pawn|GetController Character)))

(event EventPostLogin
  (params (NewPlayer :type Player%20Controller%20Object%20Reference))
  (bind _asbp_player_controller (Utilities|Casting|CastToBP_PlayerController NewPlayer))
  (bind _output_get (Variables|/Game/Blueprints/MainSystem/BP_PlayerController.BP_PlayerController_C|SetPlayerID _asbp_player_controller (Variables|Default|GetIndex)))
  (Utilities|Array|AddUnique (Variables|Default|GetPlayerID) _output_get)
  (Math|Integer|IncrementInt (Variables|Default|GetIndex)))

(event EventTick
  (params (DeltaSeconds :type Float%20%28single-precision%29)))

(event EventBeginPlay
  (EventDispatchers|BindEventtoOnPlayerDied (delegate Custom|PlayerDied)))

(fn ConstructionScript)

(fn ChoosePlayerStart
  (params (Player :type Controller%20Object%20Reference))
  (Math|Integer|IncrementInt (Variables|Default|GetNextPlayer)
    (:%20%20
      (bind _outactors (Actor|GetAllActorsOfClass "/Script/Engine.PlayerStart"))
      (return (.OutItem (Utilities|Array|Random _outactors))))))