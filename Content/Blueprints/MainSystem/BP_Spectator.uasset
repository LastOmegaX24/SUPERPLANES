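; BP_Spectator is a spectator Blueprint that handles aircraft loadout and spawning before the player takes control.
; BeginPlay adds HOTAS and default Enhanced Input mapping contexts.
; SelectAircraft sizes weapon arrays from the aircraft's hardpoint counts, and GetWeaponData fills the internal array from data table rows.
; SelectKey calls a server spawn event that creates SpawnAircraft at a random PlayerStart, passes both arrays and possesses it.
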(event Custom|SelectAircraft
  (params (NewParam :type BP%20Aircraft%202%20Class%20Reference))
  (bind _info (Utilities|GetClassDefaults NewParam))
  (bind (_name _internalhardpoints _externalhardpoints) (Utilities|Struct|BreakAircraftInfo _info))
  (Utilities|Array|Resize (Variables|Default|GetWeaponArr) _internalhardpoints)
  (Utilities|Array|Resize (Variables|Default|GetWeaponEXTArr) _externalhardpoints))

(event Custom|RPC_Server_Spawn
  (params (NewParam :type Controller%20Object%20Reference) (NewParam2 :type Pawn%20Object%20Reference))
  (bind _outactors (Actor|GetAllActorsOfClass "/Script/Engine.PlayerStart"))
  (bind _returnvalue (Game|SpawnActorfromClass :Class (Variables|Default|GetSpawnAircraft) :SpawnTransform (Math|Transform|MakeTransform (.location (Transformation|GetActorTransform (.OutItem (Utilities|Array|Random _outactors)))) (.rotation (Transformation|GetActorTransform (.OutItem (Utilities|Array|Random _outactors)))) "0.050000,0.050000,0.050000") :CollisionHandlingOverride "Undefined" :WeaponClassArray (Variables|Default|GetWeaponArr) :WeaponClassArray_Ext (Variables|Default|GetWeaponEXTArr) :Instigator 0))
  (Pawn|Possess NewParam _returnvalue))

(event Custom|GetWeaponData
  (params (ItemData :type S%20Slots%20Structure) (Index :type Integer))
  (bind _output_get (Variables|Default|SetItem%20Data ItemData))
  (bind _returnvalue (Utilities|GetDataTableRow (.datatable (Utilities|Struct|BreakS_Slots _output_get)) (.rowname (Utilities|Struct|BreakS_Slots _output_get)))
    (:then
      (Utilities|Array|SetArrayElem (Variables|Default|GetWeaponArr) Index (.WeaponClass (Utilities|Struct|BreakS_Weapons _returnvalue)) true))))

(event Input|EnhancedActionEvents|EnhancedInputActionSelectKey
  (params (ActionValue :type Boolean) (ElapsedSeconds :type Float%20%28double-precision%29) (TriggeredSeconds :type Float%20%28double-precision%29) (InputAction :type Input%20Action%20Object%20Reference :default "/Game/Input/Actions/SelectKey.SelectKey"))
  (:Triggered
    (CallFunction|RPCServerSpawn (Game|GetPlayerController 0))))

(event EventBeginPlay
  (bind _returnvalue (Game|Player|GetPlayerPawn 0))
  (Utilities|IsValid _returnvalue
    (:Is%20Valid
      (bind _asgmc_controller (Utilities|Casting|CastToGMC_Controller (Pawn|GetController _returnvalue)))
      (Utilities|IsValid (PlayerController|LocalPlayerSubsystems|GetEnhancedInputLocalPlayerSubsystem _asgmc_controller)
        (:Is%20Valid
          (Input|AddMappingContext (PlayerController|LocalPlayerSubsystems|GetEnhancedInputLocalPlayerSubsystem _asgmc_controller) "/Game/Input/HOTAS.HOTAS" 1 "(bIgnoreAllPressedKeysUntilRelease=True,bForceImmediately=False)")
          (Input|AddMappingContext (PlayerController|LocalPlayerSubsystems|GetEnhancedInputLocalPlayerSubsystem _asgmc_controller) "/Game/Input/NewInputMappingContext.NewInputMappingContext" 0 "(bIgnoreAllPressedKeysUntilRelease=True,bForceImmediately=False)"))))))

(fn ConstructionScript)