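; MapIconComponent is a component that shows a map icon for its owning actor.
; On BeginPlay it creates a MapIconWidget, initializes it with the icon data (texture, location, size) and adds it to the viewport.
; Each tick it feeds the owner's 2D position and yaw to the widget and matches its visibility to the HUD_OVR toggle.
; Once UpdateIsAlive clears the alive flag, Tick removes the widget.
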(event EventBeginPlay
  (bind _returnvalue (Game|GetPlayerController 0))
  (Utilities|IsValid _returnvalue
    (:Is%20Valid
      (bind _ashud_ovr (Utilities|Casting|CastToHUD_OVR (HUD|GetHUD _returnvalue)))
      (Variables|Default|SetAs%20HUD%20OVR _ashud_ovr)
      (bind _returnvalue_2 (UserInterface|CreateWidget "/Game/HUD/MapIconWidget.MapIconWidget_C" (Game|GetPlayerController 0)))
      (bind _output_get (Variables|Default|SetMapIconRef _returnvalue_2))
      (bind (_location _icon _size) (Class|MapItem|GetMapIconData(Message) self))
      (Default|InitIcons _output_get _icon (Math|Vector2D|MakeVector2D (.x _location) (.y _location)) _size)
      (UserInterface|Viewport|AddtoViewport _output_get 3))))

(event EventTick
  (params (DeltaSeconds :type Float%20%28single-precision%29))
  (bind _returnvalue (Components|GetOwner))
  (bind _mapiconref (Variables|Default|GetMapIconRef))
  (bind _as_hud_ovr (Variables|Default|GetAs%20HUD%20OVR))
  (if (Variables|Default|GetIs%20Alive)
    (Utilities|IsValid _mapiconref
      (:Is%20Valid
        (Default|UpdateWidgetLocation _mapiconref (Math|Conversions|ToVector2D(Vector) (Transformation|GetActorLocation _returnvalue)) (.yaw (Transformation|GetActorRotation _returnvalue)))
        (Utilities|IsValid _as_hud_ovr
          (:Is%20Valid
            (if (Variables|/Game/HUD/HUD_OVR.HUD_OVR_C|GetToggle _as_hud_ovr)
              (Widget|SetVisibility (Variables|Default|GetMapIconRef) "Visible")
              (else
                (Widget|SetVisibility (Variables|Default|GetMapIconRef) "Hidden")))))))
    (else
      (Widget|RemovefromParent (Variables|Default|GetMapIconRef)))))

(event EventUpdateIsAlive
  (params (IsAlive :type Boolean))
  (Variables|Default|SetIs%20Alive IsAlive))

(fn GetMapIconData
  (return (Transformation|GetActorLocation (Components|GetOwner)) (Variables|Default|GetImageTex) (Variables|Default|GetSize)))