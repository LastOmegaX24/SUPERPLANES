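; Homing missile that seeks actors tagged "Homing", applies heavy damage on any overlap and destroys itself.
; Each Tick, HomingTarget searches for the closest tagged actor by absolute-coordinate distance and feeds its scene component to ProjectileMovement as the homing target.
; Rotation blends the target's own rotation toward a look-at angle.
; The UpdatePosition thrust-and-gravity model never runs, and the stored player pawn reference is unused.
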(event EventBeginPlay
  (bind _asx42amagic_v2 (Utilities|Casting|CastToX42AMagic_V2 (Game|Player|GetPlayerPawn 0)))
  (Variables|Default|SetPlayerRef _asx42amagic_v2))

(event Collision|EventActorBeginOverlap
  (params (OtherActor :type Actor%20Object%20Reference))
  (Game|Damage|ApplyDamage 0 1e+03 0 0)
  (Actor|DestroyActor))

(event EventTick
  (params (DeltaSeconds :type Float%20%28single-precision%29))
  (bind _projectilemovement (Variables|Default|GetProjectileMovement))
  (bind (_homingtarget _actor) (CallFunction|HomingTarget))
  (Transformation|SetActorRotation (Math|Rotator|Lerp(Rotator) (Transformation|GetActorRotation _actor) (Math|Rotator|FindLookatRotation (Transformation|GetActorLocation) (Transformation|GetActorLocation _actor)) 0.3 true))
  (Variables|/Script/Engine.ProjectileMovementComponent|SetHomingTargetComponent _projectilemovement _homingtarget)
  (Variables|/Script/Engine.ProjectileMovementComponent|SetbIsHomingProjectile _projectilemovement true))

(fn ConstructionScript)

(fn HomingTarget
  (bind _outactors (Actor|GetAllActorsOfClasswithTag "/Script/Engine.Actor" "Homing"))
  (for _array_element _outactors
    (if (< (Math|Vector|VectorLength (- (Math|Vector|VectorGetAbs (Transformation|GetActorLocation _array_element)) (Math|Vector|VectorGetAbs (Transformation|GetActorLocation)))) (Variables|Default|GetClosest_Target))
      (Variables|Default|SetClosest_Target (Math|Vector|VectorLength (- (Math|Vector|VectorGetAbs (Transformation|GetActorLocation _array_element)) (Math|Vector|VectorGetAbs (Transformation|GetActorLocation)))))
      (Variables|Default|SetArray%20Element _array_element)))
  (return (Actor|GetComponentbyClass (Variables|Default|GetArray%20Element) "/Script/Engine.SceneComponent") (Variables|Default|GetArray%20Element)))

(fn UpdatePosition
  (params (Delta :type Float%20%28double-precision%29))
  ;[1 1 1] Calc Current Speed
  (Variables|Default|SetCurrentSpeed (Math|Float|Clamp(Float) (select (< (Variables|Default|GetThrustSpeed) (Variables|Default|GetCurrentSpeed)) (Math|Interpolation|FInterpTo (Variables|Default|GetCurrentSpeed) (Variables|Default|GetThrustSpeed) 0.0 (Variables|Default|GetDrag)) (Variables|Default|GetThrustSpeed)) 0.0 (Variables|Default|GetMaxThrustSpeed)))
  ;[1 1 1] Calc new position based on speed
  (Variables|Default|SetNewPos (* (* (Variables|Default|GetCurrentSpeed) "") (Transformation|GetActorForwardVector)))
  ;[1 1 1] Calc Applied Gravity
  (Variables|Default|SetAppliedGravity (Math|Float|MapRangeClamped (Variables|Default|GetCurrentSpeed) 0.0 (Variables|Default|GetMinThrustStall) (Variables|Default|GetGravity) 0.0))
  ;[1 1 1] Get Position
  (Transformation|AddActorWorldOffset (Math|Vector|MakeVector (.X (Class|KismetMathLibrary|BreakVector3f (Variables|Default|GetNewPos))) (.Y (Class|KismetMathLibrary|BreakVector3f (Variables|Default|GetNewPos))) (- (.Z (Class|KismetMathLibrary|BreakVector3f (Variables|Default|GetNewPos))) (* (Variables|Default|GetAppliedGravity) 1.0))) true))