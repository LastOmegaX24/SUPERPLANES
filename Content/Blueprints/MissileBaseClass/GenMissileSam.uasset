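; GMC movement component for the MissileSam actor that flies it forward and homes it onto its target after a delay.
; Each prediction tick eases speed toward thrust while homing with fuel, then decelerates with weaker steering once fuel runs out.
; FollowTarget lerps rotation toward the target's current location, as its lead-prediction branch is hardwired off.
; Flight and homing state are bound for server-authoritative GMC replication.
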(event EventBindReplicationData
  (|CallParentFunction)
  (Class|GMCReplicationCmp|BindDoublePrecisionFloat (Variables|Default|GetCurrentSpeedM) "ServerAuth_Output_ServerValidated" "AlwaysCombine" "Periodic_Output" "NearestNeighbour")
  (Class|GMCReplicationCmp|BindDoublePrecisionFloat (Variables|Default|GetFuel) "ServerAuth_Output_ServerValidated" "AlwaysCombine" "Periodic_Output" "NearestNeighbour")
  (Class|GMCReplicationCmp|BindDoublePrecisionFloat (Variables|Default|GetThrustSpeedM) "ServerAuth_Output_ServerValidated" "AlwaysCombine" "Periodic_Output" "NearestNeighbour")
  (Class|GMCReplicationCmp|BindDoublePrecisionFloat (Variables|Default|GetSpeedMultiplier) "ServerAuth_Output_ServerValidated" "AlwaysCombine" "Periodic_Output" "NearestNeighbour")
  (Class|GMCReplicationCmp|BindActorReference (Variables|Default|GetCurrentTarget) "ServerAuth_Output_ClientValidated" "AlwaysCombine" "Periodic_Output" "NearestNeighbour")
  (Class|GMCReplicationCmp|BindActorReference (Variables|Default|GetAs%20Missile%203) "ServerAuth_Output_ClientValidated" "AlwaysCombine" "Periodic_Output" "NearestNeighbour")
  (Class|GMCReplicationCmp|BindBool (Variables|Default|GetIsHoming) "ServerAuth_Output_ClientValidated" "AlwaysCombine" "Periodic_Output" "NearestNeighbour")
  (Class|GMCReplicationCmp|BindDoublePrecisionFloat (Variables|Default|GetHomingDelay) "ServerAuth_Output_ClientValidated" "AlwaysCombine" "Periodic_Output" "NearestNeighbour")
  (Class|GMCReplicationCmp|BindDoublePrecisionFloat (Variables|Default|GetTurnspeed) "ServerAuth_Output_ClientValidated" "AlwaysCombine" "Periodic_Output" "NearestNeighbour"))

(event EventGenPredictionTick
  (params (DeltaTime :type Float%20%28single-precision%29))
  (Utilities|IsValid (Variables|Default|GetAs%20Missile%203)
    (:Is%20Valid
      (if (Variables|Default|GetIsHoming)
        (if (> (Variables|Default|GetFuel) 0.0)
          (Variables|Default|SetCurrentSpeedM (Math|Interpolation|FInterpTo (Variables|Default|GetCurrentSpeedM) (Variables|Default|GetThrustSpeedM) DeltaTime 0.1))
          (Variables|Default|SetFuel (- (Variables|Default|GetFuel) DeltaTime))
          (CallFunction|FollowTarget (Variables|Default|GetTurnspeed))
          (else
            (Variables|Default|SetCurrentSpeedM (- (Variables|Default|GetCurrentSpeedM) (* DeltaTime 5.0)))
            (CallFunction|FollowTarget (* (Variables|Default|GetTurnspeed) 0.2)))))
      (Class|GMCMovementUtilityCmp|UpdateVelocity (* (Transformation|GetActorForwardVector (Class|GMCReplicationCmp|GetGMCPawnOwner)) (Variables|Default|GetCurrentSpeedM) (Variables|Default|GetSpeedMultiplier)) (Class|GMCMovementUtilityCmp|GetPhysDeltaTime))
      (Class|MovementComponent|MoveUpdatedComponent (* (Class|GMCReplicationCmp|GetVelocity) (Class|GMCMovementUtilityCmp|GetPhysDeltaTime)) (Class|GMCMovementUtilityCmp|GetRootCollisionRotation) true)
      (if (== (Variables|Default|GetHomingDelay) 0.0)
        (Utilities|FlowControl|DoOnce false
          (:Completed
            (Variables|Default|SetIsHoming true)))
        (else
          (Variables|Default|SetHomingDelay (Math|Float|Clamp(Float) (- (Variables|Default|GetHomingDelay) (Class|GMCMovementUtilityCmp|GetPhysDeltaTime)) 0.0 1e+01)))))))

(event EventBeginPlay
  (bind _asmissile_sam (Utilities|Casting|CastToMissileSam (Components|GetOwner)))
  (Variables|Default|SetAs%20Missile%203 _asmissile_sam))

(fn FollowTarget
  (params (Turnspeed :type Float%20%28double-precision%29))
  (bind _returnvalue (Components|GetOwner))
  (bind _as_missile_3 (Variables|Default|GetAs%20Missile%203))
  (bind _returnvalue_2 (Transformation|GetActorTransform _returnvalue))
  (bind _currenttarget (Variables|/Game/Blueprints/MissileBaseClass/MissileSam.MissileSam_C|GetCurrentTarget _as_missile_3))
  (bind _returnvalue_3 (Transformation|GetActorLocation _currenttarget))
  (Utilities|IsValid _currenttarget
    (:Is%20Valid
      (Transformation|SetActorRotation (Components|GetOwner) (Math|Rotator|Lerp(Rotator) (.rotation _returnvalue_2) (Math|Rotator|FindLookatRotation (.location _returnvalue_2) (select true _returnvalue_3 (+ _returnvalue_3 (* (Transformation|GetActorForwardVector _currenttarget) (* (* (Math|Vector|VectorLength (Transformation|GetVelocity _currenttarget)) 0.05) (* (Math|Vector|Distance(Vector) _returnvalue_3 (.location _returnvalue_2)) 1.0)))))) (* Turnspeed 0.1) true)))
    (:Is%20Not%20Valid
      _))
  (return))