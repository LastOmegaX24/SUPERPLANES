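; Aircraft weapon hardpoint that carries and launches a loadout of missiles and bombs.
; On BeginPlay, if player pawn 0 is a BP_Aircraft2, the server spawns each configured weapon class and attaches those tagged Weapon to WepLocEX-tagged scene components.
; Fire requests go through an RPC, where the server removes the first equipped weapon and triggers its missile or bomb fire.
; Tick sets IsEmpty when no valid weapon is first in line.
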(event Custom|RPC_Fire
  (bind _equippedweapons (Variables|Default|GetEquippedWeapons))
  (bind _output (Utilities|Array|Get(acopy) _equippedweapons))
  (Networking|SwitchHasAuthority
    (:Authority
      (bind _asmissile_3 (Utilities|Casting|CastToMissile3 _output)
        (:then
          (Utilities|Array|RemoveIndex _equippedweapons)
          (Default|MissileFireM _asmissile_3))
        (:CastFailed
          (bind _asbomb (Utilities|Casting|CastToBomb _output))
          (Utilities|Array|RemoveIndex _equippedweapons)
          (Default|BombFireM _asbomb))))))

(event Custom|RelayFire
  (CallFunction|RPCFire))

(event EventBeginPlay
  (Networking|SwitchHasAuthority
    (:Authority
      (bind _asbp_aircraft_2 (Utilities|Casting|CastToBP_Aircraft2 (Game|Player|GetPlayerPawn 0)))
      (Variables|Default|SetPlayerRef _asbp_aircraft_2)
      (for (_array_element _array_index) (Actor|GetComponentsbyTag "/Script/Engine.SceneComponent" "WepLocEX")
        (bind _returnvalue (Utilities|Array|Add (Variables|Default|GetWeaponLocation) _array_element))
        (if (Utilities|IsValidClass (Utilities|Array|Get(acopy) (Variables|Default|GetWeaponClassArray) _array_index))
          (bind _returnvalue_2 (Game|SpawnActorfromClass (Utilities|Array|Get(acopy) (Variables|Default|GetWeaponClassArray) _array_index) (Transformation|GetActorTransform) "Undefined" (Components|GetOwner) (Game|GetInstigator)))
          (if (Actor|ActorHasTag _returnvalue_2 "Weapon")
            (Utilities|Array|Add (Variables|Default|GetEquippedWeapons) _returnvalue_2)
            (Transformation|AttachComponentToComponent _returnvalue_2 (Utilities|Array|Get(acopy) (Variables|Default|GetWeaponLocation) _returnvalue) "None" "SnapToTarget" "SnapToTarget" "SnapToTarget" false)))))))

(event EventTick
  (params (DeltaSeconds :type Float%20%28single-precision%29))
  (Utilities|IsValid (Utilities|Array|Get(acopy) (Variables|Default|GetEquippedWeapons))
    (:Is%20Not%20Valid
      (Variables|Default|SetIsEmpty true))))

(fn ConstructionScript)