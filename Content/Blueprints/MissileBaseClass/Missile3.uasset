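; Aircraft-launched missile that detaches from its BP_Aircraft2 owner, takes that aircraft's lock target and speed, and flies via a GenMissile component fed fuel, thrust and turn settings.
; Once deployed, overlaps route through RPC events to damage actors other than decoys, weapons and the owner, then explode.
; Hits on anything but flares also explode it if deployed, and firing sets a fuel-based lifespan.
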(event Custom|RPC_Particle
  (Components|Activation|Activate (Variables|Default|GetNiagara) false))

(event Custom|RPC_Damage
  (params (NewParam :type Actor%20Object%20Reference))
  (Utilities|IsValid NewParam
    (:Is%20Valid
      (if (not (Actor|ActorHasTag NewParam "Weapon"))
        (if (not (== NewParam (Variables|Default|GetPlayerRef)))
          (Game|Damage|ApplyDamage NewParam (Variables|Default|GetBaseDamage) (Pawn|GetController (Game|GetInstigator)) (Game|GetInstigator) "/Game/Blueprints/MainSystem/StandardDamage.StandardDamage_C")
          (CallFunction|Explode))))))

(event Custom|RPC_Server_Damage
  (params (OtherActor :type Actor%20Object%20Reference))
  (CallFunction|RPCDamage OtherActor))

(event Custom|MissileFireM
  (bind _genmissile1 (Variables|Default|GetGenMissile1))
  (bind _playerref (Variables|Default|GetPlayerRef))
  (bind _locktargetmissile (Variables|/Game/Blueprints/AircraftBaseClass/BP_Aircraft2.BP_Aircraft2_C|GetLockTargetMissile _playerref))
  (Utilities|IsValid _locktargetmissile
    (:Is%20Valid
      (Variables|Default|SetCurrentTarget _locktargetmissile))
    (:Is%20Not%20Valid
      _))
  (Rendering|SetVisibility (Variables|Default|GetWidget) true true)
  (Transformation|DetachFromActor "KeepWorld" "KeepWorld" "KeepWorld")
  (CallFunction|RPCParticle)
  (Variables|/Game/Blueprints/MissileBaseClass/GenMissile1.GenMissile1_C|SetCurrentSpeedM _genmissile1 (Variables|/Game/Blueprints/AircraftBaseClass/BP_Aircraft2.BP_Aircraft2_C|GetCurrentSpeed (Variables|Default|GetPlayerRef)))
  (Components|Activation|Activate _genmissile1 false)
  (Actor|SetLifeSpan (+ (Variables|Default|GetFuel) 5.0)))

(event EventBeginPlay
  (bind _genmissile1 (Variables|Default|GetGenMissile1))
  (bind _asbp_aircraft_2 (Utilities|Casting|CastToBP_Aircraft2 (Game|GetInstigator)))
  (Variables|Default|SetPlayerRef _asbp_aircraft_2)
  (Variables|/Game/Blueprints/MissileBaseClass/GenMissile1.GenMissile1_C|SetFuel _genmissile1 (Variables|Default|GetFuel))
  (Variables|/Game/Blueprints/MissileBaseClass/GenMissile1.GenMissile1_C|SetThrustSpeedM _genmissile1 (Variables|Default|GetThrust%20Speed%20M))
  (Variables|/Game/Blueprints/MissileBaseClass/GenMissile1.GenMissile1_C|SetTurnspeed _genmissile1 (Variables|Default|GetTurnspeed)))

(event Collision|EventActorBeginOverlap
  (params (OtherActor :type Actor%20Object%20Reference))
  (if (Variables|Default|GetIsDeployed)
    (Utilities|IsValid OtherActor
      (:Is%20Valid
        (if (not (Actor|ActorHasTag OtherActor "Decoy"))
          (CallFunction|RPCServerDamage OtherActor))))))

(event Collision|EventHit
  (params (MyComp :type Primitive%20Component%20Object%20Reference) (Other :type Actor%20Object%20Reference) (OtherComp :type Primitive%20Component%20Object%20Reference) (bSelfMoved :type Boolean) (HitLocation :type Vector :default "0, 0, 0") (HitNormal :type Vector :default "0, 0, 0") (NormalImpulse :type Vector :default "0, 0, 0") (Hit :type Hit%20Result%20Structure%20%28by%20ref%29))
  (if (!= (.hitactor Hit) "/Game/Blueprints/AircraftBaseClass/BP_Flare.BP_Flare")
    (CallFunction|Explode)))

(fn ConstructionScript)

(fn ProximityDet
  (Utilities|IsValid 0
    (:Is%20Valid
      (if (<= (Math|Vector|Distance(Vector) (Transformation|GetActorLocation) (Transformation|GetActorLocation)) 5e+03)
        (CallFunction|RPCServerDamage)))))

(fn EjectfromOrigin
  (params (Delta :type Float%20%28double-precision%29)))

(fn SafeDestroy
  (bind _returnvalue (Transformation|GetActorTransform))
  (Effects|SpawnEmitteratLocation "/Game/StarterContent/Particles/P_Explosion.P_Explosion" (.location _returnvalue) (.rotation _returnvalue) (* (.scale _returnvalue) 4.0))
  (Actor|DestroyActor))

(fn Explode
  (if (Variables|Default|GetIsDeployed)
    (Niagara|SpawnSystematLocation "/Niagara/DefaultAssets/Templates/Systems/SimpleExplosion.SimpleExplosion" (Transformation|GetActorLocation))
    (Components|Activation|Deactivate (Variables|Default|GetGenMissile1))
    (Actor|DestroyActor)))