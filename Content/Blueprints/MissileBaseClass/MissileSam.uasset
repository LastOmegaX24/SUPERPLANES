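; Surface-to-air missile actor fired by an Ai_SAM, which it caches from its instigator.
; BeginPlay passes flight tuning to the GenMissileSam component; MissileFireM detaches, activates it and particles, sets a fuel-based lifespan and warns the target aircraft.
; Once deployed, overlaps apply damage through chained RPCs, ignoring decoys, weapons and its launcher, then explode; non-flare hits also explode.
; ProximityDet and SafeDestroy are defined but not called here.
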(event Custom|RPC_Particle
  (Components|Activation|Activate (Variables|Default|GetNiagara) false))

(event Custom|RPC_Damage
  (params (NewParam :type Actor%20Object%20Reference))
  (Utilities|IsValid NewParam
    (:Is%20Valid
      (if (not (Actor|ActorHasTag NewParam "Weapon"))
        (if (not (== NewParam (Variables|Default|GetSAMRef)))
          (Game|Damage|ApplyDamage NewParam (Variables|Default|GetBaseDamage) (Pawn|GetController (Game|GetInstigator)) (Game|GetInstigator) "/Game/Blueprints/MainSystem/StandardDamage.StandardDamage_C")
          (CallFunction|Explode))))))

(event Custom|RPC_Server_Damage
  (params (OtherActor :type Actor%20Object%20Reference))
  (CallFunction|RPCDamage OtherActor))

(event Custom|MissileFireM
  (bind _currenttarget (Variables|Default|GetCurrentTarget))
  (Utilities|IsValid (Variables|Default|GetSAMRef)
    (:Is%20Valid
      (Rendering|SetVisibility (Variables|Default|GetWidget) true true)
      (Transformation|DetachFromActor "KeepWorld" "KeepWorld" "KeepWorld")
      (CallFunction|RPCParticle)
      (Variables|/Game/Blueprints/MissileBaseClass/GenMissileSam.GenMissileSam_C|SetCurrentSpeedM (Variables|Default|GetGenMissileSam) 2e+03)
      (Components|Activation|Activate (Variables|Default|GetGenMissileSam) false)
      (Actor|SetLifeSpan (+ (Variables|Default|GetFuel) 5.0))
      (Utilities|IsValid _currenttarget
        (:Is%20Valid
          (bind _asbp_aircraft_2 (Utilities|Casting|CastToBP_Aircraft2 _currenttarget))
          (Default|MissileWarn _asbp_aircraft_2 self))))))

(event EventBeginPlay
  (bind _genmissilesam (Variables|Default|GetGenMissileSam))
  (bind _asai_sam (Utilities|Casting|CastToAi_SAM (Game|GetInstigator)))
  (Variables|Default|SetSAMRef _asai_sam)
  (Variables|/Game/Blueprints/MissileBaseClass/GenMissileSam.GenMissileSam_C|SetFuel _genmissilesam (Variables|Default|GetFuel))
  (Variables|/Game/Blueprints/MissileBaseClass/GenMissileSam.GenMissileSam_C|SetThrustSpeedM _genmissilesam (Variables|Default|GetThrust%20Speed%20M))
  (Variables|/Game/Blueprints/MissileBaseClass/GenMissileSam.GenMissileSam_C|SetTurnspeedM _genmissilesam (Variables|Default|GetTurnspeed)))

(event Collision|EventActorBeginOverlap
  (params (OtherActor :type Actor%20Object%20Reference))
  (if (Variables|Default|GetIsDeployed)
    (Utilities|IsValid OtherActor
      (:Is%20Valid
        (if (not (Actor|ActorHasTag OtherActor "Decoy"))
          (CallFunction|RPCServerDamage OtherActor))))))

(event Collision|EventHit
  (params (MyComp :type Primitive%20Component%20Object%20Reference) (Other :type Actor%20Object%20Reference) (OtherComp :type Primitive%20Component%20Object%20Reference) (bSelfMoved :type Boolean) (HitLocation :type Vector :default "0, 0, 0") (HitNormal :type Vector :default "0, 0, 0") (NormalImpulse :type Vector :default "0, 0, 0") (Hit :type Hit%20Result%20Structure%20%28by%20ref%29))
  (if (!= Other "/Game/Blueprints/AircraftBaseClass/BP_Flare.BP_Flare")
    (CallFunction|Explode)))

(fn ConstructionScript)

(fn ProximityDet
  (Utilities|IsValid 0
    (:Is%20Valid
      (if (<= (Math|Vector|Distance(Vector) (Transformation|GetActorLocation) (Transformation|GetActorLocation)) 5e+03)
        (CallFunction|RPCServerDamage)))))

(fn EjectfromOrigin
  (params (Delta :type Float%20%28double-precision%29)))

(fn SafeDestroy
  (bind _returnvalue (Transformation|GetActorTransform))
  (Effects|SpawnEmitteratLocation "/Game/StarterContent/Particles/P_Explosion.P_Explosion" (.location _returnvalue) (.rotation _returnvalue) (* (.scale _returnvalue) 4.0))
  (Actor|DestroyActor))

(fn Explode
  (if (Variables|Default|GetIsDeployed)
    (Niagara|SpawnSystematLocation "/Niagara/DefaultAssets/Templates/Systems/SimpleExplosion.SimpleExplosion" (Transformation|GetActorLocation) "0, 0, 0" "5.000000,5.000000,5.000000")
    (Components|Activation|Deactivate (Variables|Default|GetGenMissileSam))
    (Actor|DestroyActor)))