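; GMC (General Movement Component) flight movement for BP_Aircraft, with networked prediction bindings for rotation, speed and input state.
; Pitch, yaw and roll inputs rotate the camera, and each prediction tick lerps the aircraft toward that camera rotation.
; Throttle input drives interpolated forward speed, with a timed dash boost and a toggleable FCS mode that limits pitch/yaw by a speed curve.
; Dead aircraft keep moving forward while nosing down.
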(event Custom|Dash
  (Variables|Default|SetIsDash true)
  (Utilities|FlowControl|Delay 0.6)
  (Variables|Default|SetIsDash false))

(event Input|EnhancedActionEvents|EnhancedInputActionPitch
  (params (ActionValue :type Float%20%28double-precision%29) (ElapsedSeconds :type Float%20%28double-precision%29) (TriggeredSeconds :type Float%20%28double-precision%29) (InputAction :type Input%20Action%20Object%20Reference :default "/Game/Input/Actions/Pitch.Pitch"))
  (:Triggered
    (CallFunction|CamPitchF ActionValue))
  (:Canceled
    (CallFunction|CamPitchRecF :!label _label))
  (:Completed
    (goto _label)))

(event Input|EnhancedActionEvents|EnhancedInputActionYaw
  (params (ActionValue :type Float%20%28double-precision%29) (ElapsedSeconds :type Float%20%28double-precision%29) (TriggeredSeconds :type Float%20%28double-precision%29) (InputAction :type Input%20Action%20Object%20Reference :default "/Game/Input/Actions/Yaw.Yaw"))
  (:Triggered
    (CallFunction|CamYawF ActionValue))
  (:Canceled
    (CallFunction|CamYawRecF :!label _label))
  (:Completed
    (goto _label)))

(event Input|EnhancedActionEvents|EnhancedInputActionRoll
  (params (ActionValue :type Float%20%28double-precision%29) (ElapsedSeconds :type Float%20%28double-precision%29) (TriggeredSeconds :type Float%20%28double-precision%29) (InputAction :type Input%20Action%20Object%20Reference :default "/Game/Input/Actions/Roll.Roll"))
  (:Triggered
    (CallFunction|CamRollF ActionValue))
  (:Canceled
    (CallFunction|CamRollRecF :!label _label))
  (:Completed
    (goto _label)))

(event Input|EnhancedActionEvents|EnhancedInputActionAccelerateDecelerate
  (params (ActionValue :type Float%20%28double-precision%29) (ElapsedSeconds :type Float%20%28double-precision%29) (TriggeredSeconds :type Float%20%28double-precision%29) (InputAction :type Input%20Action%20Object%20Reference :default "/Game/Input/Actions/AccelerateDecelerate.AccelerateDecelerate"))
  (:Triggered
    (CallFunction|Speed0 ActionValue (Class|GMCMovementUtilityCmp|GetPhysDeltaTime) :!label _label))
  (:Ongoing
    (goto _label)))

(event Input|EnhancedActionEvents|EnhancedInputActionFCSMode
  (params (ActionValue :type Boolean) (ElapsedSeconds :type Float%20%28double-precision%29) (TriggeredSeconds :type Float%20%28double-precision%29) (InputAction :type Input%20Action%20Object%20Reference :default "/Game/Input/Actions/FCSMode.FCSMode"))
  (:Triggered
    (Utilities|FlowControl|FlipFlop
      (:A
        (Variables|Default|SetFCSLimit false))
      (:B
        (Variables|Default|SetFCSLimit true)))))

(event EventGenPredictionTick
  (params (DeltaTime :type Float%20%28single-precision%29))
  (if (Variables|/Game/Blueprints/Old/BP_Aircraft.BP_Aircraft_C|GetIsAlive (Variables|Default|GetPlayerPawnRef))
    (CallFunction|RollF)
    (CallFunction|PitchF)
    (CallFunction|YawF)
    (CallFunction|CopyRot2)
    (CallFunction|UpdatePosition (Class|GMCMovementUtilityCmp|GetPhysDeltaTime))
    (Class|MovementComponent|MoveUpdatedComponent (* (Class|GMCReplicationCmp|GetVelocity) (Class|GMCMovementUtilityCmp|GetPhysDeltaTime) 2e+01) (Class|GMCMovementUtilityCmp|GetRootCollisionRotation) true)
    (else
      (Class|MovementComponent|MoveUpdatedComponent (* (Transformation|GetActorForwardVector (Components|GetOwner)) 4e+01) (Math|Rotator|Lerp(Rotator) (Variables|Default|GetFInalRot) (Math|Rotator|MakeRotator 0.0 -9e+01 0.0) 0.7 true) true))))

(event EventBindReplicationData
  (|CallParentFunction)
  (Class|GMCReplicationCmp|BindCompressedRotator (Variables|Default|GetFInalRot) "ClientAuth_Input" "CombineIfUnchanged" "None" "NearestNeighbour")
  (Class|GMCReplicationCmp|BindCompressedRotator (Variables|Default|GetFInalRot) "ClientAuth_Input" "CombineIfUnchanged" "None" "NearestNeighbour")
  (Class|GMCReplicationCmp|BindDoublePrecisionFloat (Variables|Default|GetCurrentRoll) "ServerAuth_Output_ClientValidated" "CombineIfUnchanged" "None" "NearestNeighbour")
  (Class|GMCReplicationCmp|BindDoublePrecisionFloat (Variables|Default|GetCurrentPitch) "ServerAuth_Output_ClientValidated" "CombineIfUnchanged" "None" "NearestNeighbour")
  (Class|GMCReplicationCmp|BindDoublePrecisionFloat (Variables|Default|GetCurrentYaw) "ServerAuth_Output_ClientValidated" "CombineIfUnchanged" "None" "NearestNeighbour")
  (Class|GMCReplicationCmp|BindDoublePrecisionFloat (Variables|Default|GetTargetRoll) "ClientAuth_Input" "CombineIfUnchanged" "None" "NearestNeighbour")
  (Class|GMCReplicationCmp|BindDoublePrecisionFloat (Variables|Default|GetTargetYaw) "ClientAuth_Input" "CombineIfUnchanged" "None" "NearestNeighbour")
  (Class|GMCReplicationCmp|BindDoublePrecisionFloat (Variables|Default|GetTargetPitch) "ClientAuth_Input" "CombineIfUnchanged" "None" "NearestNeighbour")
  (Class|GMCReplicationCmp|BindDoublePrecisionFloat (Variables|Default|GetCurrentSpeed) "ServerAuth_Output_ClientValidated" "CombineIfUnchanged" "None" "NearestNeighbour")
  (Class|GMCReplicationCmp|BindDoublePrecisionFloat (Variables|Default|GetThrustSpeed) "ClientAuth_Input" "CombineIfUnchanged" "None" "NearestNeighbour")
  (Class|GMCReplicationCmp|BindBool (Variables|Default|GetFCSLimit) "ServerAuth_InputOutput_ServerValidated" "CombineIfUnchanged" "None" "NearestNeighbour")
  (Class|GMCReplicationCmp|BindBool (Variables|Default|GetIsDash) "ServerAuth_InputOutput_ServerValidated" "CombineIfUnchanged" "None" "NearestNeighbour"))

(event EventBeginPlay
  (bind _asbp_aircraft (Utilities|Casting|CastToBP_Aircraft (Components|GetOwner)))
  (bind _output_get (Variables|Default|SetPlayerPawnRef _asbp_aircraft))
  (Variables|Default|SetP_Camera (Variables|/Game/Blueprints/Old/BP_Aircraft.BP_Aircraft_C|GetCamera _output_get))
  (bind _asgmc_controller (Utilities|Casting|CastToGMC_Controller (Game|GetPlayerController 0)))
  (Utilities|IsValid (PlayerController|LocalPlayerSubsystems|GetEnhancedInputLocalPlayerSubsystem _asgmc_controller)
    (:Is%20Valid
      (Input|AddMappingContext (PlayerController|LocalPlayerSubsystems|GetEnhancedInputLocalPlayerSubsystem _asgmc_controller) "/Game/Input/NewInputMappingContext.NewInputMappingContext" 0 "(bIgnoreAllPressedKeysUntilRelease=True,bForceImmediately=False)"))))

(fn CamRollF
  (params (AngleDegrees :type Float%20%28double-precision%29))
  (bind _maxlook (Variables|Default|GetMaxLook))
  (bind _returnvalue (* _maxlook 0.35))
  (Variables|Default|SetTargetRoll (Math|Float|ClampAngle AngleDegrees (* _returnvalue -1.0) _returnvalue)))

(fn CamRollRecF
  (Variables|Default|SetTargetRoll (Math|Interpolation|FInterpTo (Variables|Default|GetTargetRoll) 0.0 (Variables|Default|GetDeltaSeconds) 0.0)))

(fn CamPitchF
  (params (AngleDegrees :type Float%20%28double-precision%29))
  (bind _currentspeed (Variables|Default|GetCurrentSpeed))
  (bind _maxlook (Variables|Default|GetMaxLook))
  (bind _fcslimit (Variables|Default|GetFCSLimit))
  (bind _rotationcurve (Variables|Default|GetRotationCurve))
  (bind _returnvalue (Math|Curves|GetFloatValue _rotationcurve _currentspeed))
  (bind _returnvalue_2 (Math|Float|Clamp(Float) _returnvalue 0.1))
  (bind _returnvalue_3 (select _fcslimit _returnvalue_2 _maxlook))
  (bind _returnvalue_4 (* _returnvalue_3 2.0))
  (Variables|Default|SetTargetPitch (Math|Float|ClampAngle AngleDegrees (* _returnvalue_4 -1.0) _returnvalue_4)))

(fn CamPitchRecF
  (Variables|Default|SetTargetPitch (Math|Interpolation|FInterpTo (Variables|Default|GetTargetPitch) 0.0 (Variables|Default|GetDeltaSeconds) 0.0)))

(fn CamYawF
  (params (AngleDegrees :type Float%20%28double-precision%29))
  (bind _currentspeed (Variables|Default|GetCurrentSpeed))
  (bind _maxlook (Variables|Default|GetMaxLook))
  (bind _fcslimit (Variables|Default|GetFCSLimit))
  (bind _rotationcurve (Variables|Default|GetRotationCurve))
  (bind _returnvalue (Math|Curves|GetFloatValue _rotationcurve _currentspeed))
  (bind _returnvalue_2 (Math|Float|Clamp(Float) _returnvalue 0.1))
  (bind _returnvalue_3 (select _fcslimit _returnvalue_2 _maxlook))
  (bind _returnvalue_4 (* _returnvalue_3 1.2))
  (Variables|Default|SetTargetYaw (Math|Float|ClampAngle AngleDegrees (* _returnvalue_4 -1.0) _returnvalue_4)))

(fn CamYawRecF
  (Variables|Default|SetTargetYaw (Math|Interpolation|FInterpTo (Variables|Default|GetTargetYaw) 0.0 (Variables|Default|GetDeltaSeconds) 0.0)))

(fn CopyRot
  (bind _returnvalue (Class|GMCReplicationCmp|GetGMCPawnOwner))
  (bind _playerpawnref (Variables|Default|GetPlayerPawnRef))
  (bind _returnvalue_2 (Transformation|GetActorRotation _returnvalue))
  (Utilities|IsValid _playerpawnref
    (:Is%20Valid
      (Transformation|SetWorldRotation (Variables|/Game/Blueprints/Old/BP_Aircraft.BP_Aircraft_C|Getcamroot _playerpawnref) (Variables|Default|GetSpawnRot) false false)
      (bind _output_get (Variables|Default|SetTargetRotation (Math|Rotator|Lerp(Rotator) (Variables|Default|GetTargetRotation) (Transformation|GetSocketRotation (Variables|Default|GetP_Camera) "None") 1.0 true)))
      (Utilities|FlowControl|Sequence
        (:then_0
          (CallFunction|Roll2 (.roll _returnvalue_2) (.roll _output_get)))
        (:then_1
          (CallFunction|Pitch2 (.pitch _returnvalue_2) (.pitch _output_get)))
        (:then_2
          (CallFunction|Yaw2 (.yaw _returnvalue_2) (.yaw _output_get)))
        (:then_3
          (bind _output_get_2 (Variables|Default|SetFInalRot (Math|Rotator|MakeRotator (Variables|Default|GetAVRoll) (Variables|Default|GetAVPitch) (Variables|Default|GetAVYaw))))
          (Transformation|AddActorLocalRotation (Class|GMCReplicationCmp|GetGMCPawnOwner) _output_get_2 false false)
          (return _output_get_2))))))

(fn UpdatePosition
  (params (Delta :type Float%20%28double-precision%29))
  (bind _returnvalue (Class|GMCMovementUtilityCmp|GetPhysDeltaTime))
  (Variables|Default|SetCurrentSpeed (Math|Float|Clamp(Float) (Math|Interpolation|FInterpTo (Variables|Default|GetCurrentSpeed) (Variables|Default|GetThrustSpeed) Delta (Variables|Default|GetDrag)) 0.0 (Variables|Default|GetMaxThrustSpeed)))
  (if (Variables|Default|GetIsDash)
    (Class|GMCMovementUtilityCmp|UpdateVelocity (* (Transformation|GetActorForwardVector (Components|GetOwner)) (+ (* (Math|Float|Clamp(Float) (Variables|Default|GetCurrentSpeed) 0.0 1.5e+03) 0.2) (Variables|Default|GetDashBoost))) _returnvalue)
    (return (* (Transformation|GetActorForwardVector (Components|GetOwner)) (+ (* (Math|Float|Clamp(Float) (Variables|Default|GetCurrentSpeed) 0.0 1.5e+03) 0.2) (Variables|Default|GetDashBoost))))
    (else
      (Class|GMCMovementUtilityCmp|UpdateVelocity (* (* (Transformation|GetActorForwardVector (Components|GetOwner)) (Variables|Default|GetCurrentSpeed)) Delta) _returnvalue)
      (return (* (* (Transformation|GetActorForwardVector (Components|GetOwner)) (Variables|Default|GetCurrentSpeed)) Delta)))))

(fn RollF
  (bind _p_camera (Variables|Default|GetP_Camera))
  (bind _output_get (Variables|Default|SetCurrentRoll (Math|Interpolation|FInterpTo (Variables|Default|GetCurrentRoll) (Variables|Default|GetTargetRoll) (Class|GMCMovementUtilityCmp|GetPhysDeltaTime) (Variables|Default|GetInterp%20Speed))))
  (Utilities|IsValid _p_camera
    (:Is%20Valid
      (Transformation|AddLocalRotation _p_camera (Math|Rotator|MakeRotator (* _output_get 5.0) 0.0 0.0) false false))))

(fn PitchF
  (bind _p_camera (Variables|Default|GetP_Camera))
  (bind _output_get (Variables|Default|SetCurrentPitch (Math|Interpolation|FInterpTo (Variables|Default|GetCurrentPitch) (Variables|Default|GetTargetPitch) (Class|GMCMovementUtilityCmp|GetPhysDeltaTime) (Variables|Default|GetInterp%20Speed))))
  (Utilities|IsValid _p_camera
    (:Is%20Valid
      (Transformation|AddLocalRotation _p_camera (Math|Rotator|MakeRotator 0.0 (* _output_get (Variables|Default|GetTurnspeed) 1.0) 0.0) false false))))

(fn YawF
  (bind _p_camera (Variables|Default|GetP_Camera))
  (bind _output_get (Variables|Default|SetCurrentYaw (Math|Interpolation|FInterpTo (Variables|Default|GetCurrentYaw) (Variables|Default|GetTargetYaw) (Class|GMCMovementUtilityCmp|GetPhysDeltaTime) (Variables|Default|GetInterp%20Speed))))
  (Utilities|IsValid _p_camera
    (:Is%20Valid
      (Transformation|AddLocalRotation _p_camera (Math|Rotator|MakeRotator 0.0 0.0 (* _output_get (Variables|Default|GetTurnspeed) 1.0)) false false))))

(fn Speed0
  (params (Speed :type Float%20%28double-precision%29) (Delta :type Float%20%28double-precision%29))
  (Variables|Default|SetThrustSpeed (Math|Float|Clamp(Float) (+ (* Speed Delta (Variables|Default|GetThrustMultiplier)) (Variables|Default|GetThrustSpeed)) 0.0 (Variables|Default|GetMaxThrustSpeed))))

(fn CopyRot2
  (bind _playerpawnref (Variables|Default|GetPlayerPawnRef))
  (Utilities|IsValid _playerpawnref
    (:Is%20Valid
      (Transformation|SetWorldRotation (Variables|/Game/Blueprints/Old/BP_Aircraft.BP_Aircraft_C|Getcamroot _playerpawnref) (Variables|Default|GetSpawnRot) false false)
      (bind _output_get (Variables|Default|SetTargetRotation (Math|Rotator|Lerp(Rotator) (Variables|Default|GetTargetRotation) (Transformation|GetSocketRotation (Variables|Default|GetP_Camera) "None") 1.0 true)))
      (bind _output_get_2 (Variables|Default|SetFInalRot (Math|Rotator|Lerp(Rotator) (Transformation|GetActorRotation (Class|GMCReplicationCmp|GetGMCPawnOwner)) _output_get 0.1 true)))
      (Transformation|SetActorRotation (Class|GMCReplicationCmp|GetGMCPawnOwner) _output_get_2)
      (return "0, 0, 0"))))

(fn Yaw2
  (params (A :type Float%20%28double-precision%29) (B :type Float%20%28double-precision%29))
  (Utilities|ComparewithError (Variables|Default|GeterrorMargin) A B
    (:EqualAbout
      (Variables|Default|SetAVYaw (Math|Interpolation|FInterptoConstant (Variables|Default|GetAVYaw) 0.0 (Class|GMCMovementUtilityCmp|GetPhysDeltaTime) 1.0)))
    (:Less
      (Variables|Default|SetAVYaw (Math|Interpolation|FInterptoConstant (Variables|Default|GetAVYaw) (+ (Variables|Default|GetAVYaw) 1.0) (Class|GMCMovementUtilityCmp|GetPhysDeltaTime) 1.0)))
    (:Greater
      (Variables|Default|SetAVYaw (Math|Interpolation|FInterptoConstant (Variables|Default|GetAVYaw) (- (Variables|Default|GetAVYaw) 1.0) (Class|GMCMovementUtilityCmp|GetPhysDeltaTime) 1.0)))))

(fn Pitch2
  (params (A :type Float%20%28double-precision%29) (B :type Float%20%28double-precision%29))
  (Utilities|ComparewithError (Variables|Default|GeterrorMargin) A B
    (:EqualAbout
      (Variables|Default|SetAVPitch (Math|Interpolation|FInterptoConstant (Variables|Default|GetAVPitch) 0.0 (Class|GMCMovementUtilityCmp|GetPhysDeltaTime) 1.0)))
    (:Less
      (Variables|Default|SetAVPitch (Math|Interpolation|FInterptoConstant (Variables|Default|GetAVPitch) (+ (Variables|Default|GetAVPitch) 1.0) (Class|GMCMovementUtilityCmp|GetPhysDeltaTime) 1.0)))
    (:Greater
      (Variables|Default|SetAVPitch (Math|Interpolation|FInterptoConstant (Variables|Default|GetAVPitch) (- (Variables|Default|GetAVPitch) 1.0) (Class|GMCMovementUtilityCmp|GetPhysDeltaTime) 1.0)))))

(fn Roll2
  (params (A :type Float%20%28double-precision%29) (B :type Float%20%28double-precision%29))
  (Utilities|ComparewithError (Variables|Default|GeterrorMargin) A B
    (:EqualAbout
      (Variables|Default|SetAVRoll (Math|Interpolation|FInterptoConstant (Variables|Default|GetAVRoll) 0.0 (Class|GMCMovementUtilityCmp|GetPhysDeltaTime) 1.0)))
    (:Less
      (Variables|Default|SetAVRoll (Math|Interpolation|FInterptoConstant (Variables|Default|GetAVRoll) (+ (Variables|Default|GetAVRoll) 1.0) (Class|GMCMovementUtilityCmp|GetPhysDeltaTime) 1.0)))
    (:Greater
      (Variables|Default|SetAVRoll (Math|Interpolation|FInterptoConstant (Variables|Default|GetAVRoll) (- (Variables|Default|GetAVRoll) 1.0) (Class|GMCMovementUtilityCmp|GetPhysDeltaTime) 1.0)))))