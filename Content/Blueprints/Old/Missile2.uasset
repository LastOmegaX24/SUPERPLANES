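; Homing missile carried by BP_Aircraft2 that damages non-weapon actors it overlaps, spawns a hit mark and destroys itself.
; MissileFireM sets the aircraft's lock target as the homing target of ProjectileMovement.
; Tick runs through RPC events; once IsAttatched is false, it detaches, launches at aircraft speed plus a boost and starts Niagara.
; Manual steering, thrust/gravity movement, proximity detection and explosion functions exist but are not called here.
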(event Custom|RPC_Particle
  (Components|Activation|Activate (Variables|Default|GetNiagara) false))

(event Custom|RPC_Server_Missile
  (params (Delta :type Float%20%28double-precision%29))
  (CallFunction|RPCMissile Delta))

(event Custom|RPC_Missile
  (params (Delta :type Float%20%28double-precision%29))
  (if (not (Variables|Default|GetIsAttatched))
    (Rendering|SetVisibility (Variables|Default|GetWidget) true true)
    (if (not (Variables|Default|GetIsDeployed))
      (Transformation|DetachFromActor "KeepWorld" "KeepWorld" "KeepWorld")
      (CallFunction|EjectfromOrigin Delta)
      (CallFunction|RPCParticle)
      (Variables|Default|SetIsDeployed true))))

(event Custom|RPC_Damage
  (params (NewParam :type Actor%20Object%20Reference))
  (Utilities|IsValid NewParam
    (:Is%20Valid
      (if (not (Actor|ActorHasTag NewParam "Weapon"))
        (if (not (== NewParam (Components|GetOwner)))
          (Game|Damage|ApplyDamage NewParam (Variables|Default|GetBaseDamage) (Pawn|GetController (Game|GetInstigator)) (Game|GetInstigator) "/Game/Blueprints/MainSystem/StandardDamage.StandardDamage_C")
          (Game|SpawnActorfromClass "/Game/Blueprints/HitMarkActor.HitMarkActor_C" (Transformation|GetActorTransform) "Undefined" 0 0)
          (Actor|DestroyActor))))))

(event Custom|RPC_Server_Damage
  (params (OtherActor :type Actor%20Object%20Reference))
  (CallFunction|RPCDamage OtherActor))

(event Custom|MissileFireM
  (bind _playerref (Variables|Default|GetPlayerRef))
  (bind _locktarget (Variables|/Game/Blueprints/BP_Aircraft2.BP_Aircraft2_C|GetLockTarget _playerref))
  (Utilities|IsValid _playerref
    (:Is%20Valid
      (Utilities|IsValid _locktarget
        (:Is%20Valid
          (Development|PrintString "Hello")
          (bind _output_get (Variables|Default|SetCurrentTarget _locktarget))
          (Variables|/Script/Engine.ProjectileMovementComponent|SetHomingTargetComponent (Variables|Default|GetProjectileMovement) (Variables|/Script/Engine.Actor|GetRootComponent _output_get))
          (Development|PrintString (Utilities|GetDisplayName (Variables|/Script/Engine.Actor|GetRootComponent _output_get))))))))

(event EventBeginPlay
  (bind _asbp_aircraft_2 (Utilities|Casting|CastToBP_Aircraft2 (Game|GetInstigator)))
  (bind _output_get (Variables|Default|SetPlayerRef _asbp_aircraft_2))
  (Collision|IgnoreActorwhenMoving (Variables|Default|GetStaticMesh) _output_get true))

(event Collision|EventActorBeginOverlap
  (params (OtherActor :type Actor%20Object%20Reference))
  (CallFunction|RPCServerDamage OtherActor))

(event Collision|EventHit
  (params (MyComp :type Primitive%20Component%20Object%20Reference) (Other :type Actor%20Object%20Reference) (OtherComp :type Primitive%20Component%20Object%20Reference) (bSelfMoved :type Boolean) (HitLocation :type Vector :default "0, 0, 0") (HitNormal :type Vector :default "0, 0, 0") (NormalImpulse :type Vector :default "0, 0, 0") (Hit :type Hit%20Result%20Structure%20%28by%20ref%29)))

(event EventTick
  (params (DeltaSeconds :type Float%20%28single-precision%29))
  (CallFunction|RPCServerMissile DeltaSeconds))

(fn ConstructionScript)

(fn ProximityDet
  (bind _current_target (Variables|Default|GetCurrent%20Target))
  (Utilities|IsValid _current_target
    (:Is%20Valid
      (if (<= (Math|Vector|Distance(Vector) (Transformation|GetActorLocation _current_target) (Transformation|GetActorLocation)) 5e+03)
        (CallFunction|RPCServerDamage)))))

(fn UpdatePosition
  (params (Delta :type Float%20%28double-precision%29))
  ;[1 1 1] Calc Current Speed
  (Variables|Default|SetCurrentSpeed (Math|Float|Clamp(Float) (Math|Interpolation|FInterpTo (Variables|Default|GetCurrentSpeed) (Variables|Default|GetThrustSpeed) Delta (Variables|Default|GetDrag)) 0.0 (Variables|Default|GetMaxThrustSpeed)))
  ;[1 1 1] Calc new position based on speed
  (Variables|Default|SetNewPos (* (* (Variables|Default|GetCurrentSpeed) Delta) (Transformation|GetActorForwardVector)))
  ;[1 1 1] Calc Applied Gravity
  (Variables|Default|SetAppliedGravity (Math|Float|MapRangeClamped (Variables|Default|GetCurrentSpeed) 0.0 (Variables|Default|GetMinThrustStall) (Variables|Default|GetGravity) 0.0))
  ;[1 1 1] Get Position
  (Transformation|AddActorWorldOffset (Math|Vector|MakeVector (.X (Class|KismetMathLibrary|BreakVector3f (Variables|Default|GetNewPos))) (.Y (Class|KismetMathLibrary|BreakVector3f (Variables|Default|GetNewPos))) (- (.Z (Class|KismetMathLibrary|BreakVector3f (Variables|Default|GetNewPos))) (* (Variables|Default|GetAppliedGravity) 1.0))) true)
  (Variables|Default|SetThrustSpeed (Math|Float|Clamp(Float) (Math|Interpolation|FInterpTo (Variables|Default|GetThrustSpeed) 0.0 Delta (Variables|Default|GetDrag)) 3.5e+03 (Variables|Default|GetMaxThrustSpeed))))

(fn EjectfromOrigin
  (params (Delta :type Float%20%28double-precision%29))
  (bind _projectilemovement (Variables|Default|GetProjectileMovement))
  (Variables|/Script/Engine.ProjectileMovementComponent|SetInitialSpeed _projectilemovement (+ (Variables|/Game/Blueprints/BP_Aircraft2.BP_Aircraft2_C|GetCurrentSpeed (Variables|Default|GetPlayerRef)) (Variables|Default|GetAddSpeed)))
  (Variables|/Script/Engine.ProjectileMovementComponent|SetbIsHomingProjectile _projectilemovement true)
  (Components|Activation|Activate (Variables|Default|GetProjectileMovement) false))

(fn Main
  (params (Delta :type Float%20%28double-precision%29))
  (bind _currenttarget (Variables|Default|GetCurrentTarget))
  (Utilities|IsValid _currenttarget
    (:Is%20Valid
      (Transformation|SetActorRotation (Class|KismetMathLibrary|RInterptoConstant (Transformation|GetActorRotation) (Math|Rotator|FindLookatRotation (Transformation|GetActorLocation) (Transformation|GetActorLocation _currenttarget)) Delta (Variables|Default|GetTurnspeed))))
    (:Is%20Not%20Valid
      _))
  (CallFunction|UpdatePosition Delta))

(fn SafeDestroy
  (bind _returnvalue (Transformation|GetActorTransform))
  (Effects|SpawnEmitteratLocation "/Game/StarterContent/Particles/P_Explosion.P_Explosion" (.location _returnvalue) (.rotation _returnvalue) (* (.scale _returnvalue) 4.0))
  (Actor|DestroyActor))