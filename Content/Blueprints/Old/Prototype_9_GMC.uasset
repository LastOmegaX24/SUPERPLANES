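; Prototype player pawn Blueprint that sets up input, HUD and startup hooks on BeginPlay.
; After casting its controller to GEN_Controller, it validates the Enhanced Input subsystem, then adds a mapping context and displays a HUD widget for player 0.
; It then calls radar, lock-hiding and server weapon setup functions, all of which are empty stubs here.
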(event EventBeginPlay
  (bind _asgen_controller (Utilities|Casting|CastToGEN_Controller (Pawn|GetController)))
  (Utilities|IsValid (PlayerController|LocalPlayerSubsystems|GetEnhancedInputLocalPlayerSubsystem _asgen_controller)
    (:Is%20Valid
      (Input|AddMappingContext (PlayerController|LocalPlayerSubsystems|GetEnhancedInputLocalPlayerSubsystem _asgen_controller) "/Game/Input/NewInputMappingContext.NewInputMappingContext" 0 "(bIgnoreAllPressedKeysUntilRelease=True,bForceImmediately=False)")
      (bind _returnvalue (UserInterface|CreateWidget "/Game/HUD/HUD_Widget.HUD_Widget_C" (Game|GetPlayerController 0)))
      (UserInterface|Viewport|AddtoViewport _returnvalue 0)
      (CallFunction|RealizeRadarOptions)
      (CallFunction|HideLockforSelf)
      (CallFunction|RPCServerRealizeWeapons))))

(fn ConstructionScript)

(fn HideLockforSelf)

(fn RealizeRadarOptions)

(fn RPCServerRealizeWeapons)