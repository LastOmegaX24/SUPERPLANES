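; BP_Railgun_Pr is a railgun projectile actor that damages what it overlaps and has a limited lifespan.
; On spawn it ignores its instigator and owner when moving.
; Overlaps route through a server RPC event into a damage event, which skips the owner and actors tagged Weapon.
; A valid hit receives standard damage credited to the instigator and its controller, then the projectile destroys itself.
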(event Custom|RPC_Damage
  (params (NewParam :type Actor%20Object%20Reference))
  (Utilities|IsValid NewParam
    (:Is%20Valid
      (if (not (Actor|ActorHasTag NewParam "Weapon"))
        (if (not (== NewParam (Components|GetOwner)))
          (Game|Damage|ApplyDamage NewParam (Variables|Default|GetBaseDamage) (Pawn|GetController (Game|GetInstigator)) (Game|GetInstigator) "/Game/Blueprints/MainSystem/StandardDamage.StandardDamage_C")
          (Actor|DestroyActor))))))

(event Custom|RPC_Server_Damage
  (params (NewParam :type Actor%20Object%20Reference))
  (CallFunction|RPCDamage NewParam))

(event Collision|EventActorBeginOverlap
  (params (OtherActor :type Actor%20Object%20Reference))
  (CallFunction|RPCServerDamage OtherActor))

(event EventBeginPlay
  (bind _root (Variables|Default|Getroot))
  (Actor|SetLifeSpan 2e+01)
  (Collision|IgnoreActorwhenMoving _root (Variables|Actor|GetInstigator) true)
  (Collision|IgnoreActorwhenMoving _root (Components|GetOwner) true))

(fn ConstructionScript)