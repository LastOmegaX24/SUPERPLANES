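; Default special-weapon Blueprint that fires BP_Railgun_Pr projectiles while it has ammo.
; FireCall forwards an index to the railgun RPC event, which delays by that index to stagger shots.
; Each shot spawns a projectile at the Arrow transform, passing on owner and instigator, then decrements Ammo.
; With no ammo left, it sets IsEmpty to false, despite the flag's name.
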(event Custom|RPC_Railgun
  (params (Index :type Integer))
  (if (> (Variables|Default|GetAmmo) 0)
    (Utilities|FlowControl|Delay (* Index 0.1))
    (Game|SpawnActorfromClass "/Game/Blueprints/Special/BP_Railgun_Pr.BP_Railgun_Pr_C" (Transformation|GetWorldTransform (Variables|Default|GetArrow)) "AlwaysSpawn" (Components|GetOwner) (Game|GetInstigator))
    (Math|Integer|DecrementInt (Variables|Default|GetAmmo))
    (else
      (Variables|Default|SetIsEmpty false))))

(event Custom|FireCall
  (params (Index :type Integer))
  (CallFunction|RPCRailgun Index))

(fn ConstructionScript)