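; Destructible structure actor with hit points that explodes when its health runs out.
; Any damage lowers health, clamped between zero and its maximum.
; At zero health it marks itself dead, spawns a large explosion effect at its location and tells its map icon component that it is no longer alive.
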(event Game|Damage|EventAnyDamage
  (params (Damage :type Float%20%28single-precision%29) (DamageType :type Damage%20Type%20Object%20Reference) (InstigatedBy :type Controller%20Object%20Reference) (DamageCauser :type Actor%20Object%20Reference))
  (bind _output_get (Variables|Default|SetHealth (Math|Float|Clamp(Float) (- (Variables|Default|GetHealth) Damage) 0.0 (Variables|Default|GetMaxHealth))))
  (if (<= _output_get 0.0)
    (Variables|Default|SetIsAlive false)
    (Niagara|SpawnSystematLocation "/Niagara/DefaultAssets/Templates/Systems/SimpleExplosion.SimpleExplosion" (Transformation|GetActorLocation) "0, 0, 0" "20.000000,20.000000,20.000000")
    (Class|IsAliveEvent|UpdateIsAlive(Message) (Variables|Default|GetMapIconComponent) false)))

(fn ConstructionScript)