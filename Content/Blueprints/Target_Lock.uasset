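; Target_Lock is an actor that attaches itself to the player's current lock target, apparently as a lock-on marker.
; BeginPlay caches the Prototype_9 player pawn and attaches to its LockTarget, if valid, using relative transforms.
; The ReCast event repeats that attachment using the cached pawn's current LockTarget.
; Tick destroys the actor whenever it has no valid attach parent.
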(event Custom|ReCast
  (bind _playerref (Variables|Default|GetPlayerRef))
  (bind _locktarget (Variables|/Game/Blueprints/Prototype_9.Prototype_9_C|GetLockTarget _playerref))
  (Utilities|IsValid _locktarget
    (:Is%20Valid
      (Transformation|AttachActorToActor _locktarget "" "KeepRelative" "KeepRelative" "KeepRelative" false))))

(event EventTick
  (params (DeltaSeconds :type Float%20%28single-precision%29))
  (Utilities|IsValid (Actor|GetAttachParentActor)
    (:Is%20Not%20Valid
      (Actor|DestroyActor))))

(event EventBeginPlay
  (bind _asprototype_9 (Utilities|Casting|CastToPrototype_9 (Game|Player|GetPlayerPawn 0)))
  (Variables|Default|SetPlayerRef _asprototype_9)
  (Utilities|IsValid (Variables|/Game/Blueprints/Prototype_9.Prototype_9_C|GetLockTarget (Variables|Default|GetPlayerRef))
    (:Is%20Valid
      (Transformation|AttachActorToActor (Variables|/Game/Blueprints/Prototype_9.Prototype_9_C|GetLockTarget (Variables|Default|GetPlayerRef)) "" "KeepRelative" "KeepRelative" "KeepRelative" false))))

(fn ConstructionScript)