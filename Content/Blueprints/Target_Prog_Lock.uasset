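; Target lock-progress marker actor that shows the player aircraft's lock progression on the actor it is attached to, through a Lock_Prog_Widget.
; Tick pushes LockProgression to the widget, stepping it down via a short Delay when not locking, and looks up the target's index in the player's AlreadyTrackingProg.
; LoseLockDelay clears IsLocking after a retriggerable delay.
; The marker destroys itself when its parent or player reference is invalid.
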(event Custom|LoseLockDelay
  (Utilities|FlowControl|RetriggerableDelay 1.0)
  (Variables|Default|SetIsLocking false))

(event EventTick
  (params (DeltaSeconds :type Float%20%28single-precision%29))
  (bind _returnvalue (Actor|GetAttachParentActor))
  (bind _playerref (Variables|Default|GetPlayerRef))
  (Utilities|IsValid _returnvalue
    (:Is%20Valid
      (Utilities|IsValid _playerref
        (:Is%20Valid
          (Variables|Default|SetCurrentTargetIndex (Utilities|Array|FindItem (Variables|/Game/Blueprints/AircraftBaseClass/BP_Aircraft2.BP_Aircraft2_C|GetAlreadyTrackingProg _playerref) _returnvalue))
          (if (Variables|Default|GetIsLocking)
            (Variables|/Game/HUD/Lock_Prog_Widget.Lock_Prog_Widget_C|SetLockProgression (Variables|Default|GetAs%20Lock%20Prog%20Widget) (Variables|Default|GetLockProgression))
            (else
              (Utilities|FlowControl|Delay 0.01)
              (Variables|Default|SetLockProgression (- (Variables|Default|GetLockProgression) 0.01))
              (Variables|/Game/HUD/Lock_Prog_Widget.Lock_Prog_Widget_C|SetLockProgression (Variables|Default|GetAs%20Lock%20Prog%20Widget) (Variables|Default|GetLockProgression)))))
        (:Is%20Not%20Valid
          (Actor|DestroyActor :!label _label))))
    (:Is%20Not%20Valid
      (goto _label))))

(event EventBeginPlay
  (bind _asbp_aircraft_2 (Utilities|Casting|CastToBP_Aircraft2 (Game|Player|GetPlayerPawn 0)))
  (Variables|Default|SetPlayerRef _asbp_aircraft_2)
  (bind _aslock_prog_widget (Utilities|Casting|CastToLock_Prog_Widget (UserInterface|GetWidget (Variables|Default|GetWidget))))
  (Variables|Default|SetAs%20Lock%20Prog%20Widget _aslock_prog_widget))

(fn ConstructionScript)

(fn OnRepLockProgression)