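; X42A flight actor that steers by following the camera of the player's CamControl pawn.
; Each tick it moves forward with drag and speed-mapped gravity, eases rotation toward the camera, updates thrust from camera input, and computes G-load.
; It takes damage, and defines functions for manual rotation, post-stall turning, alternating gunfire and sphere-trace target lock.
; Lock tracking and turn recovery are disconnected from Tick.
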(event EventBeginPlay
  (bind _ascam_control (Utilities|Casting|CastToCamControl (Game|Player|GetPlayerPawn 0)))
  (Variables|Default|SetParentCamera _ascam_control))

(event EventTick
  (params (DeltaSeconds :type Float%20%28single-precision%29))
  (CallFunction|UpdatePosition DeltaSeconds)
  (CallFunction|CopyRot)
  (CallFunction|Speed)
  (Variables|Default|SetGLoad (* (* (Variables|/Game/Blueprints/CamControl.CamControl_C|GetCurrentPitch (Variables|Default|GetParentCamera)) (Variables|Default|GetCurrentSpeed)) 0.003)))

(event Game|Damage|EventAnyDamage
  (params (Damage :type Float%20%28single-precision%29) (DamageType :type Damage%20Type%20Object%20Reference) (InstigatedBy :type Controller%20Object%20Reference) (DamageCauser :type Actor%20Object%20Reference))
  (Effects|SpawnEmitteratLocation "/Game/StarterContent/Particles/P_Explosion.P_Explosion" "0, 0, 0")
  (Variables|Default|SetHealth (Math|Float|Clamp(Float) (- (Variables|Default|GetHealth) Damage) 0.0 (Variables|Default|GetMaxHealth)))
  (if (<= (Variables|Default|GetHealth) 0.0)
    (Variables|Default|SetIsAlive false)))

(fn ConstructionScript)

(fn ThrottleInput
  (bind _tempname (Variables|Default|GetTempName))
  (if true
    (bind _result (Math|Integer|IncrementInt _tempname))
    (elif true
      (bind _result_2 (Math|Integer|DecrementInt _tempname)))))

(fn UpdatePosition
  (params (DeltaSeconds :type Float%20%28double-precision%29))
  ;[1 1 1] Calc Current Speed
  (Variables|Default|SetCurrentSpeed (Math|Float|Clamp(Float) (select (< (Variables|Default|GetThrustSpeed) (Variables|Default|GetCurrentSpeed)) (Math|Interpolation|FInterpTo (Variables|Default|GetCurrentSpeed) (Variables|Default|GetThrustSpeed) DeltaSeconds (Variables|Default|GetDrag)) (Variables|Default|GetThrustSpeed)) 0.0 (Variables|Default|GetMaxThrustSpeed)))
  ;[1 1 1] Calc new position based on speed
  (Variables|Default|SetNewPos (* (* (Variables|Default|GetCurrentSpeed) DeltaSeconds) (Transformation|GetActorForwardVector)))
  ;[1 1 1] Calc Applied Gravity
  (Variables|Default|SetAppliedGravity (Math|Float|MapRangeClamped (Variables|Default|GetCurrentSpeed) 0.0 (Variables|Default|GetMinThrustStall) (Variables|Default|GetGravity) 0.0))
  ;[1 1 1] Get Position
  (Transformation|AddActorWorldOffset (Math|Vector|MakeVector (.X (Class|KismetMathLibrary|BreakVector3f (Variables|Default|GetNewPos))) (.Y (Class|KismetMathLibrary|BreakVector3f (Variables|Default|GetNewPos))) (- (.Z (Class|KismetMathLibrary|BreakVector3f (Variables|Default|GetNewPos))) (* (Variables|Default|GetAppliedGravity) 1.0))) true)
  (CallFunction|UpdateAnimation))

(fn PrintVar
  (bind _returnvalue (Actor|GetActorOfClass "/Game/Blueprints/CamControl.CamControl_C"))
  (Utilities|FlowControl|Sequence
    (:then_0
      (Development|PrintString (Utilities|String|Append "ThrustSpeed;" (Utilities|String|ToString(Float) (Variables|Default|GetThrustSpeed)))))
    (:then_1
      (Development|PrintString (Utilities|String|Append "CurrentSpeed;" (Utilities|String|ToString(Float) (Variables|Default|GetCurrentSpeed)))))
    (:then_2
      (Development|PrintString (Utilities|String|Append "Yaw;" (Utilities|String|ToString(Float) (Variables|/Game/Blueprints/CamControl.CamControl_C|GetYawRec _returnvalue)))))
    (:then_3
      (Development|PrintString (Utilities|String|Append "Pitch;" (Utilities|String|ToString(Float) (Variables|/Game/Blueprints/CamControl.CamControl_C|GetPitchRec _returnvalue)))))
    (:then_4
      (Development|PrintString (Utilities|String|Append "Roll;" (Utilities|String|ToString(Float) (Variables|/Game/Blueprints/CamControl.CamControl_C|GetRollRec _returnvalue)))))
    (:then_5
      (Development|PrintString (Utilities|String|Append "DeltaSeconds" (Utilities|String|ToString(Float) (Utilities|Time|GetWorldDeltaSeconds)))))))

(fn UpdateYaw
  (params (DeltaSeconds :type Float%20%28double-precision%29) (Yaw :type Float%20%28double-precision%29))
  (bind _output_get (Variables|Default|SetTargetYaw Yaw))
  (Variables|Default|SetCurrentSpeed (- (Variables|Default|GetCurrentSpeed) (* (Math|Float|Absolute(Float) _output_get) 2.0)))
  (bind _output_get_2 (Variables|Default|SetCurrentYaw (Math|Interpolation|FInterpTo (Variables|Default|GetCurrentYaw) (Variables|Default|GetTargetYaw) DeltaSeconds 1e+01)))
  (Transformation|AddActorLocalRotation (Math|Rotator|MakeRotator 0.0 0.0 (* _output_get_2 DeltaSeconds (Variables|Turnspeed|GetTurnspeedZ) 4.0)) false false))

(fn UpdateRoll
  (params (DeltaSeconds :type Float%20%28double-precision%29) (Roll :type Float%20%28double-precision%29))
  (Variables|Default|SetTargetRoll Roll)
  (bind _output_get (Variables|Default|SetCurrentRoll (Math|Interpolation|FInterpTo (Variables|Default|GetCurrentRoll) (Variables|Default|GetTargetRoll) DeltaSeconds 1e+01)))
  (Transformation|AddActorLocalRotation (Math|Rotator|MakeRotator (* _output_get DeltaSeconds 5e+02) 0.0 0.0) false false))

(fn UpdatePitch
  (params (DeltaSeconds :type Float%20%28double-precision%29) (Pitch :type Float%20%28double-precision%29))
  (Variables|Default|SetCurrentPitch Pitch)
  (bind _output_get (Variables|Default|SetTargetPitch (Math|Interpolation|FInterpTo (Variables|Default|GetCurrentPitch) (Variables|Default|GetTargetPitch) 0.0 1e+01)))
  (Transformation|AddActorLocalRotation (Math|Rotator|MakeRotator 0.0 (* _output_get DeltaSeconds (Variables|Turnspeed|GetTurnspeedZ) 1e+01) 0.0) false false))

(fn HighGTurnNPSM
  (if (and (<= (Variables|Default|GetCurrentSpeed) 1.5e+03) (Variables|Default|GetIsPSMCapable))
    (Variables|Turnspeed|SetTurnspeedZ 1e+01)
    (else
      (Variables|Turnspeed|SetTurnspeedZ 3.0))))

(fn Movement)

(fn UpdateTurnRate
  (Variables|Turnspeed|SetTurnspeedZ (* (Math|Float|SafeDivide (Variables|Turnspeed|GetTurnspeedZ) (Variables|Default|GetCurrentSpeed)) 1e+03)))

(fn UpdateAnimation)

(fn UpdateTurnRecovery
  (bind _rollrecover (Variables|Default|GetRollRecover))
  (Variables|Default|SetCurrentRoll (Math|Interpolation|FInterpTo (Variables|Default|GetCurrentRoll) 0.0 (Utilities|Time|GetWorldDeltaSeconds) _rollrecover))
  (Variables|Default|SetCurrentPitch (Math|Interpolation|FInterpTo (Variables|Default|GetCurrentPitch) 0.0 (Utilities|Time|GetWorldDeltaSeconds) _rollrecover))
  (Variables|Default|SetCurrentYaw (Math|Interpolation|FInterpTo (Variables|Default|GetCurrentYaw) 0.0 (Utilities|Time|GetWorldDeltaSeconds) _rollrecover)))

(fn GunFire
  (Utilities|FlowControl|FlipFlop
    (:A
      (Game|SpawnActorfromClass "/Game/Blueprints/BP_Projectile.BP_Projectile_C" (Transformation|GetWorldTransform (Variables|Default|GetFireLocation1)) "AlwaysSpawn" 0 0))
    (:B
      (Game|SpawnActorfromClass "/Game/Blueprints/BP_Projectile.BP_Projectile_C" (Transformation|GetWorldTransform (Variables|Default|GetFireLocation2)) "AlwaysSpawn" 0 0))))

(fn TargetLock
  (bind _radarorigin (Variables|Default|GetRadarOrigin))
  (bind _returnvalue (Transformation|GetWorldLocation _radarorigin))
  (while (< (Variables|Default|GetRadarRange) (Variables|Default|GetRadarMaxRange))
    (Collision|SphereTraceByChannel _returnvalue (+ _returnvalue (* (Math|Vector|GetForwardVector (Transformation|GetWorldRotation _radarorigin)) (Variables|Default|GetRadarRange))) (Variables|Default|GetCurrentRadarRadius) "TraceTypeQuery1" false 0 "ForDuration")
    (Variables|Default|SetCurrentRadarRadius (+ (Variables|Default|GetCurrentRadarRadius) 2e+02))
    (Variables|Default|SetRadarRange (+ (Variables|Default|GetRadarRange) 1e+02)))
  (Variables|Default|SetCurrentRadarRadius 0.0)
  (Variables|Default|SetRadarRange 0.0))

(fn TargetLock2
  (bind _radarorigin (Variables|Default|GetRadarOrigin))
  (bind _returnvalue (Transformation|GetWorldLocation _radarorigin))
  (Variables|Default|GetTargetLockTracker
    (:then
      (Actor|DestroyActor (Variables|Default|GetTargetLockTracker)))
    (:else
      _))
  (Utilities|FlowControl|FlipFlop
    (:A
      (Variables|Default|SetIsTargetLocked true)
      (bind (_outhit _returnvalue_2) (Collision|SphereTraceForObjects _returnvalue (+ _returnvalue (* (Math|Vector|GetForwardVector (Transformation|GetWorldRotation _radarorigin)) (Variables|Default|GetRadarMaxRange))) (Variables|Default|GetRadarRadius) (Utilities|Array|MakeArray "ObjectTypeQuery3") false 0 "ForDuration"))
      (if _returnvalue_2
        (bind _output_get (Variables|Default|SetLockTarget (.HitActor (Collision|BreakHitResult _outhit))))
        (bind _returnvalue_3 (Game|SpawnActorfromClass "/Game/Blueprints/Target_Lock.Target_Lock_C" (Math|Transform|MakeTransform (Transformation|GetActorLocation _output_get) "0, 0, 0" "1.000000,1.000000,1.000000") "Undefined" 0 0))
        (Variables|Default|SetTargetLockTracker _returnvalue_3)))
    (:B
      (Variables|Default|SetIsTargetLocked false)
      (Variables|Default|SetLockTarget 0))))

(fn HideLockforSelf
  (bind _iff (Variables|Default|GetIFF))
  (if (not (Pawn|IsLocallyControlled))
    (Rendering|SetVisibility _iff false false)
    (else
      (Rendering|SetVisibility _iff false false))))

(fn SetScreenRatio)

(fn LockTrackFunction
  (Transformation|SetActorLocation (Variables|Default|GetTargetLockTracker) (Transformation|GetActorLocation (Variables|Default|GetLockTarget)) false false))

(fn CopyRot
  (bind _parentcamera (Variables|Default|GetParentCamera))
  (bind _camera (Variables|/Game/Blueprints/CamControl.CamControl_C|GetCamera _parentcamera))
  (bind _returnvalue (Transformation|GetSocketRotation _camera "None"))
  (Variables|Turnspeed|SetTargetRotation (Math|Rotator|MakeRotator (.roll (Math|Rotator|Lerp(Rotator) (Math|Rotator|MakeRotator (.roll (Variables|Turnspeed|GetTargetRotation)) 0.0 0.0) (Math|Rotator|MakeRotator (.roll _returnvalue) 0.0 0.0) 0.5 true)) (.pitch (Math|Rotator|Lerp(Rotator) (Math|Rotator|MakeRotator 0.0 (.pitch (Variables|Turnspeed|GetTargetRotation)) 0.0) (Math|Rotator|MakeRotator 0.0 (.pitch _returnvalue) 0.0) 0.5 true)) (.yaw (Math|Rotator|Lerp(Rotator) (Math|Rotator|MakeRotator 0.0 0.0 (.yaw (Variables|Turnspeed|GetTargetRotation))) (Math|Rotator|MakeRotator 0.0 0.0 (.yaw _returnvalue)) 0.5 true))))
  (Transformation|SetActorRotation (Math|Rotator|Lerp(Rotator) (Transformation|GetActorRotation) (Variables|Turnspeed|GetTargetRotation) 0.02 true)))

(fn Speed
  (Variables|Default|SetThrustSpeed (Math|Float|Clamp(Float) (+ (* (Variables|/Game/Blueprints/CamControl.CamControl_C|GetSendSpeedData (Variables|Default|GetParentCamera)) (Utilities|Time|GetWorldDeltaSeconds) (Variables|Default|GetThrustMultiplier)) (Variables|Default|GetThrustSpeed)) 0.0 (Variables|Default|GetMaxThrustSpeed))))

(fn DynamicOffset
  (params (Roll :type Float%20%28double-precision%29) (Pitch :type Float%20%28double-precision%29) (Yaw :type Float%20%28double-precision%29)))