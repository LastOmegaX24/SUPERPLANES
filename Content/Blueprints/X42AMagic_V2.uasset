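; Player-flown combat aircraft pawn with throttle, low-speed gravity drop, health and a HUD.
; Inputs and per-tick movement pass through Server-to-RPC event pairs, with Yaw and Pitch cross-wired between handlers.
; Steering rotates the camera and the airframe lerps after it, while speed drives swept forward movement.
; Selectable weapons fire spread bullets or missiles, and a radar box trace tags targets "Homing" and spawns a lock marker.
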(event Custom|RPC_Fire
  (Utilities|FlowControl|Delay 0.01)
  (CallFunction|GunFire))

(event Custom|RPC_Server_Fire
  (CallFunction|RPCFire))

(event Custom|RPC_Server_Pitch
  (params (Action :type Float%20%28double-precision%29))
  (CallFunction|RPCPitch Action))

(event Custom|RPC_Server_Pitch_Rec
  (CallFunction|RPCPitchRec))

(event Custom|RPC_Pitch
  (params (Action :type Float%20%28double-precision%29))
  (CallFunction|CamPitchF Action))

(event Custom|RPC_Pitch_Rec
  (CallFunction|CamPitchRecF))

(event Custom|RPC_Server_Yaw
  (params (Action :type Float%20%28double-precision%29))
  (CallFunction|RPCYaw Action))

(event Custom|RPC_Server_Yaw_Rec
  (CallFunction|RPCYawRec))

(event Custom|RPC_Yaw
  (params (Action :type Float%20%28double-precision%29))
  (CallFunction|CamYawF Action))

(event Custom|RPC_Yaw_Rec
  (CallFunction|CamYawRecF))

(event Custom|RPC_Server_Speed
  (params (Action :type Float%20%28double-precision%29))
  (CallFunction|RPCSpeed Action))

(event Custom|RPC_Speed
  (params (Action :type Float%20%28double-precision%29))
  (CallFunction|Speed Action (Utilities|Time|GetWorldDeltaSeconds)))

(event Custom|RPC_Server_Movement
  (params (Delta :type Float%20%28double-precision%29))
  (CallFunction|RPCMovement Delta))

(event Custom|RPC_Movement
  (params (Delta :type Float%20%28double-precision%29))
  (bind _radarorigin (Variables|Default|GetRadarOrigin))
  (bind _returnvalue (Transformation|GetWorldLocation _radarorigin))
  (CallFunction|UpdatePosition Delta)
  (Transformation|SetWorldRotation (Variables|Default|Getcamroot) "0, 0, 0" false false)
  (Transformation|SetWorldRotation (Variables|Default|Getmaproot) "0, 0, 0" false false)
  (CallFunction|CopyRot)
  (CallFunction|RollF)
  (CallFunction|PitchF)
  (CallFunction|YawF)
  (Variables|Default|SetGLoad (* (* (Variables|Default|GetCurrentPitch) (Variables|Default|GetCurrentSpeed)) 0.003))
  (bind _outhit (Collision|LineTraceByChannel _returnvalue (+ _returnvalue (* (Math|Vector|GetForwardVector (Transformation|GetWorldRotation _radarorigin)) (Variables|Default|GetRadarMaxRange))) "TraceTypeQuery1" false 0 "None"))
  (Variables|Default|SetHitLocation (.impactpoint _outhit))
  (if (not (.bblockinghit _outhit))
    (Variables|Default|SetHitLocation (.traceend _outhit))))

(event Custom|RPC_Server_FireMissile
  (CallFunction|RPCFireMissile))

(event Custom|RPC_Roll
  (params (Action :type Float%20%28double-precision%29))
  (CallFunction|CamRollF Action))

(event Custom|RPC_FireMissile
  (CallFunction|MissileFire))

(event Custom|RPC_Server_Roll
  (params (Action :type Float%20%28double-precision%29))
  (CallFunction|RPCRoll Action))

(event Custom|RPC_Server_Roll_Rec
  (CallFunction|RPCRollRec))

(event Custom|RPC_Roll_Rec
  (CallFunction|CamRollRecF))

(event Input|EnhancedActionEvents|EnhancedInputActionPitch
  (params (ActionValue :type Float%20%28double-precision%29) (ElapsedSeconds :type Float%20%28double-precision%29) (TriggeredSeconds :type Float%20%28double-precision%29) (InputAction :type Input%20Action%20Object%20Reference :default "/Game/Input/Actions/Pitch.Pitch"))
  (:Triggered
    (CallFunction|RPCServerYaw ActionValue :!label _label))
  (:Ongoing
    (goto _label))
  (:Canceled
    (CallFunction|RPCServerYawRec :!label _label_2))
  (:Completed
    (goto _label_2)))

(event Input|EnhancedActionEvents|EnhancedInputActionYaw
  (params (ActionValue :type Float%20%28double-precision%29) (ElapsedSeconds :type Float%20%28double-precision%29) (TriggeredSeconds :type Float%20%28double-precision%29) (InputAction :type Input%20Action%20Object%20Reference :default "/Game/Input/Actions/Yaw.Yaw"))
  (:Triggered
    (CallFunction|RPCServerPitch ActionValue :!label _label))
  (:Ongoing
    (goto _label))
  (:Canceled
    (CallFunction|RPCServerPitchRec :!label _label_2))
  (:Completed
    (goto _label_2)))

(event Input|EnhancedActionEvents|EnhancedInputActionRoll
  (params (ActionValue :type Float%20%28double-precision%29) (ElapsedSeconds :type Float%20%28double-precision%29) (TriggeredSeconds :type Float%20%28double-precision%29) (InputAction :type Input%20Action%20Object%20Reference :default "/Game/Input/Actions/Roll.Roll"))
  (:Triggered
    (CallFunction|RPCServerRoll ActionValue :!label _label))
  (:Ongoing
    (goto _label))
  (:Canceled
    (CallFunction|RPCServerRollRec :!label _label_2))
  (:Completed
    (goto _label_2)))

(event Input|EnhancedActionEvents|EnhancedInputActionAccelerateDecelerate
  (params (ActionValue :type Float%20%28double-precision%29) (ElapsedSeconds :type Float%20%28double-precision%29) (TriggeredSeconds :type Float%20%28double-precision%29) (InputAction :type Input%20Action%20Object%20Reference :default "/Game/Input/Actions/AccelerateDecelerate.AccelerateDecelerate"))
  (:Triggered
    (CallFunction|RPCServerSpeed ActionValue :!label _label))
  (:Ongoing
    (goto _label)))

(event Input|EnhancedActionEvents|EnhancedInputActionSwapWeapons
  (params (ActionValue :type Float%20%28double-precision%29) (ElapsedSeconds :type Float%20%28double-precision%29) (TriggeredSeconds :type Float%20%28double-precision%29) (InputAction :type Input%20Action%20Object%20Reference :default "/Game/Input/Actions/SwapWeapons.SwapWeapons"))
  (bind _equippedweapons (Variables|Default|GetEquippedWeapons))
  (:Triggered
    (Math|Float|CompareFloat ActionValue 0.0 :!label _label
      (:>
        (Variables|Default|SetSelectedWep (Math|Integer|%(Integer) (+ (Variables|Default|GetSelectedWep) 1) (Utilities|Array|Length _equippedweapons))))
      (:<
        (Variables|Default|SetSelectedWep (select (< (- (Variables|Default|GetSelectedWep) 1) (Utilities|Array|LastIndex _equippedweapons)) 3 (- (Variables|Default|GetSelectedWep) 1))))))
  (:Ongoing
    (goto _label)))

(event Input|EnhancedActionEvents|EnhancedInputActionFire
  (params (ActionValue :type Boolean) (ElapsedSeconds :type Float%20%28double-precision%29) (TriggeredSeconds :type Float%20%28double-precision%29) (InputAction :type Input%20Action%20Object%20Reference :default "/Game/Input/Actions/Fire.Fire"))
  (bind _selectedwep (Variables|Default|GetSelectedWep))
  (:Triggered
    (switch int _selectedwep
      (:0
        (CallFunction|RPCServerFire :!label _label))))
  (:Started
    (switch int _selectedwep
      (:1
        (CallFunction|RPCServerFireMissile))))
  (:Ongoing
    (switch int _selectedwep
      (:0
        (goto _label)))))

(event Input|EnhancedActionEvents|EnhancedInputActionLockTarget
  (params (ActionValue :type Boolean) (ElapsedSeconds :type Float%20%28double-precision%29) (TriggeredSeconds :type Float%20%28double-precision%29) (InputAction :type Input%20Action%20Object%20Reference :default "/Game/Input/Actions/LockTarget.LockTarget"))
  (bind _radarorigin (Variables|Default|GetRadarOrigin))
  (bind _returnvalue (Transformation|GetWorldLocation _radarorigin))
  (bind _returnvalue_2 (Transformation|GetWorldRotation _radarorigin))
  (:Triggered
    (bind _outhit (Class|KismetSystemLibrary|BoxTraceSingleforObjects _returnvalue (+ _returnvalue (* (Math|Vector|GetForwardVector _returnvalue_2) (Variables|Default|GetRadarMaxRange))) "5000.000000,5000.000000,5000.000000" _returnvalue_2 (Utilities|Array|MakeArray "ObjectTypeQuery3") false 0 "ForDuration" true "(R=1.000000,G=0.000000,B=0.000000,A=1.000000)" "(R=0.000000,G=1.000000,B=0.000000,A=1.000000)" 0.1))
    (Utilities|IsValid (.HitActor (Collision|BreakHitResult _outhit))
      (:Is%20Valid
        (bind _output_get (Variables|Default|SetLocation (.Location (Collision|BreakHitResult _outhit))))
        (if true
          (bind _output_get_2 (Variables|Default|SetLockTarget (.HitActor (Collision|BreakHitResult _outhit))))
          (Utilities|Array|Add (Variables|/Script/Engine.Actor|GetTags _output_get_2) "Homing")
          (bind _returnvalue_3 (Game|SpawnActorfromClass "/Game/Blueprints/Target_Lock.Target_Lock_C" (Math|Transform|MakeTransform "0, 0, 0" "0, 0, 0" "1.000000,1.000000,1.000000") "Undefined" _output_get_2 0))
          (Variables|Default|SetTargetLockTracker _returnvalue_3))))))

(event EventBeginPlay
  (bind _asplayer_controller (Utilities|Casting|CastToPlayerController (Pawn|GetController)))
  (Utilities|IsValid (PlayerController|LocalPlayerSubsystems|GetEnhancedInputLocalPlayerSubsystem _asplayer_controller)
    (:Is%20Valid
      (Input|AddMappingContext (PlayerController|LocalPlayerSubsystems|GetEnhancedInputLocalPlayerSubsystem _asplayer_controller) "/Game/Input/NewInputMappingContext.NewInputMappingContext" 0 "(bIgnoreAllPressedKeysUntilRelease=True,bForceImmediately=False)")
      (bind _returnvalue (UserInterface|CreateWidget "/Game/HUD/HUD_Widget.HUD_Widget_C"))
      (UserInterface|Viewport|AddtoViewport _returnvalue 0))))

(event EventTick
  (params (DeltaSeconds :type Float%20%28single-precision%29))
  (CallFunction|RPCServerMovement DeltaSeconds))

(event Game|Damage|EventAnyDamage
  (params (Damage :type Float%20%28single-precision%29) (DamageType :type Damage%20Type%20Object%20Reference) (InstigatedBy :type Controller%20Object%20Reference) (DamageCauser :type Actor%20Object%20Reference))
  (Effects|SpawnEmitteratLocation "/Game/StarterContent/Particles/P_Explosion.P_Explosion" "0, 0, 0")
  (Variables|Default|SetHealth (Math|Float|Clamp(Float) (- (Variables|Default|GetHealth) Damage) 0.0 (Variables|Default|GetMaxHealth)))
  (if (<= (Variables|Default|GetHealth) 0.0)
    (Variables|Default|SetIsAlive false)
    (Actor|DestroyActor)))

(fn ConstructionScript)

(fn ThrottleInput
  (bind _tempname (Variables|Default|GetTempName))
  (if true
    (bind _result (Math|Integer|IncrementInt _tempname))
    (elif true
      (bind _result_2 (Math|Integer|DecrementInt _tempname)))))

(fn UpdatePosition
  (params (DeltaSeconds :type Float%20%28double-precision%29))
  ;[1 1 1] Calc Current Speed
  (Variables|Default|SetCurrentSpeed (Math|Float|Clamp(Float) (select (< (Variables|Default|GetThrustSpeed) (Variables|Default|GetCurrentSpeed)) (Math|Interpolation|FInterpTo (Variables|Default|GetCurrentSpeed) (Variables|Default|GetThrustSpeed) DeltaSeconds (Variables|Default|GetDrag)) (Variables|Default|GetThrustSpeed)) 0.0 (Variables|Default|GetMaxThrustSpeed)))
  ;[1 1 1] Calc new position based on speed
  (Variables|Default|SetNewPos (* (* (Variables|Default|GetCurrentSpeed) DeltaSeconds) (Transformation|GetActorForwardVector)))
  ;[1 1 1] Calc Applied Gravity
  (Variables|Default|SetAppliedGravity (Math|Float|MapRangeClamped (Variables|Default|GetCurrentSpeed) 0.0 (Variables|Default|GetMinThrustStall) (Variables|Default|GetGravity) 0.0))
  ;[1 1 1] Get Position
  (Transformation|AddActorWorldOffset (Math|Vector|MakeVector (.X (Class|KismetMathLibrary|BreakVector3f (Variables|Default|GetNewPos))) (.Y (Class|KismetMathLibrary|BreakVector3f (Variables|Default|GetNewPos))) (- (.Z (Class|KismetMathLibrary|BreakVector3f (Variables|Default|GetNewPos))) (* (Variables|Default|GetAppliedGravity) 1.0))) true)
  (CallFunction|UpdateAnimation))

(fn PrintVar
  (Utilities|FlowControl|Sequence
    (:then_0
      (Development|PrintString (Utilities|String|Append "ThrustSpeed;" (Utilities|String|ToString(Float) (Variables|Default|GetThrustSpeed)))))
    (:then_1
      (Development|PrintString (Utilities|String|Append "CurrentSpeed;" (Utilities|String|ToString(Float) (Variables|Default|GetCurrentSpeed)))))
    (:then_2
      (Development|PrintString (Utilities|String|Append "Yaw;" (Utilities|String|ToString(Float) 0.0))))
    (:then_3
      (Development|PrintString (Utilities|String|Append "Pitch;" (Utilities|String|ToString(Float) 0.0))))
    (:then_4
      (Development|PrintString (Utilities|String|Append "Roll;" (Utilities|String|ToString(Float) 0.0))))
    (:then_5
      (Development|PrintString (Utilities|String|Append "DeltaSeconds" (Utilities|String|ToString(Float) (Utilities|Time|GetWorldDeltaSeconds)))))))

(fn UpdateYaw
  (params (DeltaSeconds :type Float%20%28double-precision%29) (Yaw :type Float%20%28double-precision%29))
  (bind _output_get (Variables|Default|SetTargetYaw Yaw))
  (Variables|Default|SetCurrentSpeed (- (Variables|Default|GetCurrentSpeed) (* (Math|Float|Absolute(Float) _output_get) 2.0)))
  (bind _output_get_2 (Variables|Default|SetCurrentYaw (Math|Interpolation|FInterpTo (Variables|Default|GetCurrentYaw) (Variables|Default|GetTargetYaw) DeltaSeconds 1e+01)))
  (Transformation|AddActorLocalRotation (Math|Rotator|MakeRotator 0.0 0.0 (* _output_get_2 DeltaSeconds (Variables|Turnspeed|GetTurnspeedZ) 4.0)) false false))

(fn UpdateRoll
  (params (DeltaSeconds :type Float%20%28double-precision%29) (Roll :type Float%20%28double-precision%29))
  (Variables|Default|SetTargetRoll Roll)
  (bind _output_get (Variables|Default|SetCurrentRoll (Math|Interpolation|FInterpTo (Variables|Default|GetCurrentRoll) (Variables|Default|GetTargetRoll) DeltaSeconds 1e+01)))
  (Transformation|AddActorLocalRotation (Math|Rotator|MakeRotator (* _output_get DeltaSeconds 5e+02) 0.0 0.0) false false))

(fn UpdatePitch
  (params (DeltaSeconds :type Float%20%28double-precision%29) (Pitch :type Float%20%28double-precision%29))
  (Variables|Default|SetCurrentPitch Pitch)
  (bind _output_get (Variables|Default|SetTargetPitch (Math|Interpolation|FInterpTo (Variables|Default|GetCurrentPitch) (Variables|Default|GetTargetPitch) 0.0 1e+01)))
  (Transformation|AddActorLocalRotation (Math|Rotator|MakeRotator 0.0 (* _output_get DeltaSeconds (Variables|Turnspeed|GetTurnspeedZ) 1e+01) 0.0) false false))

(fn HighGTurnNPSM
  (if (and (<= (Variables|Default|GetCurrentSpeed) 1.5e+03) (Variables|Default|GetIsPSMCapable))
    (Variables|Turnspeed|SetTurnspeedZ 1e+01)
    (else
      (Variables|Turnspeed|SetTurnspeedZ 3.0))))

(fn Movement)

(fn UpdateTurnRate
  (Variables|Turnspeed|SetTurnspeedZ (* (Math|Float|SafeDivide (Variables|Turnspeed|GetTurnspeedZ) (Variables|Default|GetCurrentSpeed)) 1e+03)))

(fn UpdateAnimation)

(fn UpdateTurnRecovery
  (bind _rollrecover (Variables|Default|GetRollRecover))
  (Variables|Default|SetCurrentRoll (Math|Interpolation|FInterpTo (Variables|Default|GetCurrentRoll) 0.0 (Utilities|Time|GetWorldDeltaSeconds) _rollrecover))
  (Variables|Default|SetCurrentPitch (Math|Interpolation|FInterpTo (Variables|Default|GetCurrentPitch) 0.0 (Utilities|Time|GetWorldDeltaSeconds) _rollrecover))
  (Variables|Default|SetCurrentYaw (Math|Interpolation|FInterpTo (Variables|Default|GetCurrentYaw) 0.0 (Utilities|Time|GetWorldDeltaSeconds) _rollrecover)))

(fn GunFire
  (Utilities|FlowControl|FlipFlop
    (:A
      (Game|SpawnActorfromClass "/Game/Blueprints/BP_Projectile.BP_Projectile_C" (Transformation|GetWorldTransform (Variables|Default|GetFireLocation1)) "AlwaysSpawn" 0 0))
    (:B
      (Game|SpawnActorfromClass "/Game/Blueprints/BP_Projectile.BP_Projectile_C" (Transformation|GetWorldTransform (Variables|Default|GetFireLocation2)) "AlwaysSpawn" 0 0))))

(fn TargetLock
  (bind _radarorigin (Variables|Default|GetRadarOrigin))
  (bind _returnvalue (Transformation|GetWorldLocation _radarorigin))
  (while (< (Variables|Default|GetRadarRange) (Variables|Default|GetRadarMaxRange))
    (Collision|SphereTraceByChannel _returnvalue (+ _returnvalue (* (Math|Vector|GetForwardVector (Transformation|GetWorldRotation _radarorigin)) (Variables|Default|GetRadarRange))) (Variables|Default|GetCurrentRadarRadius) "TraceTypeQuery1" false 0 "ForDuration")
    (Variables|Default|SetCurrentRadarRadius (+ (Variables|Default|GetCurrentRadarRadius) 2e+02))
    (Variables|Default|SetRadarRange (+ (Variables|Default|GetRadarRange) 1e+02)))
  (Variables|Default|SetCurrentRadarRadius 0.0)
  (Variables|Default|SetRadarRange 0.0))

(fn TargetLock2
  (bind _radarorigin (Variables|Default|GetRadarOrigin))
  (bind _returnvalue (Transformation|GetWorldLocation _radarorigin))
  (Variables|Default|GetTargetLockTracker
    (:then
      (Actor|DestroyActor (Variables|Default|GetTargetLockTracker)))
    (:else
      _))
  (Utilities|FlowControl|FlipFlop
    (:A
      (Variables|Default|SetIsTargetLocked true)
      (bind (_outhit _returnvalue_2) (Collision|SphereTraceForObjects _returnvalue (+ _returnvalue (* (Math|Vector|GetForwardVector (Transformation|GetWorldRotation _radarorigin)) (Variables|Default|GetRadarMaxRange))) (Variables|Default|GetRadarRadius) (Utilities|Array|MakeArray "ObjectTypeQuery3") false 0 "ForDuration"))
      (if _returnvalue_2
        (bind _output_get (Variables|Default|SetLockTarget (.HitActor (Collision|BreakHitResult _outhit))))
        (bind _returnvalue_3 (Game|SpawnActorfromClass "/Game/Blueprints/Target_Lock.Target_Lock_C" (Math|Transform|MakeTransform (Transformation|GetActorLocation _output_get) "0, 0, 0" "1.000000,1.000000,1.000000") "Undefined" 0 0))
        (Variables|Default|SetTargetLockTracker _returnvalue_3)))
    (:B
      (Variables|Default|SetIsTargetLocked false)
      (Variables|Default|SetLockTarget 0))))

(fn HideLockforSelf
  (bind _iff (Variables|Default|GetIFF))
  (if (not (Pawn|IsLocallyControlled))
    (Rendering|SetVisibility _iff false false)
    (else
      (Rendering|SetVisibility _iff false false))))

(fn SetScreenRatio)

(fn LockTrackFunction
  (Transformation|SetActorLocation (Variables|Default|GetTargetLockTracker) (Transformation|GetActorLocation (Variables|Default|GetLockTarget)) false false))

(fn CopyRot
  (bind _camera (Variables|Default|GetCamera))
  (bind _returnvalue (Transformation|GetSocketRotation _camera "None"))
  (Variables|Turnspeed|SetTargetRotation (Math|Rotator|MakeRotator (.roll (Math|Rotator|Lerp(Rotator) (Math|Rotator|MakeRotator (.roll (Variables|Turnspeed|GetTargetRotation)) 0.0 0.0) (Math|Rotator|MakeRotator (.roll _returnvalue) 0.0 0.0) 0.1 true)) (.pitch (Math|Rotator|Lerp(Rotator) (Math|Rotator|MakeRotator 0.0 (.pitch (Variables|Turnspeed|GetTargetRotation)) 0.0) (Math|Rotator|MakeRotator 0.0 (.pitch _returnvalue) 0.0) 0.1 true)) (.yaw (Math|Rotator|Lerp(Rotator) (Math|Rotator|MakeRotator 0.0 0.0 (.yaw (Variables|Turnspeed|GetTargetRotation))) (Math|Rotator|MakeRotator 0.0 0.0 (.yaw _returnvalue)) 0.1 true))))
  (Transformation|SetActorRotation (Math|Rotator|Lerp(Rotator) (Transformation|GetActorRotation) (Variables|Turnspeed|GetTargetRotation) 0.1 true)))

(fn Speed
  (params (Speed :type Float%20%28double-precision%29) (Delta :type Float%20%28double-precision%29))
  (Variables|Default|SetThrustSpeed (Math|Float|Clamp(Float) (+ (* Speed Delta (Variables|Default|GetThrustMultiplier)) (Variables|Default|GetThrustSpeed)) 0.0 (Variables|Default|GetMaxThrustSpeed))))

(fn DynamicOffset
  (params (Roll :type Float%20%28double-precision%29) (Pitch :type Float%20%28double-precision%29) (Yaw :type Float%20%28double-precision%29)))

(fn PitchF
  (bind _output_get (Variables|Default|SetCurrentPitch (Math|Interpolation|FInterpTo (Variables|Default|GetCurrentPitch) (Variables|Default|GetTargetPitch) (Utilities|Time|GetWorldDeltaSeconds) (Variables|Default|GetInterp%20Speed))))
  (Transformation|AddLocalRotation (Variables|Default|GetCamera) (Math|Rotator|MakeRotator 0.0 (* _output_get (Variables|Default|GetTurnspeed) 1.0) 0.0) false false))

(fn YawF
  (bind _output_get (Variables|Default|SetCurrentYaw (Math|Interpolation|FInterpTo (Variables|Default|GetCurrentYaw) (Variables|Default|GetTargetYaw) (Utilities|Time|GetWorldDeltaSeconds) (Variables|Default|GetInterp%20Speed))))
  (Transformation|AddLocalRotation (Variables|Default|GetCamera) (Math|Rotator|MakeRotator 0.0 0.0 (* _output_get (Variables|Default|GetTurnspeed) 1.0)) false false))

(fn RollF
  (bind _output_get (Variables|Default|SetCurrentRoll (Math|Interpolation|FInterpTo (Variables|Default|GetCurrentRoll) (Variables|Default|GetTargetRoll) (Utilities|Time|GetWorldDeltaSeconds) (Variables|Default|GetInterp%20Speed))))
  (Transformation|AddLocalRotation (Variables|Default|GetCamera) (Math|Rotator|MakeRotator (* _output_get 5.0) 0.0 0.0) false false))

(fn GunFire
  (Variables|Default|SetFireLoc (Variables|Default|GetFireLocation1))
  (Game|SpawnActorfromClass "/Game/Blueprints/BP_Bullet.BP_Bullet_C" (Math|Transform|MakeTransform (.location (Transformation|GetWorldTransform (Variables|Default|GetFireLoc))) (Math|Rotator|MakeRotator (.roll (.rotation (Transformation|GetWorldTransform (Variables|Default|GetFireLoc)))) (+ (.pitch (.rotation (Transformation|GetWorldTransform (Variables|Default|GetFireLoc)))) (Math|Random|RandomFloatinRange -1.0 1.0)) (+ (.yaw (.rotation (Transformation|GetWorldTransform (Variables|Default|GetFireLoc)))) (Math|Random|RandomFloatinRange -1.0 1.0))) (.scale (Transformation|GetWorldTransform (Variables|Default|GetFireLoc)))) "AlwaysSpawn" (Game|Player|GetPlayerPawn 0) 0))

(fn CamRollF
  (params (AngleDegrees :type Float%20%28double-precision%29))
  (bind _maxlook (Variables|Default|GetMaxLook))
  (bind _returnvalue (* _maxlook 0.35))
  (Variables|Default|SetTargetRoll (Math|Float|ClampAngle AngleDegrees (* _returnvalue -1.0) _returnvalue))
  (Variables|Default|SetIsRoll true))

(fn CamPitchF
  (params (AngleDegrees :type Float%20%28double-precision%29))
  (bind _maxlook (Variables|Default|GetMaxLook))
  (bind _returnvalue (* _maxlook 1.2))
  (Variables|Default|SetTargetYaw (Math|Float|ClampAngle AngleDegrees (* _returnvalue -1.0) _returnvalue))
  (Variables|Default|SetIsYaw true))

(fn CamYawF
  (params (AngleDegrees :type Float%20%28double-precision%29))
  (bind _maxlook (Variables|Default|GetMaxLook))
  (bind _returnvalue (* _maxlook 2.0))
  (Variables|Default|SetTargetPitch (Math|Float|ClampAngle AngleDegrees (* _returnvalue -1.0) _returnvalue))
  (Variables|Default|SetIsPitch true))

(fn CamRollRecF
  (Variables|Default|SetTargetRoll (Math|Interpolation|FInterpTo (Variables|Default|GetTargetRoll) 0.0 (Utilities|Time|GetWorldDeltaSeconds) 0.0))
  (Variables|Default|SetIsRoll false))

(fn CamPitchRecF
  (Variables|Default|SetTargetYaw (Math|Interpolation|FInterpTo (Variables|Default|GetTargetYaw) 0.0 (Utilities|Time|GetWorldDeltaSeconds) 0.0))
  (Variables|Default|SetIsYaw false))

(fn CamYawRecF
  (Variables|Default|SetTargetPitch (Math|Interpolation|FInterpTo (Variables|Default|GetTargetPitch) 0.0 (Utilities|Time|GetWorldDeltaSeconds) 0.0))
  (Variables|Default|SetIsPitch false))

(fn MissileFire
  (Game|SpawnActorfromClass "/Game/Blueprints/Missile.Missile_C" (Transformation|GetActorTransform) "Undefined" 0 0))