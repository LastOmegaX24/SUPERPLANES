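; BPC_WeaponSystem is a weapon component that holds weapon slots and toggles the weapon loadout HUD.
; On BeginPlay it adds the KBM Enhanced Input mapping context to the local player.
; OpenWeaponLoadout creates or removes the HUD, loads its slots and switches cursor and input mode.
; SelectKey also closes the HUD but leaves IsOpen and the widget reference unchanged, while AddModule appends items to WeaponSlots.
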(event Input|EnhancedActionEvents|EnhancedInputActionSelectKey
  (params (ActionValue :type Boolean) (ElapsedSeconds :type Float%20%28double-precision%29) (TriggeredSeconds :type Float%20%28double-precision%29) (InputAction :type Input%20Action%20Object%20Reference :default "/Game/Input/Actions/SelectKey.SelectKey"))
  (bind _returnvalue (Game|GetPlayerController 0))
  (:Triggered
    (bind _weaponhudref (Variables|Default|GetWeaponHUDRef)
      (:then
        (Widget|RemovefromParent _weaponhudref)
        (Input|SetInputModeGameOnly _returnvalue false)
        (Variables|/Script/Engine.PlayerController|SetbShowMouseCursor _returnvalue false))
      (:else))))

(event Input|EnhancedActionEvents|EnhancedInputActionOpenWeaponLoadout
  (params (ActionValue :type Boolean) (ElapsedSeconds :type Float%20%28double-precision%29) (TriggeredSeconds :type Float%20%28double-precision%29) (InputAction :type Input%20Action%20Object%20Reference :default "/Game/Input/Actions/OpenWeaponLoadout.OpenWeaponLoadout"))
  (bind _returnvalue (Game|GetPlayerController 0))
  (:Started
    (if (not (Variables|Default|GetisOpen))
      (Variables|Default|SetisOpen true)
      (bind _returnvalue_2 (UserInterface|CreateWidget "/Game/Menu/InGame/WeaponHUD.WeaponHUD_C"))
      (bind _output_get (Variables|Default|SetWeaponHUDRef _returnvalue_2))
      (UserInterface|Viewport|AddtoViewport _output_get 0)
      (Variables|/Script/Engine.PlayerController|SetbShowMouseCursor _returnvalue true)
      (Input|SetInputModeGameandUI _returnvalue (Variables|Default|GetWeaponHUDRef) "DoNotLock" true false)
      (Default|LoadWeaponSlots (Variables|Default|GetWeaponHUDRef))
      (else
        (Variables|Default|SetisOpen false)
        (bind _weaponhudref (Variables|Default|GetWeaponHUDRef)
          (:then
            (Widget|RemovefromParent _weaponhudref)
            (Variables|Default|SetWeaponHUDRef 0)
            (Variables|/Script/Engine.PlayerController|SetbShowMouseCursor _returnvalue false)
            (Input|SetInputModeGameOnly _returnvalue false))
          (:else))))))

(event EventBeginPlay
  (bind _asgmc_controller (Utilities|Casting|CastToGMC_Controller (Game|GetPlayerController 0)))
  (Utilities|IsValid (PlayerController|LocalPlayerSubsystems|GetEnhancedInputLocalPlayerSubsystem _asgmc_controller)
    (:Is%20Valid
      (Input|AddMappingContext (PlayerController|LocalPlayerSubsystems|GetEnhancedInputLocalPlayerSubsystem _asgmc_controller) "/Game/Input/KBM.KBM" 0 "(bIgnoreAllPressedKeysUntilRelease=True,bForceImmediately=False)"))))

(fn AddModule
  (params (AddItem :type S%20Slots%20Structure))
  (Utilities|Array|Add (Variables|Default|GetweaponSlots) AddItem))