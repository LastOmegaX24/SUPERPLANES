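; Predicted, networked movement component for a UFO-style pawn, built on the General Movement Component plugin.
; It binds rotation input and thrust, reverse and brake flags as client-authoritative replicated inputs.
; Each prediction tick brakes or accelerates along the forward vector, rotates the pawn locally, caps speed, then moves it and adjusts velocity on hits.
; Input handlers that would set the flags are not connected to any event.
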(event EventBeginPlay
  (bind _asplayer_controller (Utilities|Casting|CastToPlayerController (Pawn|GetController (Class|PawnMovementComponent|GetPawnOwner))))
  (Utilities|IsValid _asplayer_controller
    (:Is%20Valid
      (Input|AddMappingContext (PlayerController|LocalPlayerSubsystems|GetEnhancedInputLocalPlayerSubsystem _asplayer_controller) 0 0 "(bIgnoreAllPressedKeysUntilRelease=True,bForceImmediately=False)"))))

(event EventBindReplicationData
  (|CallParentFunction)
  (Class|GMCReplicationCmp|BindCompressedVector (Variables|Movement|GetRawInputVector) "ClientAuth_Input" "CombineIfUnchanged" "None" "NearestNeighbour")
  (Class|GMCReplicationCmp|BindBool (Variables|Movement|GetThrust) "ClientAuth_Input" "CombineIfUnchanged" "None" "NearestNeighbour")
  (Class|GMCReplicationCmp|BindBool (Variables|Movement|GetReverse) "ClientAuth_Input" "CombineIfUnchanged" "None" "NearestNeighbour")
  (Class|GMCReplicationCmp|BindBool (Variables|Movement|GetBrake) "ClientAuth_Input" "CombineIfUnchanged" "None" "NearestNeighbour"))

(event EventPreLocalMoveExecution
  (params (LocalMove :type GMC%20Move%20Structure%20%28by%20ref%29))
  (bind _returnvalue (Class|PawnMovementComponent|ConsumeInputVector))
  (Variables|Movement|SetRawInputVector _returnvalue))

(event EventGenPredictionTick
  (params (DeltaTime :type Float%20%28single-precision%29))
  (bind _returnvalue (Class|GMCReplicationCmp|GetVelocity))
  (bind _returnvalue_2 (Class|GMCMovementUtilityCmp|GetPhysDeltaTime))
  (bind _returnvalue_3 (Class|GMCMovementUtilityCmp|GetRootCollisionRotation))
  (bind _returnvalue_4 (Class|GMCReplicationCmp|GetVelocity))
  (bind _rawinputvector (Variables|Movement|GetRawInputVector))
  (bind _returnvalue_5 (* _returnvalue _returnvalue_2))
  (if (Variables|Movement|GetBrake)
    ;[1 0.749 0] Apply braking.
    (Class|GMCMovementUtilityCmp|UpdateVelocity (Class|GMCMovementUtilityCmp|ResizeVector _returnvalue_4 (Math|Interpolation|FInterptoConstant (Math|Vector|VectorLength _returnvalue_4) 0.0 DeltaTime (Variables|Movement|GetBrakeSpeed))) 0.0)
    (else
      (Class|GMCMovementUtilityCmp|AddAcceleration (* (* (Transformation|GetActorForwardVector (Class|PawnMovementComponent|GetPawnOwner)) (select (Variables|Movement|GetReverse) -1.0 1.0)) (* (Variables|Movement|GetAcceleration) (Math|Conversions|ToFloat(Boolean) (Variables|Movement|GetThrust)))) 0.0)))
  (Transformation|AddActorLocalRotation (Class|PawnMovementComponent|GetPawnOwner) (* (Math|Rotator|MakeRotator (.x _rawinputvector) (.y _rawinputvector) (.z _rawinputvector)) (* (Variables|Movement|GetRotationRate) (Class|GMCMovementUtilityCmp|GetPhysDeltaTime))) false false)
  (if (> (Math|Vector|VectorLength (Class|GMCReplicationCmp|GetVelocity)) (Variables|Movement|GetMaxSpeed))
    ;[1 0.749 0] Limit velocity to max speed.
    (Class|GMCMovementUtilityCmp|UpdateVelocity (Class|GMCMovementUtilityCmp|ResizeVector (Class|GMCReplicationCmp|GetVelocity) (Variables|Movement|GetMaxSpeed)) 0.0))
  ;[1 0.749 0] Apply the location delta for this frame.
  (bind _outhit (Class|MovementComponent|MoveUpdatedComponent _returnvalue_5 _returnvalue_3 true))
  ;[1 0.749 0] Adjust for collisions so we don't get stuck immediately when hitting something.
  (if (.bBlockingHit (Collision|BreakHitResult _outhit))
    (Class|GMCMovementUtilityCmp|AdjustVelocityfromHit _outhit false 0.0)
    (Class|MovementComponent|MoveUpdatedComponent _returnvalue_5 _returnvalue_3 true)))